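; Anim notify that plays an FMOD event from an animated skeletal mesh.
; With Follow on, it attaches the event to the mesh at AttachName, then assigns the notify's attenuation and occlusion details to the returned audio component.
; Otherwise it plays the event at the mesh component's world transform, without the attach name or those details.
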(fn `Received_Notify`
  (params (MeshComp :type "SkeletalMeshComponent Object Reference") (Animation :type "AnimSequenceBase Object Reference") (EventReference :type "AnimNotifyEventReference Structure (by ref)"))
  (returns (ReturnValue :type Boolean))
  (if (`self.bFollow`)
    (bind _returnvalue (`FMODBlueprintStatics.PlayEventAttached` (`self.Event`) MeshComp (`KismetStringLibrary.Conv_StringToName` (`self.AttachName`)) (0.0 0.0 0.0) "KeepRelativeOffset"))
    (set `FMODAudioComponent.AttenuationDetails` (`self.Attenuation Details`) _returnvalue)
    (set `FMODAudioComponent.OcclusionDetails` (`self.Occlusion Details`) _returnvalue)
    (else
      (`FMODBlueprintStatics.PlayEventAtLocation` (`self.Event`) (`SceneComponent.K2_GetComponentToWorld` MeshComp))))
  (return false))