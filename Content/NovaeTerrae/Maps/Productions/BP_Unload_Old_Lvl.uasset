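; Trigger actor that unloads earlier streamed main levels when a BP_NTBaseCharacter overlaps its Trigger component.
; An integer counter on the actor selects the level, so successive overlaps unload Lvl_main_1, Lvl_main_2, then Lvl_main_3 without blocking.
; The counter stops advancing at the last step, so any later overlap requests the Lvl_main_3 unload again.
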(event `self.Trigger.OnComponentBeginOverlap`
  (params (OverlappedComponent :type "PrimitiveComponent Object Reference") (OtherActor :type "Actor Object Reference") (OtherComp :type "PrimitiveComponent Object Reference") (OtherBodyIndex :type Integer) (bFromSweep :type Boolean) (SweepResult :type "HitResult Structure (by ref)"))
  (cast `/Game/NovaeTerrae/Core/Characters/Base/BP_NTBaseCharacter` OtherActor)
  (if (== (`self.Int`) 0)
    (`GameplayStatics.UnloadStreamLevel` "Lvl_main_1")
    (set `self.Int` 1)
    (elif (== (`self.Int`) 1)
      (`GameplayStatics.UnloadStreamLevel` "Lvl_main_2")
      (set `self.Int` 2)
      (elif (== (`self.Int`) 2)
        (`GameplayStatics.UnloadStreamLevel` "Lvl_main_3")))))

(fn `UserConstructionScript`)