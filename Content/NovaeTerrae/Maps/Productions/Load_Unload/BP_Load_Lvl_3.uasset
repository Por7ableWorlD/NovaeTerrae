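; Level-streaming trigger actor that loads Lvl_main_3 and records it as the level to load in the save game.
; When a BP_NTBaseCharacter overlaps Trigger, it streams the level in without blocking and makes it visible.
; A separate Trigger_Lvl_To_Save overlap writes the level name to the SaveRef of the player character cached on BeginPlay and saves it to the Save_Info slot.
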(event `self.ReceiveBeginPlay`
  (bind _asbp_ntbase_character (cast `/Game/NovaeTerrae/Core/Characters/Base/BP_NTBaseCharacter` (`GameplayStatics.GetPlayerCharacter` 0)))
  (set `self.Char_Ref` _asbp_ntbase_character))

(event `self.Trigger.OnComponentBeginOverlap`
  (params (OverlappedComponent :type "PrimitiveComponent Object Reference") (OtherActor :type "Actor Object Reference") (OtherComp :type "PrimitiveComponent Object Reference") (OtherBodyIndex :type Integer) (bFromSweep :type Boolean) (SweepResult :type "HitResult Structure (by ref)"))
  (cast `/Game/NovaeTerrae/Core/Characters/Base/BP_NTBaseCharacter` OtherActor)
  (`GameplayStatics.LoadStreamLevel` "Lvl_main_3" true))

(event `self.Trigger_Lvl_To_Save.OnComponentBeginOverlap`
  (params (OverlappedComponent :type "PrimitiveComponent Object Reference") (OtherActor :type "Actor Object Reference") (OtherComp :type "PrimitiveComponent Object Reference") (OtherBodyIndex :type Integer) (bFromSweep :type Boolean) (SweepResult :type "HitResult Structure (by ref)"))
  (bind _save_ref (`/Game/NovaeTerrae/Core/Characters/Base/BP_NTBaseCharacter.Save_Ref` (`self.Char_Ref`)))
  (cast `/Game/NovaeTerrae/Core/Characters/Base/BP_NTBaseCharacter` OtherActor)
  (set `/Game/NovaeTerrae/Puzzles/Altar/BP_Save.Lvl_To_Load` "Lvl_main_3" _save_ref)
  (`GameplayStatics.SaveGameToSlot` _save_ref "Save_Info"))

(fn `UserConstructionScript`)