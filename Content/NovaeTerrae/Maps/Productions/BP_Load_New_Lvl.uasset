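; BP_Load_New_Lvl is a trigger actor that streams in a main level section when the player character overlaps it.
; The overlap passes a DoOnce that is never reset, then the Int variable selects which level to load asynchronously and make visible.
; Int advances after the first two cases, but each instance loads only once, so its starting value determines the level.
; CharRef is cached on BeginPlay but never used.
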(event `self.ReceiveBeginPlay`
  (bind _asbp_ntbase_character (cast `/Game/NovaeTerrae/Core/Characters/Base/BP_NTBaseCharacter` (`GameplayStatics.GetPlayerCharacter` 0)))
  (set `self.Char_Ref` _asbp_ntbase_character))

(event `self.Trigger.OnComponentBeginOverlap`
  (params (OverlappedComponent :type "PrimitiveComponent Object Reference") (OtherActor :type "Actor Object Reference") (OtherComp :type "PrimitiveComponent Object Reference") (OtherBodyIndex :type Integer) (bFromSweep :type Boolean) (SweepResult :type "HitResult Structure (by ref)"))
  (cast `/Game/NovaeTerrae/Core/Characters/Base/BP_NTBaseCharacter` OtherActor)
  (`/Engine/EditorBlueprintResources/StandardMacros.DoOnce` false
    (:`Completed`
      (if (== (`self.Int`) 0)
        (`GameplayStatics.LoadStreamLevel` "Lvl_main_1_2" true)
        (set `self.Int` 1)
        (elif (== (`self.Int`) 1)
          (`GameplayStatics.LoadStreamLevel` "Lvl_main_2" true)
          (set `self.Int` 2)
          (elif (== (`self.Int`) 2)
            (`GameplayStatics.LoadStreamLevel` "Lvl_main_3" true)
            (elif (== (`self.Int`) 3)
              (`GameplayStatics.LoadStreamLevel` "Lvl_main_4" true))))))))

(fn `UserConstructionScript`)