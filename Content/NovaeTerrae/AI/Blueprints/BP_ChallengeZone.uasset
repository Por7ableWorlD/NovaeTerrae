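; Challenge zone actor that starts and cancels a challenge through a box trigger and activate/deactivate event dispatchers.
; A base character entering the box broadcasts activation; exiting it or the player's death triggers deactivation.
; BeginPlay caches all deactivation objects and the core, and binds to the player's death.
; EndChallenge, with no caller in this graph, completes the challenge by killing every cached deactivation object.
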(event `self.ReceiveBeginPlay`
  (bind _outactors (`GameplayStatics.GetAllActorsOfClass` "/Game/NovaeTerrae/AI/Blueprints/BP_DeactivationObject.BP_DeactivationObject_C"))
  (set `self.Deactivators` _outactors)
  (bind _returnvalue (`GameplayStatics.GetActorOfClass` "/Game/NovaeTerrae/AI/Blueprints/BP_Core.BP_Core_C"))
  (set `self.Core` _returnvalue)
  (bind _asbp_ntbase_character (cast `/Game/NovaeTerrae/Core/Characters/Base/BP_NTBaseCharacter` (`GameplayStatics.GetPlayerCharacter` 0)))
  (add `/Game/NovaeTerrae/Core/Characters/Base/BP_NTBaseCharacter.OnDeath` _asbp_ntbase_character (delegate `OnDeath_Event`)))

(event `OnDeath_Event`
  (`self.OnDeactivateChallenge`)
  (`KismetSystemLibrary.PrintString` "Challenge deactivated" true true (struct :`R` 0.027728 :`G` 0.270796 :`B` 1.0 :`A` 1.0)))

(event `self.Box.OnComponentEndOverlap`
  (params (OverlappedComponent :type "PrimitiveComponent Object Reference") (OtherActor :type "Actor Object Reference") (OtherComp :type "PrimitiveComponent Object Reference") (OtherBodyIndex :type Integer))
  (cast `/Game/NovaeTerrae/Core/Characters/Base/BP_NTBaseCharacter` OtherActor)
  (`self.OnDeath_Event`))

(event `EndChallenge`
  (for _array_element (`self.Deactivators`)
    (`/Game/NovaeTerrae/AI/Blueprints/BP_DeactivationObject.Die` _array_element))
  (`KismetSystemLibrary.PrintString` "Challenge completed" true true (struct :`R` 0.085807 :`G` 1.0 :`A` 1.0)))

(event `self.Box.OnComponentBeginOverlap`
  (params (OverlappedComponent :type "PrimitiveComponent Object Reference") (OtherActor :type "Actor Object Reference") (OtherComp :type "PrimitiveComponent Object Reference") (OtherBodyIndex :type Integer) (bFromSweep :type Boolean) (SweepResult :type "HitResult Structure (by ref)"))
  (cast `/Game/NovaeTerrae/Core/Characters/Base/BP_NTBaseCharacter` OtherActor)
  (`self.OnActivateChallenge`)
  (`KismetSystemLibrary.PrintString` "Challenge has begun" true true (struct :`R` 1.0 :`A` 1.0)))

(fn `UserConstructionScript`)