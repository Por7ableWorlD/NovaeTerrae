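; BP_Core is the challenge zone's core, which the player can deactivate to end the challenge.
; It finds the BP_ChallengeZone and counts its Deactivators down and up through their disabled and enabled events.
; When the count hits zero, it shows a text prompt and opens a 20-second window.
; Interacting while overlapping its sphere during that window calls EndChallenge on the zone.
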(event `self.ReceiveBeginPlay`
  (bind _deactivators (`/Game/NovaeTerrae/AI/Environment/BP_ChallengeZone.Deactivators` (`self.ChallengeZone`)))
  (bind _returnvalue (`GameplayStatics.GetActorOfClass` "/Game/NovaeTerrae/AI/Environment/BP_ChallengeZone.BP_ChallengeZone_C"))
  (set `self.ChallengeZone` _returnvalue)
  (`KismetSystemLibrary.Delay` 0.5)
  (set `self.DeactivatorsCounter` (`KismetArrayLibrary.Array_Length` _deactivators))
  (for _array_element _deactivators
    (add `/Game/NovaeTerrae/AI/Environment/BP_DeactivationObject.OnDisabled` _array_element (delegate `DecreaseCounter`))
    (add `/Game/NovaeTerrae/AI/Environment/BP_DeactivationObject.OnEnabled` _array_element (delegate `IncreaseCounter`))
    (bind _asbp_ntbase_character (cast `/Game/NovaeTerrae/Core/Characters/Base/BP_NTBaseCharacter` (`GameplayStatics.GetPlayerCharacter` 0)))
    (add `/Game/NovaeTerrae/Core/Characters/Base/BP_NTBaseCharacter.OnInteract` _asbp_ntbase_character (delegate `Interact`))))

(event `Interact`
  (if (and (`PrimitiveComponent.IsOverlappingActor` (`self.Sphere1`) (stale `self.ReceiveBeginPlay` _asbp_ntbase_character)) (`self.IsDeactivationAvailable`))
    (`/Game/NovaeTerrae/AI/Environment/BP_ChallengeZone.EndChallenge` (`self.ChallengeZone`))))

(event `DecreaseCounter`
  (bind _result (`/Engine/EditorBlueprintResources/StandardMacros.DecrementInt` (`self.DeactivatorsCounter`))
    (:`  `
      (if (== _result 0)
        (`self.StartReactivationSequence`)))))

(event `IncreaseCounter`
  (`/Engine/EditorBlueprintResources/StandardMacros.IncrementInt` (`self.DeactivatorsCounter`)))

(event `StartReactivationSequence`
  (set `self.IsDeactivationAvailable` true)
  (`SceneComponent.SetHiddenInGame` (`self.TextRender`) false false)
  (`KismetSystemLibrary.Delay` 20.0)
  (set `self.IsDeactivationAvailable` false)
  (`SceneComponent.SetHiddenInGame` (`self.TextRender`) true false))

(fn `UserConstructionScript`)