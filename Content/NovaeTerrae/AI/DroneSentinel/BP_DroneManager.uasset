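; BP_DroneManager assigns drones to turrets for repair, capping how many drones serve each turret.
; On BeginPlay it maps every BP_Turret to its free drone slots.
; FindBestTargetToRepair releases the drone's slot, then picks an open turret other than its previous one with the lowest health, breaking ties by distance.
; RemoveDrone destroys a drone, returning any slot it held.
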(event `self.ReceiveBeginPlay`
  (bind _outactors (`GameplayStatics.GetAllActorsOfClass` "/Game/NovaeTerrae/AI/TurretSentinel/BP_Turret.BP_Turret_C"))
  (for _array_element _outactors
    (`BlueprintMapLibrary.Map_Add` (`self.Turrets`) _array_element (`self.MaxNumberOfDronesPerTurret`))))

(fn `FindBestTargetToRepair`
  (params (Drone :type "/Game/NovaeTerrae/AI/DroneSentinel/BP_DroneSentinel Object Reference"))
  (returns (Result :type "/Game/NovaeTerrae/AI/TurretSentinel/BP_Turret Object Reference"))
  (locals (ResultTarget :type "/Game/NovaeTerrae/AI/TurretSentinel/BP_Turret Object Reference") (Target :type "/Game/NovaeTerrae/AI/TurretSentinel/BP_Turret Object Reference") (BestDistance :type "Float (double-precision)") (LastTurret :type "/Game/NovaeTerrae/AI/TurretSentinel/BP_Turret Object Reference"))
  (bind _turrets (`self.Turrets`))
  (bind (_value _returnvalue) (`BlueprintMapLibrary.Map_Find` (`self.DronesLastTargets`) (`local.Drone`)))
  (bind (_value_2 _returnvalue_2) (`BlueprintMapLibrary.Map_Find` (`self.DronesCurrentTargets`) (`local.Drone`)))
  (bind _returnvalue_3 (`self.GetDistanceTo` (`local.Drone`) (`local.Target`)))
  (bind _returnvalue_4 (`NTHealthComponent.GetCurrentHealth` (`/Game/NovaeTerrae/AI/TurretSentinel/BP_Turret.NTEnemyHealth` (`local.ResultTarget`))))
  (bind _returnvalue_5 (`NTHealthComponent.GetCurrentHealth` (`/Game/NovaeTerrae/AI/TurretSentinel/BP_Turret.NTEnemyHealth` (`local.Target`))))
  (`/Engine/EditorBlueprintResources/StandardMacros.IsValid` Drone
    (:`Is Valid`
      (if _returnvalue_2
        (set `local.LastTurret` _value_2)
        (`BlueprintMapLibrary.Map_Add` (`self.Turrets`) (`local.LastTurret`) (+ (`BlueprintMapLibrary.Map_Find` (`self.Turrets`) (`local.LastTurret`)) 1))
        (`BlueprintMapLibrary.Map_Remove` (`self.DronesCurrentTargets`) (`local.Drone`))
        (elif _returnvalue
          (set `local.LastTurret` _value)))
      (bind _keys (`BlueprintMapLibrary.Map_Keys` (`self.Turrets`)))
      (for _array_element _keys
        (bind _output_get (set `local.Target` _array_element))
        (if (!= _output_get (`local.LastTurret`))
          (if (> (`BlueprintMapLibrary.Map_Find` (`self.Turrets`) (`local.Target`)) 0)
            (`local.ResultTarget`
              (:`then`
                (if (< _returnvalue_5 _returnvalue_4)
                  (set `local.BestDistance` _returnvalue_3 :!label _label)
                  (set `local.ResultTarget` (`local.Target`))
                  (elif (== _returnvalue_5 _returnvalue_4)
                    (if (< _returnvalue_3 (`local.BestDistance`))
                      (goto _label)))))
              (:`else`
                (goto _label))))))
      (`BlueprintMapLibrary.Map_Add` (`self.DronesLastTargets`) (`local.Drone`) (`local.LastTurret`))
      (`local.ResultTarget`
        (:`then`
          (if (> (`BlueprintMapLibrary.Map_Find` (`self.Turrets`) (`local.ResultTarget`)) 0)
            (`BlueprintMapLibrary.Map_Add` _turrets (`local.ResultTarget`) (- (`BlueprintMapLibrary.Map_Find` _turrets (`local.ResultTarget`)) 1))
            (`BlueprintMapLibrary.Map_Add` (`self.DronesCurrentTargets`) (`local.Drone`) (`local.ResultTarget`))
            (return (`local.ResultTarget`))
            (else
              (return null))))
        (:`else`
          (return null))))
    (:`Is Not Valid`
      (return null))))

(fn `Print`
  (bind _turrets (`self.Turrets`))
  (bind _keys (`BlueprintMapLibrary.Map_Keys` _turrets))
  (for _array_element _keys
    (`KismetSystemLibrary.PrintString` (`KismetStringLibrary.Concat_StrStr` (`KismetStringLibrary.Concat_StrStr` (`KismetSystemLibrary.GetDisplayName` _array_element) ": ") (`KismetStringLibrary.Conv_IntToString` (`BlueprintMapLibrary.Map_Find` _turrets _array_element))))))

(fn `RemoveDrone`
  (params (Drone :type "/Game/NovaeTerrae/AI/DroneSentinel/BP_DroneSentinel Object Reference"))
  (returns (Result :type "/Game/NovaeTerrae/AI/TurretSentinel/BP_Turret Object Reference"))
  (locals (LastTurret :type "/Game/NovaeTerrae/AI/TurretSentinel/BP_Turret Object Reference"))
  (bind (_value _returnvalue) (`BlueprintMapLibrary.Map_Find` (`self.DronesCurrentTargets`) (`local.Drone`)))
  (`/Engine/EditorBlueprintResources/StandardMacros.IsValid` Drone
    (:`Is Valid`
      (if _returnvalue
        (set `local.LastTurret` _value)
        (`BlueprintMapLibrary.Map_Add` (`self.Turrets`) (`local.LastTurret`) (+ (`BlueprintMapLibrary.Map_Find` (`self.Turrets`) (`local.LastTurret`)) 1))
        (`BlueprintMapLibrary.Map_Remove` (`self.DronesCurrentTargets`) (`local.Drone`))
        (`BlueprintMapLibrary.Map_Remove` (`self.DronesLastTargets`) (`local.Drone`))
        (`self.K2_DestroyActor` (`local.Drone`))
        (else
          (`self.K2_DestroyActor` (`local.Drone`)))))
    (:`Is Not Valid`
      (return null))))

(fn `UserConstructionScript`)