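; BP_DroneSentinel is a support drone that asks the level's BP_DroneManager for the best target to repair.
; A data table row supplies its max health and the healing amount written to the AI Blackboard, and movement states map to fixed speeds.
; On death it spawns an explosion and leaves the manager.
; When the manager is disabled, it detaches from its controller and drops as a physics body that ignores pawns.
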(event `self.ReceiveBeginPlay`
  (bind _returnvalue (`GameplayStatics.GetActorOfClass` "/Game/NovaeTerrae/AI/DroneSentinel/BP_DroneManager.BP_DroneManager_C"))
  (set `self.DroneManager` _returnvalue)
  (add `NTHealthComponent.OnDeath` (`self.HealthComponent`) (delegate `OnDeath_Event`))
  (bind _dronemanager (`self.DroneManager`)
    (:`then`
      (add `/Game/NovaeTerrae/AI/DroneSentinel/BP_DroneManager.ManagerDisabled` _dronemanager (delegate `DisableDrone`)))
    (:`else`)))

(event `OnDeath_Event`
  (params (DeathCauser :type "Actor Object Reference"))
  (`NiagaraFunctionLibrary.SpawnSystemAtLocation` "/Game/NovaeTerrae/Art/VFX/NS_Explosion_eyes.NS_Explosion_eyes" (`SceneComponent.K2_GetComponentLocation` (`self.Cone`)))
  (bind _dronemanager (`self.DroneManager`)
    (:`then`
      (`/Game/NovaeTerrae/AI/DroneSentinel/BP_DroneManager.RemoveDrone` _dronemanager self))
    (:`else`)))

(event `DisableDrone`
  (`self.DetachFromControllerPendingDestroy`)
  (`PrimitiveComponent.SetSimulatePhysics` (`self.Cone`) true)
  (`PrimitiveComponent.SetCollisionResponseToChannel` (`self.CapsuleComponent`) "ECC_Pawn" "ECR_Ignore")
  (`PrimitiveComponent.SetCollisionResponseToChannel` (`self.Cone`) "ECC_Pawn" "ECR_Ignore"))

(fn `FindTarget`
  (returns (Target :type "Actor Object Reference"))
  (bind _dronemanager (`self.DroneManager`)
    (:`then`
      (bind _result (`/Game/NovaeTerrae/AI/DroneSentinel/BP_DroneManager.FindBestTargetToRepair` _dronemanager self))
      (return _result))
    (:`else`)))

(fn `GetMovementSpeed`
  (params (`Movement Speed` :type "/Game/NovaeTerrae/AI/Enums/E_MovementSpeed Enum" :default "NewEnumerator0"))
  (returns (Speed :type "Float (double-precision)"))
  (return (select `/Game/NovaeTerrae/AI/Enums/E_MovementSpeed` `Movement Speed` :`NewEnumerator1` 100.0 :`NewEnumerator2` 300.0 :`NewEnumerator3` 600.0 :`NewEnumerator6` 1000.0)))

(fn `PrepareParametersFromDatatable`
  (locals (Blackboard :type "BlackboardComponent Object Reference"))
  (set `local.Blackboard` (`AIBlueprintHelperLibrary.GetBlackboard` (`AIBlueprintHelperLibrary.GetAIController` self)))
  (bind _returnvalue (`|GetDataTableRow` "/Game/NovaeTerrae/AI/DataTables/DT_DroneSentinel.DT_DroneSentinel" (`self.DataTableRowName`))
    (:`then`
      (`NTEnemyHealthComponent.SetDefaultMaxHealth` (`self.HealthComponent`) (break `/Game/NovaeTerrae/AI/DataTables/S_DroneSentinel` _returnvalue))
      (`BlackboardComponent.SetValueAsFloat` (`local.Blackboard`) "HealingAmount" (`.HealingAmount_5_1BCFF95B4F68DD68511F89B676413FA8` (break `/Game/NovaeTerrae/AI/DataTables/S_DroneSentinel` _returnvalue))))))

(fn `UserConstructionScript`)