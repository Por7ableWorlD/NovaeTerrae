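; Base AI controller for enemies that drives a blackboard state machine, from Passive through Investigating, Distracted and Agressive to Dead.
; Sight, hearing, damage and prediction handlers set states and targets, snapping invalid locations to nearby reachable points; losing sight of the player requests a movement prediction.
; Damage from the player or weak points feeds the damage sense.
; State changes update target aggro; timed stuns grant temporary immunity afterward.
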(event `self.ReceiveBeginPlay`
  (`self.SetCurrentState` "NewEnumerator0"))

(event `self.ReceivePossess`
  (params (PossessedPawn :type "Pawn Object Reference"))
  (add `self.OnTakeAnyDamage` PossessedPawn (delegate `OnTakeAnyDamage_Event`)))

(event `OnTakeAnyDamage_Event` :!signature `self.OnTakeAnyDamage`
  (params (DamagedActor :type "Actor Object Reference") (Damage :type "Float (single-precision)") (DamageType :type "DamageType Object Reference") (InstigatedBy :type "Controller Object Reference") (DamageCauser :type "Actor Object Reference"))
  (`/Engine/EditorBlueprintResources/StandardMacros.IsValid` InstigatedBy
    (:`Is Valid`
      (`self.ReportReceivedDamage` (`self.K2_GetPawn` InstigatedBy) Damage))
    (:`Is Not Valid`
      (`self.ReportReceivedDamage` DamageCauser Damage true))))

(event `self.ReceiveUnPossess`
  (params (UnpossessedPawn :type "Pawn Object Reference"))
  (bind _returnvalue (`BlackboardComponent.GetValueAsObject` (`self.Blackboard`) (`self.TargetActorKeyName`)))
  (`/Engine/EditorBlueprintResources/StandardMacros.IsValid` _returnvalue
    (:`Is Valid`
      (message `/Game/NovaeTerrae/AI/Interfaces/BPI_AgroInterface.RemoveAgroFocus` _returnvalue))))

(event `/Game/NovaeTerrae/AI/Interfaces/BPI_StatusInterface.ApplyStun`
  (params (StunDuration :type "Float (double-precision)"))
  (if (`self.CanBeDisabled`)
    (set `self.CanBeDisabled` false)
    (`self.SetCurrentState` "NewEnumerator3")
    (`KismetSystemLibrary.Delay` StunDuration)
    (bind _state (`self.GetCurrentState`))
    (if (`|EnumInequality` _state "NewEnumerator4")
      (`self.SetCurrentState` "NewEnumerator1")
      (`KismetSystemLibrary.Delay` (`self.DisableImmuneDuration`))
      (set `self.CanBeDisabled` true))))

(fn `AISafeGetLocation`
  (params (Location :type "Vector Structure"))
  (returns (ResultLocation :type "Vector Structure"))
  (if (`AIBlueprintHelperLibrary.IsValidAILocation` Location)
    (return (`local.Location`))
    (else
      (return (`NavigationSystemV1.K2_GetRandomReachablePointInRadius` (`local.Location`) 200.0 null null)))))

(fn `BaseHandleDamageSense`
  (params (Stimulus :type "AIStimulus Structure"))
  (bind (_age _expirationage _strength _stimuluslocation _receiverlocation _tag _bsuccessfullysensed) (break `AIStimulus` (`local.Stimulus`)))
  (bind _resultlocation (`self.AISafeGetLocation` _stimuluslocation))
  (bind _returnvalue (`AIPerceptionSystem.GetSenseClassForStimulus` Stimulus))
  (if (== _returnvalue "/Script/AIModule.AISense_Damage")
    (if _bsuccessfullysensed
      (bind _state (`self.GetCurrentState`))
      (switch `/Game/NovaeTerrae/AI/Enums/E_EnemyState` _state
        (:`NewEnumerator0`
          (`self.SetStateAsInvestigating` _resultlocation))
        (:`NewEnumerator2`
          (`self.SetStateAsDistracted` _resultlocation))))))

(fn `BaseHandleHearingSense`
  (params (Stimulus :type "AIStimulus Structure"))
  (bind (_age _expirationage _strength _stimuluslocation _receiverlocation _tag _bsuccessfullysensed) (break `AIStimulus` (`local.Stimulus`)))
  (bind _resultlocation (`self.AISafeGetLocation` _stimuluslocation))
  (bind _returnvalue (`AIPerceptionSystem.GetSenseClassForStimulus` Stimulus))
  (if (== _returnvalue "/Script/AIModule.AISense_Hearing")
    (if _bsuccessfullysensed
      (bind _state (`self.GetCurrentState`))
      (switch `/Game/NovaeTerrae/AI/Enums/E_EnemyState` _state
        (:`NewEnumerator0`
          (`self.SetStateAsInvestigating` _resultlocation :!label _label))
        (:`NewEnumerator2`
          (if (> (`KismetMathLibrary.Vector_Distance` _stimuluslocation _receiverlocation) (`self.NoiseDistanceToRetriggerInvestigation`))
            (goto _label)
            (else
              (`self.SetStateAsDistracted` _resultlocation))))))))

(fn `BaseHandlePredictionSense`
  (params (Stimulus :type "AIStimulus Structure"))
  (bind _returnvalue (`AIPerceptionSystem.GetSenseClassForStimulus` Stimulus))
  (if (== _returnvalue "/Script/AIModule.AISense_Prediction")
    (`BlackboardComponent.SetValueAsVector` (`self.Blackboard`) (`self.TargetLocationKeyName`) (`self.AISafeGetLocation` (`.StimulusLocation` (break `AIStimulus` (`local.Stimulus`)))))))

(fn `BaseHandleSightSense`
  (params (Actor :type "Actor Object Reference") (Stimulus :type "AIStimulus Structure"))
  (bind (_age _expirationage _strength _stimuluslocation _receiverlocation _tag _bsuccessfullysensed) (break `AIStimulus` (`local.Stimulus`)))
  (bind _returnvalue (`AIPerceptionSystem.GetSenseClassForStimulus` Stimulus))
  (if (== _returnvalue "/Script/AIModule.AISense_Sight")
    (if (== (`local.Actor`) (`GameplayStatics.GetPlayerCharacter` 0))
      (bind _state (`self.GetCurrentState`))
      (switch `/Game/NovaeTerrae/AI/Enums/E_EnemyState` _state
        (:`NewEnumerator0`
          (if _bsuccessfullysensed :!label _label
            (`self.SetStateAsAgressive` (`local.Actor`))))
        (:`NewEnumerator1`
          (if (not _bsuccessfullysensed)
            (`BlackboardComponent.SetValueAsObject` (`self.Blackboard`) (`self.TargetActorKeyName`) null)
            (`AISense_Prediction.RequestPawnPredictionEvent` (`self.K2_GetPawn`) (`local.Actor`) 0.2)
            (`self.SetCurrentState` "NewEnumerator2")))
        (:`NewEnumerator6`
          (goto _label))
        (:`NewEnumerator2`
          (goto _label))))))

(fn `DetermineAISightPerceptionViewPoint`
  (returns (OutLocation :type "Vector Structure") (OutRotation :type "Rotator Structure"))
  (bind _returnvalue (`self.K2_GetPawn`))
  (bind (_outlocation _outrotation) (`self.GetActorEyesViewPoint` _returnvalue))
  (`/Engine/EditorBlueprintResources/StandardMacros.IsValid` _returnvalue
    (:`Is Valid`
      (return _outlocation _outrotation))))

(fn `GetCurrentState`
  (returns (State :type "/Game/NovaeTerrae/AI/Enums/E_EnemyState Enum"))
  (return (cast `/Game/NovaeTerrae/AI/Enums/E_EnemyState` (`BlackboardComponent.GetValueAsEnum` (`self.Blackboard`) (`self.StateKeyName`)))))

(fn `ReportReceivedDamage`
  (params (Damager :type "Actor Object Reference") (Damage :type "Float (double-precision)") (ByDamageCauser :type Boolean))
  (if (or (== (`local.Damager`) (`GameplayStatics.GetPlayerCharacter` 0)) (and (`GameplayStatics.ObjectIsA` (`local.Damager`) "/Game/NovaeTerrae/AI/Blueprints/BP_WeakPoint.BP_WeakPoint_C") (`local.ByDamageCauser`)))
    (`AISense_Damage.ReportDamageEvent` self (`local.Damager`) (`local.Damage`) (`self.K2_GetActorLocation` (`local.Damager`)))))

(fn `SetCurrentState`
  (params (State :type "/Game/NovaeTerrae/AI/Enums/E_EnemyState Enum" :default "NewEnumerator0"))
  (bind _state (`local.State`))
  (bind _returnvalue (`BlackboardComponent.GetValueAsObject` (`self.Blackboard`) (`self.TargetActorKeyName`)))
  (bind _returnvalue_2 (`BlackboardComponent.GetValueAsObject` (`self.Blackboard`) (`self.TargetActorKeyName`)))
  (`BlackboardComponent.SetValueAsEnum` (`self.Blackboard`) (`self.StateKeyName`) State)
  (`self.OnStateUpdated` _state)
  (switch `/Game/NovaeTerrae/AI/Enums/E_EnemyState` _state
    (:`NewEnumerator0`
      (`/Engine/EditorBlueprintResources/StandardMacros.IsValid` _returnvalue_2 :!label _label
        (:`Is Valid`
          (message `/Game/NovaeTerrae/AI/Interfaces/BPI_AgroInterface.RemoveAgroFocus` _returnvalue_2))))
    (:`NewEnumerator1`
      (`/Engine/EditorBlueprintResources/StandardMacros.IsValid` _returnvalue
        (:`Is Valid`
          (message `/Game/NovaeTerrae/AI/Interfaces/BPI_AgroInterface.ReportAgroFocus` _returnvalue))))
    (:`NewEnumerator4`
      (set `self.CanBeDisabled` false)
      (goto _label))))

(fn `SetStateAsAgressive`
  (params (Actor :type "Actor Object Reference"))
  (`BlackboardComponent.SetValueAsObject` (`self.Blackboard`) (`self.TargetActorKeyName`) (`local.Actor`))
  (`self.SetCurrentState` "NewEnumerator1"))

(fn `SetStateAsAlerted`
  (params (Actor :type "Actor Object Reference"))
  (`BlackboardComponent.SetValueAsObject` (`self.Blackboard`) (`self.TargetActorKeyName`) (`local.Actor`))
  (`self.SetCurrentState` "NewEnumerator7"))

(fn `SetStateAsDistracted`
  (params (Location :type "Vector Structure"))
  (`BlackboardComponent.SetValueAsVector` (`self.Blackboard`) (`self.DistractionLocationKeyName`) (`local.Location`))
  (`self.SetCurrentState` "NewEnumerator6"))

(fn `SetStateAsInvestigating`
  (params (Location :type "Vector Structure"))
  (`BlackboardComponent.SetValueAsVector` (`self.Blackboard`) (`self.TargetLocationKeyName`) (`local.Location`))
  (`self.SetCurrentState` "NewEnumerator2"))

(fn `UserConstructionScript`)