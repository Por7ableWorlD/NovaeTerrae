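; AI controller for the companion that follows the player, driven by BT_Companion.
; On BeginPlay it requires a BP_NTBaseCharacter player, caches all points of interest, starts the tree and seeds its blackboard with the player and follow distance.
; TryScan sets the Scanning key behind a one-second cooldown.
; Its binding to the character's scan request is disconnected, so nothing here triggers it.
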(event `self.ReceiveBeginPlay`
  (bind _returnvalue (`AIBlueprintHelperLibrary.GetBlackboard` null))
  (bind _asbp_ntbase_character (cast `/Game/NovaeTerrae/Core/Characters/Base/BP_NTBaseCharacter` (`GameplayStatics.GetPlayerCharacter` 0)))
  (bind _outactors (`GameplayStatics.GetAllActorsOfClass` "/Game/NovaeTerrae/AI/Environment/BP_PointOfInterest.BP_PointOfInterest_C"))
  (set `self.PointsOfInterest` _outactors)
  (`self.RunBehaviorTree` "/Game/NovaeTerrae/AI/Companion/BT_Companion.BT_Companion")
  (`BlackboardComponent.SetValueAsObject` _returnvalue "Player" (`GameplayStatics.GetPlayerCharacter` 0))
  (`BlackboardComponent.SetValueAsFloat` _returnvalue "StartFollowingDistance" 150.0))

(event `TryScan`
  (if (`self.CanScan`)
    (set `self.CanScan` false)
    (`BlackboardComponent.SetValueAsBool` (`AIBlueprintHelperLibrary.GetBlackboard` null) "Scanning" true)
    (`KismetSystemLibrary.Delay` 1.0)
    (set `self.CanScan` true)))

(fn `UserConstructionScript`)