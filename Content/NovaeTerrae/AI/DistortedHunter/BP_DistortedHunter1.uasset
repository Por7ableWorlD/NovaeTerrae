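; Enemy character Blueprint for the Distorted Hunter, an AI creature with melee and projectile attacks.
; On BeginPlay it loads health, attack ranges, cooldown and damage from DT_DistortedHunter into itself and the Blackboard, and stores its spawn point.
; Five child-actor weak points offset 95% body damage resistance; destroying one plays a stun montage while switching AI state.
; Request functions supply attack data, and death removes weak points and health bar.
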(event `self.ReceiveBeginPlay`
  (`self.PrepareParametersFromDatatable`)
  (bind _asbp_base_enemy_contoller (cast `/Game/NovaeTerrae/AI/BP_BaseEnemyContoller` (`AIBlueprintHelperLibrary.GetAIController` self)))
  (set `self.AIController` _asbp_base_enemy_contoller)
  (`BlackboardComponent.SetValueAsVector` (`AIBlueprintHelperLibrary.GetBlackboard` (`self.AIController`)) "BasePoint" (`self.K2_GetActorLocation`))
  (bind _asbp_weak_point (cast `/Game/NovaeTerrae/AI/Blueprints/BP_WeakPoint` (`ChildActorComponent.ChildActor` (`self.WeakPoint1`))))
  (`NTWeakPoint.SetParameters` _asbp_weak_point 20.0 25.0 15.0)
  (add `NTWeakPoint.OnWeakPointDestroyed` _asbp_weak_point (delegate `WeakPoint1Destroyed`))
  (bind _asbp_weak_point_2 (cast `/Game/NovaeTerrae/AI/Blueprints/BP_WeakPoint` (`ChildActorComponent.ChildActor` (`self.WeakPoint2`))))
  (`NTWeakPoint.SetParameters` _asbp_weak_point_2 20.0 25.0 15.0)
  (add `NTWeakPoint.OnWeakPointDestroyed` _asbp_weak_point_2 (delegate `WeakPoint2Destroyed`))
  (bind _asbp_weak_point_3 (cast `/Game/NovaeTerrae/AI/Blueprints/BP_WeakPoint` (`ChildActorComponent.ChildActor` (`self.WeakPoint3`))))
  (`NTWeakPoint.SetParameters` _asbp_weak_point_3 50.0 50.0 30.0)
  (add `NTWeakPoint.OnWeakPointDestroyed` _asbp_weak_point_3 (delegate `WeakPoint3Destroyed`))
  (bind _asbp_weak_point_4 (cast `/Game/NovaeTerrae/AI/Blueprints/BP_WeakPoint` (`ChildActorComponent.ChildActor` (`self.WeakPoint4`))))
  (`NTWeakPoint.SetParameters` _asbp_weak_point_4 50.0 50.0 30.0)
  (add `NTWeakPoint.OnWeakPointDestroyed` _asbp_weak_point_4 (delegate `WeakPoint4Destroyed`))
  (bind _asbp_weak_point_5 (cast `/Game/NovaeTerrae/AI/Blueprints/BP_WeakPoint` (`ChildActorComponent.ChildActor` (`self.WeakPoint5`))))
  (`NTWeakPoint.SetParameters` _asbp_weak_point_5 70.0 50.0 40.0)
  (add `NTWeakPoint.OnWeakPointDestroyed` _asbp_weak_point_5 (delegate `WeakPoint5Destroyed`))
  (add `self.OnTakeAnyDamage` (delegate `UpdateHealthBar`))
  (bind _aswbp_health_bar_widget (cast `/Game/NovaeTerrae/UI/WBP_HealthBarWidget` (`WidgetComponent.GetUserWidgetObject` (`self.HealthBar`))))
  (bind _output_get (set `self.HealthWidget` _aswbp_health_bar_widget))
  (set `/Game/NovaeTerrae/UI/WBP_HealthBarWidget.Health` 1.0 _output_get)
  (add `NTHealthComponent.OnDeath` (`self.HealthComponent`) (delegate `ClearWeakPointsAndHP`))
  (set `NTEnemyHealthComponent.DamageResistancePercentage` 95.0 (`self.HealthComponent`))
  (`Widget.SetVisibility` (`self.HealthWidget`) "Hidden"))

(event `UpdateHealthBar` :!signature `self.OnTakeAnyDamage`
  (params (DamagedActor :type "Actor Object Reference") (Damage :type "Float (single-precision)") (DamageType :type "DamageType Object Reference") (InstigatedBy :type "Controller Object Reference") (DamageCauser :type "Actor Object Reference"))
  (bind _healthcomponent (`self.HealthComponent`))
  (set `/Game/NovaeTerrae/UI/WBP_HealthBarWidget.Health` (/ (`NTHealthComponent.GetCurrentHealth` _healthcomponent) (`NTHealthComponent.GetMaxHealth` _healthcomponent)) (`self.HealthWidget`)))

(event `ClearWeakPointsAndHP`
  (params (DeathCauser :type "Actor Object Reference"))
  (`self.ClearComponents`))

(event `WeakPoint1Destroyed`
  (`self.AddStun` "/Game/NovaeTerrae/Art/Enemy/Tiger/Anim/AM_TigerMale_DamageLow.AM_TigerMale_DamageLow"))

(event `WeakPoint2Destroyed`
  (`self.AddStun` "/Game/NovaeTerrae/Art/Enemy/Tiger/Anim/AM_TigerMale_DamageLow.AM_TigerMale_DamageLow"))

(event `WeakPoint3Destroyed`
  (`self.AddStun` "/Game/NovaeTerrae/Art/Enemy/Tiger/Anim/AM_TigerMale_DamageLow.AM_TigerMale_DamageLow"))

(event `WeakPoint4Destroyed`
  (`self.AddStun` "/Game/NovaeTerrae/Art/Enemy/Tiger/Anim/AM_TigerMale_DamageLow.AM_TigerMale_DamageLow"))

(event `WeakPoint5Destroyed`
  (`self.AddStun` "/Game/NovaeTerrae/Art/Enemy/Tiger/Anim/AM_TigerMale_DamageHeavy.AM_TigerMale_DamageHeavy"))

(event `self.ReceiveTick`
  (params (DeltaSeconds :type "Float (single-precision)")))

(event `AddStun`
  (params (MontageToPlay :type "AnimMontage Object Reference"))
  (`/Engine/EditorBlueprintResources/StandardMacros.IsValid` MontageToPlay
    (:`Is Valid`
      (bind _aicontroller (`self.AIController`)
        (:`then`
          (`/Game/NovaeTerrae/AI/BP_BaseEnemyContoller.SetCurrentState` _aicontroller "NewEnumerator3")
          (bind _returnvalue (`self.PlayAnimMontage` MontageToPlay))
          (`KismetSystemLibrary.Delay` _returnvalue)
          (bind _aicontroller_2 (`self.AIController`)
            (:`then`
              (`/Game/NovaeTerrae/AI/BP_BaseEnemyContoller.SetCurrentState` _aicontroller_2 "NewEnumerator1"))
            (:`else`)))
        (:`else`)))))

(fn `ClearComponents`
  (`ActorComponent.K2_DestroyComponent` (`self.WeakPoint1`))
  (`ActorComponent.K2_DestroyComponent` (`self.WeakPoint2`))
  (`ActorComponent.K2_DestroyComponent` (`self.WeakPoint3`))
  (`ActorComponent.K2_DestroyComponent` (`self.WeakPoint4`))
  (`ActorComponent.K2_DestroyComponent` (`self.WeakPoint5`))
  (`ActorComponent.K2_DestroyComponent` (`self.HealthBar`)))

(fn `GetMovementSpeed`
  (params (`Movement Speed` :type "/Game/NovaeTerrae/AI/Enums/E_MovementSpeed Enum" :default "NewEnumerator0"))
  (returns (Speed :type "Float (double-precision)"))
  (return (select `/Game/NovaeTerrae/AI/Enums/E_MovementSpeed` `Movement Speed` :`NewEnumerator1` 100.0 :`NewEnumerator2` 150.0 :`NewEnumerator3` 1000.0 :`NewEnumerator6` 2500.0)))

(fn `PrepareParametersFromDatatable`
  (locals (Blackboard :type "BlackboardComponent Object Reference"))
  (set `local.Blackboard` (`AIBlueprintHelperLibrary.GetBlackboard` (`AIBlueprintHelperLibrary.GetAIController` self)))
  (bind _returnvalue (`|GetDataTableRow` "/Game/NovaeTerrae/AI/DataTables/DT_DistortedHunter.DT_DistortedHunter" (`self.RowName`))
    (:`then`
      (`NTEnemyHealthComponent.SetDefaultMaxHealth` (`self.HealthComponent`) (break `/Game/NovaeTerrae/AI/DataTables/S_DistortedHunter` _returnvalue))
      (`BlackboardComponent.SetValueAsFloat` (`local.Blackboard`) "AttackDistance" (`.AttackDistance_10_0868FFA5414631E3167784B190C0E6A5` (break `/Game/NovaeTerrae/AI/DataTables/S_DistortedHunter` _returnvalue)))
      (`BlackboardComponent.SetValueAsFloat` (`local.Blackboard`) "CloseRangeAttackRadius" (`.CloseRangeAttackRadius_4_E4FCCB4C49DB1519E21B229E06018BB1` (break `/Game/NovaeTerrae/AI/DataTables/S_DistortedHunter` _returnvalue)))
      (`BlackboardComponent.SetValueAsFloat` (`local.Blackboard`) "MediumRangeAttackRadius" (`.MediumRangeAttackRadius_6_D87E924941D83691CAB713B1ACEBBE68` (break `/Game/NovaeTerrae/AI/DataTables/S_DistortedHunter` _returnvalue)))
      (`BlackboardComponent.SetValueAsFloat` (`local.Blackboard`) "LongRangeAttackRadius" (`.LongRangeAttackRadius_8_0C594B3A4A34AA185AEE9F872B3EEF51` (break `/Game/NovaeTerrae/AI/DataTables/S_DistortedHunter` _returnvalue)))
      (`BlackboardComponent.SetValueAsFloat` (`local.Blackboard`) "AttackCooldown" (`.AttackCooldown_12_2D66234049DAC758EE8457AC6E285171` (break `/Game/NovaeTerrae/AI/DataTables/S_DistortedHunter` _returnvalue)))
      (set `self.MeleeLightDamage` (`.LightMeleeAttackDamage_17_FDE30B6847C952ABA5CDFDA196982DDB` (break `/Game/NovaeTerrae/AI/DataTables/S_DistortedHunter` _returnvalue)))
      (set `self.MeleeHeavyDamage` (`.HeavyMeleeAttackDamage_18_1530E6E241DCE4944F50D5B9CD3FFB77` (break `/Game/NovaeTerrae/AI/DataTables/S_DistortedHunter` _returnvalue)))
      (set `self.ProjectileDamage` (`.RangeAttackDamage_20_0A47DAB44EF62C0949A4AEA750E55A04` (break `/Game/NovaeTerrae/AI/DataTables/S_DistortedHunter` _returnvalue))))))

(fn `RequestDamageZone`
  (params (AttackName :type Name))
  (returns (DamageZone :type "PrimitiveComponent Object Reference"))
  (bind _damagezone (`/Game/NovaeTerrae/AI/Interfaces/BPI_CombatInterface.RequestDataForMeleeAttack` AttackName))
  (return _damagezone))

(fn `RequestDataForMeleeAttack`
  (params (AttackName :type Name))
  (returns (DamageZone :type "PrimitiveComponent Object Reference") (Damage :type "Float (double-precision)") (AttackMontage :type "AnimMontage Object Reference"))
  (if (== AttackName "Light_1")
    (return (`self.LightAttackSphere`) (`self.MeleeLightDamage`) "/Game/NovaeTerrae/Art/Enemy/Tiger/Anim/AM_TigerMale_AttackLow.AM_TigerMale_AttackLow")
    (elif (== AttackName "Light_2")
      (return (`self.LightAttackSphere`) (`self.MeleeLightDamage`) "/Game/NovaeTerrae/Art/Enemy/Tiger/Anim/AM_TigerMale_AttackLow2.AM_TigerMale_AttackLow2")
      (elif (== AttackName "Heavy")
        (return (`self.HeavyAttackSphere`) (`self.MeleeHeavyDamage`) "/Game/NovaeTerrae/Art/Enemy/Tiger/Anim/AM_TigerMale_AttackHeavy.AM_TigerMale_AttackHeavy")))))

(fn `RequestDataForProjectileAttack`
  (returns (LaunchTransform :type "Transform Structure") (Damage :type "Float (double-precision)"))
  (return (`SceneComponent.K2_GetComponentToWorld` (`self.ShootArrow`)) (`self.ProjectileDamage`)))

(fn `RequestHealthBarWidget`
  (returns (HealthWidget :type "/Game/NovaeTerrae/UI/WBP_HealthBarWidget Object Reference"))
  (return (`self.HealthWidget`)))

(fn `UserConstructionScript`)