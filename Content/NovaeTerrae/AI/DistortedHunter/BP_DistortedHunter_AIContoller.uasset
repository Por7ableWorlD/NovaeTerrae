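; AI controller for the Distorted Hunter that starts its behavior tree on BeginPlay and reacts to AI Perception updates.
; Each update passes through sight and damage handlers, which switch the hunter from Passive to Alerted and ignore all other states.
; Sight reacts only to the player character, without checking whether sensing succeeded.
; Successfully sensed damage always alerts on the player, whatever actor was reported.
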(event `self.ReceiveBeginPlay`
  (`self.RunBehaviorTree` "/Game/NovaeTerrae/AI/DistortedHunter/BT_DistortedHunter.BT_DistortedHunter")
  (`parent.ReceiveBeginPlay`))

(event `self.AIPerception.OnTargetPerceptionUpdated`
  (params (Actor :type "Actor Object Reference") (Stimulus :type "AIStimulus Structure"))
  (`self.HandleSightSense` Actor Stimulus)
  (`self.HandleDamageSense` Stimulus))

(fn `HandleDamageSense`
  (params (Stimulus :type "AIStimulus Structure"))
  (bind _returnvalue (`AIPerceptionSystem.GetSenseClassForStimulus` Stimulus))
  (if (== _returnvalue "/Script/AIModule.AISense_Damage")
    (if (`.bSuccessfullySensed` (break `AIStimulus` (`local.Stimulus`)))
      (bind _state (`self.GetCurrentState`))
      (switch `/Game/NovaeTerrae/AI/Enums/E_EnemyState` _state
        (:`NewEnumerator0`
          (`self.SetStateAsAlerted` (`GameplayStatics.GetPlayerCharacter` 0)))))))

(fn `HandleSightSense`
  (params (Actor :type "Actor Object Reference") (Stimulus :type "AIStimulus Structure"))
  (bind _returnvalue (`AIPerceptionSystem.GetSenseClassForStimulus` Stimulus))
  (if (== _returnvalue "/Script/AIModule.AISense_Sight")
    (if (== (`local.Actor`) (`GameplayStatics.GetPlayerCharacter` 0))
      (bind _state (`self.GetCurrentState`))
      (switch `/Game/NovaeTerrae/AI/Enums/E_EnemyState` _state
        (:`NewEnumerator0`
          (`self.SetStateAsAlerted` (`local.Actor`)))))))

(fn `UserConstructionScript`)