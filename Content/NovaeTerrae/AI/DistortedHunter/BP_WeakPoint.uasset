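; Destructible weak point actor, filed under the Distorted Hunter AI, that relays damage it takes to its owner.
; SetParameters supplies the owner and damage tuning, scales the actor and snaps it to a socket on a given component.
; Damage is forwarded with a multiplier, plus bonus damage once its own NTHealth is depleted.
; On depletion it also fires OnWeakPointDestroyed, spawns an explosion effect and destroys itself.
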(event `self.ReceiveBeginPlay`
  (add `self.OnTakeAnyDamage` (delegate `TransferDamage`)))

(event `TransferDamage` :!signature `self.OnTakeAnyDamage`
  (params (DamagedActor :type "Actor Object Reference") (Damage :type "Float (single-precision)") (DamageType :type "DamageType Object Reference") (InstigatedBy :type "Controller Object Reference") (DamageCauser :type "Actor Object Reference"))
  (bind (_returnvalue_location _returnvalue_rotation _returnvalue_scale) (`KismetMathLibrary.BreakTransform` (`self.GetTransform`)))
  (bind _returnvalue (* Damage (`self.DamageModifier`)))
  (bind _returnvalue_2 (> (`NTHealthComponent.GetCurrentHealth` (`self.NTHealth`)) 0.0))
  (`GameplayStatics.ApplyDamage` (`self.OwnerRef`) (`KismetMathLibrary.SelectFloat` _returnvalue (+ _returnvalue (`self.DeathAdditionalDamage`)) _returnvalue_2) null self)
  (if (not _returnvalue_2)
    (`self.OnWeakPointDestroyed`)
    (`NiagaraFunctionLibrary.SpawnSystemAtLocation` "/Game/NovaeTerrae/Art/VFX/NS_Explosion_eyes.NS_Explosion_eyes" _returnvalue_location _returnvalue_rotation _returnvalue_scale)
    (`self.K2_DestroyActor`)))

(event `SetParameters`
  (params (DamageModifier :type "Float (double-precision)") (DeathAdditionalDamage :type "Float (double-precision)") (OwnerRef :type "Character Object Reference") (Component :type "SceneComponent Object Reference") (Scale :type "Vector Structure") (SocketName :type Name))
  (set `self.DamageModifier` DamageModifier)
  (set `self.DeathAdditionalDamage` DeathAdditionalDamage)
  (set `self.OwnerRef` OwnerRef)
  (`self.SetActorScale3D` Scale)
  (`self.K2_AttachToComponent` Component SocketName "SnapToTarget" "KeepRelative" "KeepWorld"))

(fn `UserConstructionScript`)