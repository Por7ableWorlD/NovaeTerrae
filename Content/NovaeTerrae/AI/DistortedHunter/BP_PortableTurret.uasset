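; Portable AI turret for the Distorted Hunter enemy that tracks an assigned TargetActor and shoots projectiles at it.
; Tick turns the head mesh at constant speed with clamped pitch toward the target.
; When a sphere trace finds no obstruction and a dot-product check confirms tight aim, it spawns BP_Projectile, plays a shot sound and starts a cooldown timer.
; On death, the head droops to its lower pitch limit, then actor tick is disabled.
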(event `self.ReceiveBeginPlay`)

(event `self.ReceiveTick`
  (params (DeltaSeconds :type "Float (single-precision)"))
  (bind (_returnvalue_roll _returnvalue_pitch _returnvalue_yaw) (`KismetMathLibrary.BreakRotator` (`SceneComponent.K2_GetComponentRotation` (`self.StaticMesh1`))))
  (bind (_returnvalue_roll_2 _returnvalue_pitch_2) (`KismetMathLibrary.BreakRotator` (`KismetMathLibrary.NormalizedDeltaRotator` (struct :`Pitch` -50.0) (`KismetMathLibrary.MakeRotator` 0.0 _returnvalue_pitch))))
  (if (`NTHealthComponent.IsDead` (`self.NTEnemyHealth`))
    (`self.SetRotation` (`KismetMathLibrary.MakeRotator` _returnvalue_roll -50.0 _returnvalue_yaw) DeltaSeconds)
    (if (< (`KismetMathLibrary.Abs` _returnvalue_pitch_2) 0.1)
      (`self.SetActorTickEnabled` false))
    (else
      (`self.TargetActor`
        (:`then`
          (`self.UpdateTurretRotation` DeltaSeconds)
          (if (`self.CanFire`)
            (`self.UpdateFire`)))
        (:`else`)))))

(event `Fire`
  (bind _staticmesh2 (`self.StaticMesh2`))
  (set `self.CanFire` false)
  (`|SpawnActorFromClass` "/Game/NovaeTerrae/AI/Blueprints/BP_Projectile.BP_Projectile_C" (`KismetMathLibrary.MakeTransform` (`SceneComponent.GetSocketLocation` _staticmesh2 "ProjectileSocket") (`SceneComponent.K2_GetComponentRotation` _staticmesh2) (0.7 0.7 0.7)) "Undefined" "MultiplyWithRoot" null (`self.BulletDamage`) (`self.DamageRadius`) self)
  (`KismetSystemLibrary.K2_SetTimerDelegate` (delegate `ResetFire`) (`self.FireCooldown`)))

(event `ResetFire`
  (set `self.CanFire` true))

(fn `SetRotation`
  (params (TargetAngle :type "Rotator Structure") (DeltaSeconds :type "Float (double-precision)"))
  (bind (_returnvalue_roll _returnvalue_pitch _returnvalue_yaw) (`KismetMathLibrary.BreakRotator` (`KismetMathLibrary.RInterpTo_Constant` (`SceneComponent.K2_GetComponentRotation` (`self.StaticMesh1`)) TargetAngle DeltaSeconds (`self.RotationSpeed`))))
  (`SceneComponent.K2_SetWorldRotation` (`self.StaticMesh1`) (`KismetMathLibrary.MakeRotator` _returnvalue_roll (`KismetMathLibrary.ClampAngle` _returnvalue_pitch -50.0 80.0) _returnvalue_yaw) false false))

(fn `UpdateFire`
  (bind _returnvalue (`self.K2_GetActorLocation` (`self.TargetActor`)))
  (bind _returnvalue_2 (`SceneComponent.K2_GetComponentLocation` (`self.StaticMesh1`)))
  (bind (_outhit _returnvalue_3) (`KismetSystemLibrary.SphereTraceSingle` _returnvalue_2 _returnvalue 30.0 "TraceTypeQuery1"))
  (if (and (not _returnvalue_3) (> (`KismetMathLibrary.Dot_VectorVector` (`KismetMathLibrary.GetDirectionUnitVector` _returnvalue_2 _returnvalue) (`SceneComponent.GetForwardVector` (`self.StaticMesh1`))) 0.99))
    (`self.Fire`)
    (`FMODBlueprintStatics.PlayEventAttached` "/Game/FMOD/Events/Enemies/Tiger/EnTigerWepShotNm.EnTigerWepShotNm" (`self.StaticMesh`) "None" (0.0 0.0 0.0) "KeepRelativeOffset")))

(fn `UpdateTurretRotation`
  (params (DeltaSeconds :type "Float (double-precision)"))
  (locals (TargetAngle :type "Rotator Structure"))
  (`self.SetRotation` (`KismetMathLibrary.FindLookAtRotation` (`SceneComponent.K2_GetComponentLocation` (`self.StaticMesh1`)) (`self.K2_GetActorLocation` (`self.TargetActor`))) DeltaSeconds))

(fn `UserConstructionScript`)