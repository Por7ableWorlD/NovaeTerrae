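; AI-controlled turret sentinel that fires projectiles with random spread from a socket on its mesh.
; On BeginPlay a data table row sets health and bullet damage, and feeds attack timings, bullet count and the rotating mesh to the Blackboard.
; Query functions supply sight and projectile data; melee and other queries are stubs.
; On death Tick droops the mesh at clamped pitch, then disables itself while a looping timer polls for revival.
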(event `self.ReceiveBeginPlay`
  (`self.PrepareParametersFromDatatable`))

(event `self.ReceiveTick`
  (params (DeltaSeconds :type "Float (single-precision)"))
  (bind (_returnvalue_roll _returnvalue_pitch _returnvalue_yaw) (`KismetMathLibrary.BreakRotator` (`SceneComponent.K2_GetComponentRotation` (`self.StaticMesh1`))))
  (bind (_returnvalue_roll_2 _returnvalue_pitch_2) (`KismetMathLibrary.BreakRotator` (`KismetMathLibrary.NormalizedDeltaRotator` (struct :`Pitch` -50.0) (`KismetMathLibrary.MakeRotator` 0.0 _returnvalue_pitch))))
  (if (`NTHealthComponent.IsDead` (`self.HealthComponent`))
    (`self.SetRotation` (`KismetMathLibrary.MakeRotator` _returnvalue_roll -50.0 _returnvalue_yaw) DeltaSeconds)
    (if (< (`KismetMathLibrary.Abs` _returnvalue_pitch_2) 0.1)
      (`self.SetActorTickEnabled` false)
      (`KismetSystemLibrary.K2_SetTimerDelegate` (delegate `Revive`) 0.5 true))))

(event `Revive`
  (if (not (`NTHealthComponent.IsDead` (`self.HealthComponent`)))
    (`self.SetActorTickEnabled` true)))

(fn `GetSightTransform`
  (returns (SightTransform :type "Transform Structure"))
  (return (`SceneComponent.K2_GetComponentToWorld` (`self.StaticMesh1`))))

(fn `PrepareParametersFromDatatable`
  (locals (Blackboard :type "BlackboardComponent Object Reference"))
  (set `local.Blackboard` (`AIBlueprintHelperLibrary.GetBlackboard` (`AIBlueprintHelperLibrary.GetAIController` self)))
  (bind _returnvalue (`|GetDataTableRow` "/Game/NovaeTerrae/AI/DataTables/DT_TurretSentinel.DT_TurretSentinel" (`self.DataTableRowName`))
    (:`then`
      (`NTEnemyHealthComponent.SetDefaultMaxHealth` (`self.HealthComponent`) (break `/Game/NovaeTerrae/AI/DataTables/S_TurretSentinel` _returnvalue))
      (set `self.BulletDamage` (`.BulletDamage_4_D77972EF4352B75E3D5D98ADFF223650` (break `/Game/NovaeTerrae/AI/DataTables/S_TurretSentinel` _returnvalue)))
      (`BlackboardComponent.SetValueAsFloat` (`local.Blackboard`) "AttackCooldown" (`.AttackCooldown_6_9BC1498A4A093E6495224D924EBC0C79` (break `/Game/NovaeTerrae/AI/DataTables/S_TurretSentinel` _returnvalue)))
      (`BlackboardComponent.SetValueAsFloat` (`local.Blackboard`) "FiringRate" (`.FiringRate_9_FC6D85A8438E88A2C68DC9829E8DBEEF` (break `/Game/NovaeTerrae/AI/DataTables/S_TurretSentinel` _returnvalue)))
      (`BlackboardComponent.SetValueAsInt` (`local.Blackboard`) "NumberOfBullets" (`.NumberOfBullets_12_5FBF2A2B480A432F38472BABEA023340` (break `/Game/NovaeTerrae/AI/DataTables/S_TurretSentinel` _returnvalue)))
      (`BlackboardComponent.SetValueAsObject` (`local.Blackboard`) "RotatingPart" (`self.StaticMesh1`))
      (`BlackboardComponent.SetValueAsFloat` (`local.Blackboard`) "TimeUntilBecomePassive" (`.TimeUntilBecomePassive_15_8AA0430C4282EF581F165E8E54CA6026` (break `/Game/NovaeTerrae/AI/DataTables/S_TurretSentinel` _returnvalue))))))

(fn `RequestDamageZone`
  (params (AttackName :type Name))
  (returns (DamageZone :type "PrimitiveComponent Object Reference"))
  (return null))

(fn `RequestDataForMeleeAttack`
  (params (AttackName :type Name))
  (returns (DamageZone :type "PrimitiveComponent Object Reference") (Damage :type "Float (double-precision)") (AttackMontage :type "AnimMontage Object Reference"))
  (return null 0.0 null))

(fn `RequestDataForProjectileAttack`
  (returns (LaunchTransform :type "Transform Structure") (Damage :type "Float (double-precision)"))
  (bind _returnvalue (`KismetMathLibrary.RandomFloatInRange` -5.0 5.0))
  (bind _staticmesh2 (`self.StaticMesh2`))
  (bind (_returnvalue_roll _returnvalue_pitch _returnvalue_yaw) (`KismetMathLibrary.BreakRotator` (`SceneComponent.K2_GetComponentRotation` _staticmesh2)))
  (return (`KismetMathLibrary.MakeTransform` (`SceneComponent.GetSocketLocation` _staticmesh2 "ProjectileSocket") (`KismetMathLibrary.MakeRotator` _returnvalue_roll (+ _returnvalue_pitch _returnvalue) (+ _returnvalue_yaw _returnvalue)) (0.3 0.3 0.3)) (`self.BulletDamage`)))

(fn `RequestFiringSocketLocation`
  (returns (SocketLocation :type "Vector Structure"))
  (return (0.0 0.0 0.0)))

(fn `RequestHealthBarWidget`
  (returns (HealthWidget :type "/Game/NovaeTerrae/UI/WBP_HealthBarWidget Object Reference"))
  (return null))

(fn `SetRotation`
  (params (TargetAngle :type "Rotator Structure") (DeltaSeconds :type "Float (double-precision)"))
  (bind (_returnvalue_roll _returnvalue_pitch _returnvalue_yaw) (`KismetMathLibrary.BreakRotator` (`KismetMathLibrary.RInterpTo_Constant` (`SceneComponent.K2_GetComponentRotation` (`self.StaticMesh1`)) TargetAngle DeltaSeconds (`self.RotationSpeed`))))
  (`SceneComponent.K2_SetWorldRotation` (`self.StaticMesh1`) (`KismetMathLibrary.MakeRotator` _returnvalue_roll (`KismetMathLibrary.ClampAngle` _returnvalue_pitch -50.0 80.0) _returnvalue_yaw) false false))

(fn `UserConstructionScript`)