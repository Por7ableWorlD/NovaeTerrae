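; AI controller for the Turret Sentinel that runs its behavior tree and reacts to perception updates.
; Sighting the player turns it aggressive; while aggressive, losing sight swaps the Blackboard target actor for the last stimulus location.
; Hearing and damage stimuli go to base handlers, while ClearAgressiveState is left empty.
; The sight viewpoint comes from the controlled pawn via a GetSightTransformMessage call.
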(event `self.ReceiveBeginPlay`
  (`self.RunBehaviorTree` "/Game/NovaeTerrae/AI/TurretSentinel/BT_TurretSentinel.BT_TurretSentinel")
  (`parent.ReceiveBeginPlay`))

(event `self.AIPerception.OnTargetPerceptionUpdated`
  (params (Actor :type "Actor Object Reference") (Stimulus :type "AIStimulus Structure"))
  (`self.HandleSightSense` Actor Stimulus)
  (`self.BaseHandleHearingSense` Stimulus)
  (`self.BaseHandleDamageSense` Stimulus))

(fn `ClearAgressiveState`)

(fn `DetermineAISightPerceptionViewPoint`
  (returns (OutLocation :type "Vector Structure") (OutRotation :type "Rotator Structure"))
  (bind _sighttransform (message `/Game/NovaeTerrae/AI/Interfaces/BPI_CustomSightLocationInterface.GetSightTransform` (`self.K2_GetPawn`)))
  (return (.location _sighttransform) (.rotation _sighttransform)))

(fn `HandleSightSense`
  (params (Actor :type "Actor Object Reference") (Stimulus :type "AIStimulus Structure"))
  (bind (_age _expirationage _strength _stimuluslocation _receiverlocation _tag _bsuccessfullysensed) (break `AIStimulus` (`local.Stimulus`)))
  (bind _returnvalue (`AIPerceptionSystem.GetSenseClassForStimulus` Stimulus))
  (if (== _returnvalue "/Script/AIModule.AISense_Sight")
    (if (== (`local.Actor`) (`GameplayStatics.GetPlayerCharacter` 0))
      (bind _state (`self.GetCurrentState`))
      (switch `/Game/NovaeTerrae/AI/Enums/E_EnemyState` _state
        (:`NewEnumerator0`
          (if _bsuccessfullysensed :!label _label
            (`self.SetStateAsAgressive` (`local.Actor`))))
        (:`NewEnumerator1`
          (if (not _bsuccessfullysensed)
            (`BlackboardComponent.SetValueAsObject` (`self.Blackboard`) (`self.TargetActorKeyName`) null)
            (`BlackboardComponent.SetValueAsVector` (`self.Blackboard`) (`self.TargetLocationKeyName`) _stimuluslocation)
            (else
              (`BlackboardComponent.SetValueAsObject` (`self.Blackboard`) (`self.TargetActorKeyName`) (`local.Actor`)))))
        (:`NewEnumerator6`
          (goto _label))
        (:`NewEnumerator2`
          (goto _label))))))

(fn `UserConstructionScript`
  (`parent.UserConstructionScript`))