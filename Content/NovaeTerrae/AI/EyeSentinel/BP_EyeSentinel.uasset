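; Eye Sentinel AI enemy with a laser attack, configured from the DefaultSettings row of DT_EyeSentinel.
; On BeginPlay it sets max health and a strafe threshold on its HealthComponent and writes attack and laser tuning to the Blackboard, deriving the engage radius from attack radius.
; It also passes its SplineComponent to the Blackboard.
; GetMovementSpeed maps movement states to fixed speeds.
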(event `self.ReceiveTick`
  (params (DeltaSeconds :type "Float (single-precision)")))

(event `self.ReceiveBeginPlay`
  (`self.PrepareParametersFromDatatable`)
  (`BlackboardComponent.SetValueAsObject` (`AIBlueprintHelperLibrary.GetBlackboard` (`AIBlueprintHelperLibrary.GetAIController` self)) "Spline" (`self.SplineComponent`)))

(fn `GetMovementSpeed`
  (params (`Movement Speed` :type "/Game/NovaeTerrae/AI/Enums/E_MovementSpeed Enum" :default "NewEnumerator0"))
  (returns (Speed :type "Float (double-precision)"))
  (return (select `/Game/NovaeTerrae/AI/Enums/E_MovementSpeed` `Movement Speed` :`NewEnumerator1` 200.0 :`NewEnumerator2` 600.0 :`NewEnumerator3` 900.0 :`NewEnumerator6` 2000.0 :!type "Float (single-precision)")))

(fn `PrepareParametersFromDatatable`
  (locals (Blackboard :type "BlackboardComponent Object Reference"))
  (bind _healthcomponent (`self.HealthComponent`))
  (set `local.Blackboard` (`AIBlueprintHelperLibrary.GetBlackboard` (`AIBlueprintHelperLibrary.GetAIController` self)))
  (bind _returnvalue (`|GetDataTableRow` "/Game/NovaeTerrae/AI/DataTables/DT_EyeSentinel.DT_EyeSentinel" "DefaultSettings")
    (:`then`
      (`NTEnemyHealthComponent.SetDefaultMaxHealth` _healthcomponent (break `/Game/NovaeTerrae/AI/DataTables/S_EyeSentinel` _returnvalue))
      (set `NTEnemyHealthComponent.ActionThresholdPercentage` (`.StrafeThresholdPercentage_8_0C0939494758C6CAA879D7B098C75B91` (break `/Game/NovaeTerrae/AI/DataTables/S_EyeSentinel` _returnvalue)) _healthcomponent)
      (`BlackboardComponent.SetValueAsFloat` (`local.Blackboard`) "AttackRadius" (`.AttackRadius_5_95AE91AD406526808A902C8421979AF8` (break `/Game/NovaeTerrae/AI/DataTables/S_EyeSentinel` _returnvalue)))
      (`BlackboardComponent.SetValueAsFloat` (`local.Blackboard`) "LaserTickDamage" (`.LaserTickDamage_11_4E5CD15B45C812EA45400297C65B376F` (break `/Game/NovaeTerrae/AI/DataTables/S_EyeSentinel` _returnvalue)))
      (`BlackboardComponent.SetValueAsFloat` (`local.Blackboard`) "AttackCooldown" (`.AttackCooldown_15_158986B04CE62A4376BD70AF320841AF` (break `/Game/NovaeTerrae/AI/DataTables/S_EyeSentinel` _returnvalue)))
      (`BlackboardComponent.SetValueAsFloat` (`local.Blackboard`) "LaserDuration" (`.LaserDuration_21_7891ACED4141A13D4A14EDA06E4F0628` (break `/Game/NovaeTerrae/AI/DataTables/S_EyeSentinel` _returnvalue)))
      (`BlackboardComponent.SetValueAsFloat` (`local.Blackboard`) "AttackDelay" (`.AttackDelay_24_4E3C36A3484124EDCFDAF5810F4A4062` (break `/Game/NovaeTerrae/AI/DataTables/S_EyeSentinel` _returnvalue)))
      (`BlackboardComponent.SetValueAsFloat` (`local.Blackboard`) "AttackEngageRadius" (- (`.AttackRadius_5_95AE91AD406526808A902C8421979AF8` (break `/Game/NovaeTerrae/AI/DataTables/S_EyeSentinel` _returnvalue)) 300.0)))))

(fn `UserConstructionScript`)