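; AI controller for the Rocket Sentinel enemy, running its behavior tree and turning perception updates into blackboard values.
; Sighting the player sets the target actor and aggressive state and enables the pawn's LAA message.
; Losing sight clears the target, disables that message and requests a short prediction event, whose stimulus writes the predicted position to TargetLocation.
; The aggressive state is never reset here.
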(event `self.ReceiveBeginPlay`
  (`self.RunBehaviorTree` "/Game/NovaeTerrae/AI/RocketSentinel/BT_RocketSentinel.BT_RocketSentinel"))

(event `self.AIPerception.OnTargetPerceptionUpdated`
  (params (Actor :type "Actor Object Reference") (Stimulus :type "AIStimulus Structure"))
  (`self.HandleSightSense` Actor Stimulus)
  (`self.HandlePredictionSense` Stimulus))

(fn `HandlePredictionSense`
  (params (Stimulus :type "AIStimulus Structure"))
  (bind _returnvalue (`AIPerceptionSystem.GetSenseClassForStimulus` Stimulus))
  (if (== _returnvalue "/Script/AIModule.AISense_Prediction")
    (`BlackboardComponent.SetValueAsVector` (`self.Blackboard`) "TargetLocation" (`.StimulusLocation` (break `AIStimulus` (`local.Stimulus`))))))

(fn `HandleSightSense`
  (params (Actor :type "Actor Object Reference") (Stimulus :type "AIStimulus Structure"))
  (bind _returnvalue (`self.K2_GetPawn`))
  (bind (_age _expirationage _strength _stimuluslocation _receiverlocation _tag _bsuccessfullysensed) (break `AIStimulus` (`local.Stimulus`)))
  (bind _returnvalue_2 (`AIPerceptionSystem.GetSenseClassForStimulus` Stimulus))
  (if (== _returnvalue_2 "/Script/AIModule.AISense_Sight")
    (if (== Actor (`GameplayStatics.GetPlayerCharacter` 0))
      (`BlackboardComponent.SetValueAsObject` (`self.Blackboard`) "TargetActor" (`KismetMathLibrary.SelectObject` (`local.Actor`) null _bsuccessfullysensed))
      (if _bsuccessfullysensed
        (message `/Game/NovaeTerrae/AI/BPI_LAAInterface.EnableLAA` _returnvalue)
        (`BlackboardComponent.SetValueAsBool` (`self.Blackboard`) "AgressiveState" true)
        (else
          (message `/Game/NovaeTerrae/AI/BPI_LAAInterface.DisableLAA` _returnvalue)
          (`AISense_Prediction.RequestPawnPredictionEvent` _returnvalue (`local.Actor`) 1.5))))))

(fn `UserConstructionScript`)