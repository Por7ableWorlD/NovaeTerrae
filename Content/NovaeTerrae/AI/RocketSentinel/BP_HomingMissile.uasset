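; BP_HomingMissile is a homing projectile in the RocketSentinel AI folder that explodes on hit, dealing radial damage before destroying itself.
; SetupHomingMissile turns on gravity-free homing in ProjectileMovement, caps its speed and starts a lifetime timer; no homing target is assigned here.
; Despite its name, the timer's MissileExplosion event only enables mesh physics, then destroys the actor after a short delay.
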(event `self.ReceiveBeginPlay`)

(event `self.ReceiveHit`
  (params (MyComp :type "PrimitiveComponent Object Reference") (Other :type "Actor Object Reference") (OtherComp :type "PrimitiveComponent Object Reference") (bSelfMoved :type Boolean) (HitLocation :type "Vector Structure") (HitNormal :type "Vector Structure") (NormalImpulse :type "Vector Structure") (Hit :type "HitResult Structure (by ref)"))
  (bind _returnvalue (`self.K2_GetActorLocation`))
  (`NiagaraFunctionLibrary.SpawnSystemAtLocation` "/Game/NovaeTerrae/Art/VFX/NS_Explosion_eyes.NS_Explosion_eyes" _returnvalue (struct) (1.0 1.0 1.0) true true "AutoRelease")
  (`GameplayStatics.ApplyRadialDamage` :`BaseDamage` 40.0 :`Origin` _returnvalue :`DamageRadius` 300.0 :`DamageTypeClass` "/Script/Engine.DamageType" :`DamageCauser` self :`InstigatedByController` null)
  (`self.K2_DestroyActor`))

(event `SetupHomingMissile`
  (set `ProjectileMovementComponent.bIsHomingProjectile` true (`self.ProjectileMovement`))
  (set `ProjectileMovementComponent.ProjectileGravityScale` 0.0 (`self.ProjectileMovement`))
  (set `ProjectileMovementComponent.MaxSpeed` 1000.0 (`self.ProjectileMovement`))
  (`KismetSystemLibrary.K2_SetTimerDelegate` (delegate `MissileExplosion`) 10.0))

(event `MissileExplosion`
  (`PrimitiveComponent.SetSimulatePhysics` (`self.StaticMesh`) true)
  (`KismetSystemLibrary.Delay` 2.0)
  (`self.K2_DestroyActor`))

(fn `UserConstructionScript`)