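; Rocket Sentinel AI enemy that attacks with missiles in homing or artillery mode.
; After a short BeginPlay delay, it loads stats from a DT_RocketSentinel row into its health component, Blackboard and variables, then stores its BasePoint.
; LaunchMissile spawns a BP_HomingMissile that either tracks the player or lobs toward a random navigable point near TargetLocation using a suggested high-arc velocity, with debug drawing.
; GetRandomNumberOfMissiles picks a count from per-mode ranges.
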(event `self.ReceiveBeginPlay`
  (`KismetSystemLibrary.Delay` 0.5)
  (`self.PrepareParametersFromDatatable`)
  (`BlackboardComponent.SetValueAsVector` (`AIBlueprintHelperLibrary.GetBlackboard` (`AIBlueprintHelperLibrary.GetAIController` self)) "BasePoint" (`self.K2_GetActorLocation`)))

(event `/Game/NovaeTerrae/AI/Interfaces/BPI_LaunchMissileInterface.LaunchMissile`
  (params (HomingMode :type Boolean))
  (bind _returnvalue (`SceneComponent.K2_GetComponentLocation` (`self.MissileSlot`)))
  (if HomingMode
    (bind _returnvalue_2 (`|SpawnActorFromClass` "/Game/NovaeTerrae/AI/Blueprints/BP_HomingMissile.BP_HomingMissile_C" (`KismetMathLibrary.MakeTransform` _returnvalue (`self.K2_GetActorRotation`)) "Undefined" "MultiplyWithRoot" null self))
    (`/Game/NovaeTerrae/AI/Blueprints/BP_HomingMissile.SetupHomingMissile` _returnvalue_2)
    (set `ProjectileMovementComponent.HomingTargetComponent` (`Actor.RootComponent` (`GameplayStatics.GetPlayerCharacter` 0)) (`/Game/NovaeTerrae/AI/Blueprints/BP_HomingMissile.ProjectileMovement` _returnvalue_2))
    (`/Game/NovaeTerrae/AI/Blueprints/BP_HomingMissile.SetupParameters` _returnvalue_2 (`self.MissilesDamage`) (`self.DamageRadius`))
    (else
      (bind _returnvalue_3 (`|SpawnActorFromClass` "/Game/NovaeTerrae/AI/Blueprints/BP_HomingMissile.BP_HomingMissile_C" (`KismetMathLibrary.MakeTransform` _returnvalue (struct :`Pitch` 90.0)) "Undefined" "MultiplyWithRoot" null self))
      (`/Game/NovaeTerrae/AI/Blueprints/BP_HomingMissile.SetupParameters` _returnvalue_3 (`self.MissilesDamage`) (`self.DamageRadius`))
      (bind _randomlocation (`NavigationSystemV1.K2_GetRandomLocationInNavigableRadius` (`BlackboardComponent.GetValueAsVector` (`AIBlueprintHelperLibrary.GetBlackboard` (`AIBlueprintHelperLibrary.GetAIController` self)) "TargetLocation") (`self.ArtilleryBarrageRadius`) null null))
      (`KismetSystemLibrary.DrawDebugSphere` _randomlocation 100.0 12 (struct :`R` 0.347065 :`G` 0.630617 :`B` 1.0 :`A` 1.0) 5.0 3.0)
      (bind (_tossvelocity _returnvalue_4) (`GameplayStatics.BlueprintSuggestProjectileVelocity` _returnvalue _randomlocation 2000.0 0.0 "DoNotTrace" 0.0 true true))
      (if _returnvalue_4
        (bind _result (`/Engine/EditorBlueprintResources/StandardMacros.NegateFloat` (.x _tossvelocity))
          (:`  `
            (`ProjectileMovementComponent.SetVelocityInLocalSpace` (`/Game/NovaeTerrae/AI/Blueprints/BP_HomingMissile.ProjectileMovement` _returnvalue_3) (`KismetMathLibrary.MakeVector` (.z _tossvelocity) (.y _tossvelocity) _result))))))))

(fn `GetRandomNumberOfMissiles`
  (params (HomingMode :type Boolean))
  (returns (NumberOfMissiles :type Integer))
  (return (`KismetMathLibrary.RandomIntegerInRange` (`KismetMathLibrary.SelectInt` (`self.MinMissilesHomingMode`) (`self.MinMissilesArtilleryMode`) HomingMode) (`KismetMathLibrary.SelectInt` (`self.MaxMissilesHomingMode`) (`self.MaxMissilesArtilleryMode`) HomingMode))))

(fn `PrepareParametersFromDatatable`
  (locals (Blackboard :type "BlackboardComponent Object Reference"))
  (bind _healthcomponent (`self.HealthComponent`))
  (set `local.Blackboard` (`AIBlueprintHelperLibrary.GetBlackboard` (`AIBlueprintHelperLibrary.GetAIController` self)))
  (bind _returnvalue (`|GetDataTableRow` "/Game/NovaeTerrae/AI/DataTables/DT_RocketSentinel.DT_RocketSentinel" (`self.DataTableRowName`))
    (:`then`
      (`NTEnemyHealthComponent.SetDefaultMaxHealth` _healthcomponent (break `/Game/NovaeTerrae/AI/DataTables/S_RocketSentinel` _returnvalue))
      (set `NTEnemyHealthComponent.ActionThresholdPercentage` (`.ShieldThresholdPercentage_20_F3B2A7BF481ACFCAA0C4009426093D21` (break `/Game/NovaeTerrae/AI/DataTables/S_RocketSentinel` _returnvalue)) _healthcomponent)
      (`BlackboardComponent.SetValueAsFloat` (`local.Blackboard`) "AttackCooldown" (`.AttackCooldown_18_BAD8A29C44DBD9FF7BD22E90EEA35C9F` (break `/Game/NovaeTerrae/AI/DataTables/S_RocketSentinel` _returnvalue)))
      (set `self.MissilesDamage` (`.MissileMaxDamage_10_5E6628594F315A8B4F0998B99536ECD0` (break `/Game/NovaeTerrae/AI/DataTables/S_RocketSentinel` _returnvalue)))
      (set `self.DamageRadius` (`.MissileExposionRadius_11_AFF9F6D445FF60827A35CAB1C61C9E82` (break `/Game/NovaeTerrae/AI/DataTables/S_RocketSentinel` _returnvalue)))
      (set `self.ShieldDuration` (`.ShieldDuration_22_914E216F45CFC2A80FB1EA9858AE96B3` (break `/Game/NovaeTerrae/AI/DataTables/S_RocketSentinel` _returnvalue)))
      (`BlackboardComponent.SetValueAsFloat` (`local.Blackboard`) "ActiveTeleportationDistance" (`.ActiveTeleportationDistance_7_3F91C06F4E5260F99E8CBEAFFE822015` (break `/Game/NovaeTerrae/AI/DataTables/S_RocketSentinel` _returnvalue)))
      (`BlackboardComponent.SetValueAsFloat` (`local.Blackboard`) "PassiveTeleportationCooldown" (`.PassiveTeleportationCooldown_13_26FAEB9A499E825CE29584B1A41465BC` (break `/Game/NovaeTerrae/AI/DataTables/S_RocketSentinel` _returnvalue)))
      (set `self.MinMissilesHomingMode` (`.MinMissilesHomingMode_25_53CF4EFD490B1101BA3E13975D3F827C` (break `/Game/NovaeTerrae/AI/DataTables/S_RocketSentinel` _returnvalue)))
      (set `self.MaxMissilesHomingMode` (`.MaxMissilesHomingMode_27_C95192A64640A113B162D8B9C938BAD2` (break `/Game/NovaeTerrae/AI/DataTables/S_RocketSentinel` _returnvalue)))
      (set `self.MinMissilesArtilleryMode` (`.MinMissilesArtilleryMode_30_0B8DD3F24548EF95100A908B81D4D413` (break `/Game/NovaeTerrae/AI/DataTables/S_RocketSentinel` _returnvalue)))
      (set `self.MaxMissilesArtilleryMode` (`.MaxMissilesArtilleryMode_32_6D23072B472F1CB116358D9E6915CDB5` (break `/Game/NovaeTerrae/AI/DataTables/S_RocketSentinel` _returnvalue)))
      (set `self.ArtilleryBarrageRadius` (`.ArtilleryBarrageRadius_35_8405DA854C48E68BB792BDBDF9DC6DF7` (break `/Game/NovaeTerrae/AI/DataTables/S_RocketSentinel` _returnvalue))))))

(fn `UserConstructionScript`)