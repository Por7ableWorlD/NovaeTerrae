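; Dialogue component that assembles a dialogue sequence from DT_Dialogue and sends it to the player's dialogue widget.
; On BeginPlay it retries on a short retriggerable delay until the player character's DialogueWG is valid, then caches it.
; StartDialogue follows NextLineName from row to row, starting at DialogueName, until no row is found, then queues the collected lines on the widget.
; Later calls reuse the filled array instead of reading the table again.
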(event `self.ReceiveBeginPlay`
  (set `self.DialogueName` (`KismetStringLibrary.Replace` (`self.DialogueName`) " "))
  (bind _asbp_ntbase_character (cast `/Game/NovaeTerrae/Core/Characters/Base/BP_NTBaseCharacter` (`GameplayStatics.GetPlayerCharacter` 0)))
  (bind _dialogue_wg (`/Game/NovaeTerrae/Core/Characters/Base/BP_NTBaseCharacter.Dialogue_WG` _asbp_ntbase_character :!label _label)
    (:`then`
      (`/Engine/EditorBlueprintResources/StandardMacros.DoOnce` false
        (:`Completed`
          (set `self.Dialogue_WG` _dialogue_wg))))
    (:`else`
      (`KismetSystemLibrary.RetriggerableDelay` 0.2)
      (goto _label))))

(event `StartDialogue`
  (bind _dialogue_dialogue (break `/Game/NovaeTerrae/Narrative/S_Dialogue` (`self.Dialogue`)))
  (bind _dialogue_dialogue_2 (break `/Game/NovaeTerrae/Narrative/S_Dialogue` (`self.Dialogue`)))
  (if (`KismetArrayLibrary.Array_IsEmpty` _dialogue_dialogue_2)
    (bind _returnvalue (`|GetDataTableRow` "/Game/NovaeTerrae/Narrative/DT_Dialogue.DT_Dialogue" (`KismetStringLibrary.Conv_StringToName` (`self.DialogueName`)) :!label _label_2)
      (:`then`
        (`KismetArrayLibrary.Array_Add` _dialogue_dialogue _returnvalue)
        (set `self.DialogueName` (`KismetStringLibrary.Replace` (`.NextLineName_10_49FF2B714D0C6C8D674DBDBA4AAD0E81` (break `/Game/NovaeTerrae/Narrative/S_DialogueLine` _returnvalue)) " "))
        (goto _label_2))
      (:`RowNotFound`
        (message `/Game/NovaeTerrae/Narrative/BPI_DialogueInterface.SendDialogueToQueue` (`self.Dialogue_WG`) (`self.Dialogue`))))
    (else
      (message `/Game/NovaeTerrae/Narrative/BPI_DialogueInterface.SendDialogueToQueue` (`self.Dialogue_WG`) (`self.Dialogue`)))))