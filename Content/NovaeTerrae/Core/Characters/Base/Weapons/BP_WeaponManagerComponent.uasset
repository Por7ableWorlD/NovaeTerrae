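; Weapon component that manages the player's four ammo types (base, stun, shield-gain, explosive) with per-type magazines and unlocks stored in BP_Save.
; Fire traces from the camera, re-traces from the firing socket, applies the current type's effect, makes noise and auto-reloads on empty.
; Reloads run on a timer, and switching cancels them but is blocked by the Thirst tag.
; It creates and drives the crosshair widget and broadcasts ammo changes.
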(event `self.ReceiveBeginPlay`
  (bind _currentammotype (`self.CurrentAmmoType`))
  (`self.LoadUnlockedAmmo`)
  (for _array_element (`self.AmmoInfo`)
    (if (`.IsUnlocked_11_7EEC6904499E566808063AB214B24887` (break `/Game/NovaeTerrae/Core/Characters/Base/Weapons/S_AmmoInfo` _array_element))
      (`BlueprintMapLibrary.Map_Add` (`self.AmmoAmount`) (break `/Game/NovaeTerrae/Core/Characters/Base/Weapons/S_AmmoInfo` _array_element) (`self.GetAmmoCapacity` (break `/Game/NovaeTerrae/Core/Characters/Base/Weapons/S_AmmoInfo` _array_element)))))
  (bind _returnvalue (`|CreateWidget` "/Game/NovaeTerrae/UI/Char_WG/Crosshair_Aim.Crosshair_Aim_C" (`GameplayStatics.GetPlayerController` 0) self))
  (bind _output_get (set `self.CrosshairWidget` _returnvalue))
  (`UserWidget.AddToViewport` _output_get 0)
  (`self.OnBulletNumberChanged` _currentammotype (`self.GetLoadedAmmo` _currentammotype) (`self.GetAmmoCapacity` _currentammotype)))

(event `Fire`
  (bind _returnvalue (`self.GetOwner`))
  (bind _currentammotype (`self.CurrentAmmoType`))
  (bind _currentammotype_2 (`self.CurrentAmmoType`))
  (bind _hit (`self.LaunchShootingTrace`))
  (`self.ChooseShootFunction` _hit)
  (`Actor.MakeNoise` _returnvalue 1.0 null (`Actor.K2_GetActorLocation` _returnvalue) (`self.GetNoiseRadius` (`self.CurrentAmmoType`)) "None")
  (`BlueprintMapLibrary.Map_Add` (`self.AmmoAmount`) _currentammotype_2 (- (`self.GetLoadedAmmo` _currentammotype_2) 1))
  (`/Game/NovaeTerrae/UI/Char_WG/Crosshair_Aim.Decrease Bar On Shot` (`self.CrosshairWidget`))
  (`self.OnBulletNumberChanged` _currentammotype (`self.GetLoadedAmmo` _currentammotype) (`self.GetAmmoCapacity` _currentammotype))
  (if (== (`self.GetLoadedAmmo` (`self.CurrentAmmoType`)) 0)
    (`self.BeginReload`)))

(fn `BeginReload`
  (bind _currentammotype (`self.CurrentAmmoType`))
  (bind _reloadtime (`self.GetReloadTime` (`self.CurrentAmmoType`)))
  (if (== (`self.GetLoadedAmmo` _currentammotype) (`self.GetAmmoCapacity` _currentammotype))
    _
    (elif (not (`KismetSystemLibrary.K2_IsTimerActiveHandle` (`self.ReloadTimerHandle`)))
      (bind _returnvalue (`KismetSystemLibrary.K2_SetTimer` null "EndReload" _reloadtime))
      (set `self.ReloadTimerHandle` _returnvalue)
      (`/Game/NovaeTerrae/UI/Char_WG/Crosshair_Aim.Fill_Reload_Bar` (`self.CrosshairWidget`) _reloadtime))))

(fn `CancelReload`
  (`KismetSystemLibrary.K2_ClearAndInvalidateTimerHandle` (`self.ReloadTimerHandle`)))

(fn `ChooseShootFunction`
  (params (Hit :type "HitResult Structure"))
  (locals (ImpactPoint :type "Vector Structure") (DamagedActor :type "Actor Object Reference"))
  (bind (_bblockinghit _binitialoverlap _time _distance _location _impactpoint _normal _impactnormal _physmat _hitactor) (`GameplayStatics.BreakHitResult` Hit))
  (set `local.ImpactPoint` _impactpoint)
  (set `local.DamagedActor` _hitactor)
  (if (`|EnumEquality` (`self.CurrentAmmoType`) "NewEnumerator0")
    (`self.ShootingBase` (`local.DamagedActor`))
    (elif (`|EnumEquality` (`self.CurrentAmmoType`) "NewEnumerator1")
      (`self.ShootingStun` (`local.DamagedActor`))
      (elif (`|EnumEquality` (`self.CurrentAmmoType`) "NewEnumerator2")
        (`self.ShootingShield` (`local.DamagedActor`))
        (elif (`|EnumEquality` (`self.CurrentAmmoType`) "NewEnumerator3")
          (`self.ShootingExplosive` (`local.ImpactPoint`)))))))

(fn `EndReload`
  (bind _currentammotype (`self.CurrentAmmoType`))
  (bind _currentammotype_2 (`self.CurrentAmmoType`))
  (`BlueprintMapLibrary.Map_Add` (`self.AmmoAmount`) _currentammotype_2 (`self.GetAmmoCapacity` _currentammotype_2))
  (`/Game/NovaeTerrae/UI/Char_WG/Crosshair_Aim.Reload_Bar_Fade` (`self.CrosshairWidget`))
  (`self.OnBulletNumberChanged` _currentammotype (`self.GetLoadedAmmo` _currentammotype) (`self.GetAmmoCapacity` _currentammotype)))

(fn `FinishShooting`
  (set `self.CanShoot` true))

(fn `GetAmmoCapacity`
  (params (AmmoType :type "/Game/NovaeTerrae/Core/Characters/Base/Weapons/E_AmmoType Enum" :default "NewEnumerator0"))
  (returns (AmmoCapacity :type Integer))
  (return (`.WeaponAmmoCapacity_14_BC12465A4BB71C38580016A9F06F39A6` (break `/Game/NovaeTerrae/Core/Characters/Base/Weapons/S_AmmoInfo` (`self.GetAmmoInfo` AmmoType)))))

(fn `GetAmmoDamage`
  (params (AmmoType :type "/Game/NovaeTerrae/Core/Characters/Base/Weapons/E_AmmoType Enum" :default "NewEnumerator0"))
  (returns (AmmoDamage :type "Float (double-precision)"))
  (return (`.AmmoDamage_21_C3C2C3954C29323E2AD4D2B422C91475` (break `/Game/NovaeTerrae/Core/Characters/Base/Weapons/S_AmmoInfo` (`self.GetAmmoInfo` AmmoType)))))

(fn `GetAmmoInfo`
  (params (AmmoType :type "/Game/NovaeTerrae/Core/Characters/Base/Weapons/E_AmmoType Enum" :default "NewEnumerator0"))
  (returns (Ammo :type "/Game/NovaeTerrae/Core/Characters/Base/Weapons/S_AmmoInfo Structure") (AmmoIndex :type Integer))
  (for (_array_element _array_index) (`self.AmmoInfo`)
    (if (`|EnumEquality` (`.AmmoType_5_94B939C34B0F0DFD35E8BEBE08123533` (break `/Game/NovaeTerrae/Core/Characters/Base/Weapons/S_AmmoInfo` _array_element)) (`local.AmmoType`))
      (return _array_element _array_index))))

(fn `GetAmmoPause`
  (params (AmmoType :type "/Game/NovaeTerrae/Core/Characters/Base/Weapons/E_AmmoType Enum" :default "NewEnumerator0"))
  (returns (`Ammo Pause` :type "Float (double-precision)"))
  (return (`.AmmoPause_25_69546E354FB80927769991988191512C` (break `/Game/NovaeTerrae/Core/Characters/Base/Weapons/S_AmmoInfo` (`self.GetAmmoInfo` AmmoType)))))

(fn `GetAmmoRange`
  (params (AmmoType :type "/Game/NovaeTerrae/Core/Characters/Base/Weapons/E_AmmoType Enum" :default "NewEnumerator0"))
  (returns (AmmoRange :type "Float (double-precision)"))
  (return (`.AmmoRange_23_425AD77141E57E8FA22B0CBD6AE7C776` (break `/Game/NovaeTerrae/Core/Characters/Base/Weapons/S_AmmoInfo` (`self.GetAmmoInfo` AmmoType)))))

(fn `GetExplosionRadius`
  (params (AmmoType :type "/Game/NovaeTerrae/Core/Characters/Base/Weapons/E_AmmoType Enum" :default "NewEnumerator0"))
  (returns (`Explosion Radius` :type "Float (double-precision)"))
  (return (`.ExplosionRadius_31_6E673FEB4889A8675ABC5F920CD2792C` (break `/Game/NovaeTerrae/Core/Characters/Base/Weapons/S_AmmoInfo` (`self.GetAmmoInfo` AmmoType)))))

(fn `GetIsUnlocked`
  (params (AmmoType :type "/Game/NovaeTerrae/Core/Characters/Base/Weapons/E_AmmoType Enum" :default "NewEnumerator0"))
  (returns (IsUnlocked :type Boolean))
  (return (`.IsUnlocked_11_7EEC6904499E566808063AB214B24887` (break `/Game/NovaeTerrae/Core/Characters/Base/Weapons/S_AmmoInfo` (`self.GetAmmoInfo` AmmoType)))))

(fn `GetLoadedAmmo`
  (params (AmmoType :type "/Game/NovaeTerrae/Core/Characters/Base/Weapons/E_AmmoType Enum" :default "NewEnumerator0"))
  (returns (AmmoAmount :type Integer))
  (return (`BlueprintMapLibrary.Map_Find` (`self.AmmoAmount`) AmmoType)))

(fn `GetNextAmmo`
  (returns (ResultAmmoType :type "/Game/NovaeTerrae/Core/Characters/Base/Weapons/E_AmmoType Enum"))
  (locals (AmmoIndex :type Integer :default 0))
  (bind _returnvalue (`KismetArrayLibrary.Array_Length` (`self.AmmoInfo`)))
  (bind _output_get (set `local.AmmoIndex` (`.AmmoIndex` (`self.GetAmmoInfo` (`self.CurrentAmmoType`)))))
  (for _index (range 1 (+ _returnvalue 1))
    (bind (_output_ammotype _output_weaponammocapacity _output_isunlocked) (break `/Game/NovaeTerrae/Core/Characters/Base/Weapons/S_AmmoInfo` (`|GetArrayItem` (`self.AmmoInfo`) (mod (+ _index _output_get) _returnvalue))))
    (if _output_isunlocked
      (return _output_ammotype))))

(fn `GetNoiseRadius`
  (params (AmmoType :type "/Game/NovaeTerrae/Core/Characters/Base/Weapons/E_AmmoType Enum" :default "NewEnumerator0"))
  (returns (NoiseRadius :type "Float (double-precision)"))
  (return (`.AmmoNoiseRadius_34_12CE02A842417E521D3AE3B04479ABFA` (break `/Game/NovaeTerrae/Core/Characters/Base/Weapons/S_AmmoInfo` (`self.GetAmmoInfo` AmmoType)))))

(fn `GetPreviousAmmo`
  (returns (ResultAmmoType :type "/Game/NovaeTerrae/Core/Characters/Base/Weapons/E_AmmoType Enum"))
  (locals (AmmoIndex :type Integer))
  (bind _returnvalue (`KismetArrayLibrary.Array_Length` (`self.AmmoInfo`)))
  (set `local.AmmoIndex` (+ (`.AmmoIndex` (`self.GetAmmoInfo` (`self.CurrentAmmoType`))) _returnvalue))
  (for _index (range 1 (+ _returnvalue 1))
    (bind (_output_ammotype _output_weaponammocapacity _output_isunlocked) (break `/Game/NovaeTerrae/Core/Characters/Base/Weapons/S_AmmoInfo` (`|GetArrayItem` (`self.AmmoInfo`) (mod (- (`local.AmmoIndex`) _index) (`KismetArrayLibrary.Array_Length` (`self.AmmoInfo`))))))
    (if _output_isunlocked
      (return _output_ammotype))))

(fn `GetReloadTime`
  (params (AmmoType :type "/Game/NovaeTerrae/Core/Characters/Base/Weapons/E_AmmoType Enum" :default "NewEnumerator0"))
  (returns (ReloadTime :type "Float (double-precision)"))
  (return (`KismetMathLibrary.SelectFloat` 0.1 (`.ReloadTime_19_C8C395B94D3B0421BC49B59AC8E4361C` (break `/Game/NovaeTerrae/Core/Characters/Base/Weapons/S_AmmoInfo` (`self.GetAmmoInfo` AmmoType))) (`self.IsFastReloadEnabled`))))

(fn `LaunchShootingTrace`
  (returns (Hit :type "HitResult Structure"))
  (bind _returnvalue (`GameplayStatics.GetPlayerCameraManager` 0))
  (bind _returnvalue_2 (`PlayerCameraManager.GetCameraLocation` _returnvalue))
  (bind _outhit (`KismetSystemLibrary.LineTraceSingle` :`Start` _returnvalue_2 :`End` (+ _returnvalue_2 (* (`KismetMathLibrary.GetForwardVector` (`PlayerCameraManager.GetCameraRotation` _returnvalue)) (`self.GetAmmoRange` (`self.CurrentAmmoType`)))) :`TraceChannel` "TraceTypeQuery1" :`DrawDebugType` "ForDuration" :`DrawTime` 2.0))
  (bind _socketlocation (message `/Game/NovaeTerrae/AI/Interfaces/BPI_CombatInterface.RequestFiringSocketLocation` (`self.GetOwner`)))
  (bind (_bblockinghit _binitialoverlap _time _distance _location _impactpoint _normal _impactnormal _physmat _hitactor _hitcomponent _hitbonename _bonename _hititem _elementindex _faceindex _tracestart _traceend) (`GameplayStatics.BreakHitResult` _outhit))
  (bind _returnvalue_3 (- _location _socketlocation))
  (bind _outhit_2 (`KismetSystemLibrary.LineTraceSingle` :`Start` _socketlocation :`End` (`KismetMathLibrary.SelectVector` (+ (* (/ _returnvalue_3 (`KismetMathLibrary.VSize` _returnvalue_3)) (`self.GetAmmoRange` (`self.CurrentAmmoType`))) _location) _traceend _bblockinghit) :`TraceChannel` "TraceTypeQuery1" :`DrawDebugType` "ForDuration" :`TraceColor` (struct :`R` 0.969434 :`G` 1.0 :`A` 1.0)))
  (return _outhit_2))

(fn `LoadUnlockedAmmo`
  (bind (_ammo _ammoindex) (`self.GetAmmoInfo` "NewEnumerator3"))
  (bind (_ammo_2 _ammoindex_2) (`self.GetAmmoInfo` "NewEnumerator1"))
  (bind (_ammo_3 _ammoindex_3) (`self.GetAmmoInfo` "NewEnumerator2"))
  (bind _returnvalue (`GameplayStatics.LoadGameFromSlot` "Save_Info"))
  (bind _asbp_save (cast `/Game/NovaeTerrae/Puzzles/Altar/BP_Save` _returnvalue))
  (`KismetArrayLibrary.Array_Set` (`self.AmmoInfo`) _ammoindex_2 (make `/Game/NovaeTerrae/Core/Characters/Base/Weapons/S_AmmoInfo` (break `/Game/NovaeTerrae/Core/Characters/Base/Weapons/S_AmmoInfo` _ammo_2) (`.WeaponAmmoCapacity_14_BC12465A4BB71C38580016A9F06F39A6` (break `/Game/NovaeTerrae/Core/Characters/Base/Weapons/S_AmmoInfo` _ammo_2)) (`/Game/NovaeTerrae/Puzzles/Altar/BP_Save.Ammo_Stun_Unlocked` _asbp_save) (`.ReloadTime_19_C8C395B94D3B0421BC49B59AC8E4361C` (break `/Game/NovaeTerrae/Core/Characters/Base/Weapons/S_AmmoInfo` _ammo_2)) (`.AmmoDamage_21_C3C2C3954C29323E2AD4D2B422C91475` (break `/Game/NovaeTerrae/Core/Characters/Base/Weapons/S_AmmoInfo` _ammo_2)) (`.AmmoRange_23_425AD77141E57E8FA22B0CBD6AE7C776` (break `/Game/NovaeTerrae/Core/Characters/Base/Weapons/S_AmmoInfo` _ammo_2)) (`.AmmoPause_25_69546E354FB80927769991988191512C` (break `/Game/NovaeTerrae/Core/Characters/Base/Weapons/S_AmmoInfo` _ammo_2)) (`.ExplosionRadius_31_6E673FEB4889A8675ABC5F920CD2792C` (break `/Game/NovaeTerrae/Core/Characters/Base/Weapons/S_AmmoInfo` _ammo_2)) (`.AmmoNoiseRadius_34_12CE02A842417E521D3AE3B04479ABFA` (break `/Game/NovaeTerrae/Core/Characters/Base/Weapons/S_AmmoInfo` _ammo_2))))
  (`KismetArrayLibrary.Array_Set` (`self.AmmoInfo`) _ammoindex_3 (make `/Game/NovaeTerrae/Core/Characters/Base/Weapons/S_AmmoInfo` (break `/Game/NovaeTerrae/Core/Characters/Base/Weapons/S_AmmoInfo` _ammo_3) (`.WeaponAmmoCapacity_14_BC12465A4BB71C38580016A9F06F39A6` (break `/Game/NovaeTerrae/Core/Characters/Base/Weapons/S_AmmoInfo` _ammo_3)) (`/Game/NovaeTerrae/Puzzles/Altar/BP_Save.Ammo_Shield_Unlocked` _asbp_save) (`.ReloadTime_19_C8C395B94D3B0421BC49B59AC8E4361C` (break `/Game/NovaeTerrae/Core/Characters/Base/Weapons/S_AmmoInfo` _ammo_3)) (`.AmmoDamage_21_C3C2C3954C29323E2AD4D2B422C91475` (break `/Game/NovaeTerrae/Core/Characters/Base/Weapons/S_AmmoInfo` _ammo_3)) (`.AmmoRange_23_425AD77141E57E8FA22B0CBD6AE7C776` (break `/Game/NovaeTerrae/Core/Characters/Base/Weapons/S_AmmoInfo` _ammo_3)) (`.AmmoPause_25_69546E354FB80927769991988191512C` (break `/Game/NovaeTerrae/Core/Characters/Base/Weapons/S_AmmoInfo` _ammo_3)) (`.ExplosionRadius_31_6E673FEB4889A8675ABC5F920CD2792C` (break `/Game/NovaeTerrae/Core/Characters/Base/Weapons/S_AmmoInfo` _ammo_3)) (`.AmmoNoiseRadius_34_12CE02A842417E521D3AE3B04479ABFA` (break `/Game/NovaeTerrae/Core/Characters/Base/Weapons/S_AmmoInfo` _ammo_3))))
  (`KismetArrayLibrary.Array_Set` (`self.AmmoInfo`) _ammoindex (make `/Game/NovaeTerrae/Core/Characters/Base/Weapons/S_AmmoInfo` (break `/Game/NovaeTerrae/Core/Characters/Base/Weapons/S_AmmoInfo` _ammo) (`.WeaponAmmoCapacity_14_BC12465A4BB71C38580016A9F06F39A6` (break `/Game/NovaeTerrae/Core/Characters/Base/Weapons/S_AmmoInfo` _ammo)) (`/Game/NovaeTerrae/Puzzles/Altar/BP_Save.Ammo_AoE_Unlocked` _asbp_save) (`.ReloadTime_19_C8C395B94D3B0421BC49B59AC8E4361C` (break `/Game/NovaeTerrae/Core/Characters/Base/Weapons/S_AmmoInfo` _ammo)) (`.AmmoDamage_21_C3C2C3954C29323E2AD4D2B422C91475` (break `/Game/NovaeTerrae/Core/Characters/Base/Weapons/S_AmmoInfo` _ammo)) (`.AmmoRange_23_425AD77141E57E8FA22B0CBD6AE7C776` (break `/Game/NovaeTerrae/Core/Characters/Base/Weapons/S_AmmoInfo` _ammo)) (`.AmmoPause_25_69546E354FB80927769991988191512C` (break `/Game/NovaeTerrae/Core/Characters/Base/Weapons/S_AmmoInfo` _ammo)) (`.ExplosionRadius_31_6E673FEB4889A8675ABC5F920CD2792C` (break `/Game/NovaeTerrae/Core/Characters/Base/Weapons/S_AmmoInfo` _ammo)) (`.AmmoNoiseRadius_34_12CE02A842417E521D3AE3B04479ABFA` (break `/Game/NovaeTerrae/Core/Characters/Base/Weapons/S_AmmoInfo` _ammo)))))

(fn `PickUpAmmo`
  (params (AmmoType :type "/Game/NovaeTerrae/Core/Characters/Base/Weapons/E_AmmoType Enum" :default "NewEnumerator0"))
  (locals (UnlockedNewAmmo :type Boolean))
  (bind (_ammo _ammoindex) (`self.GetAmmoInfo` AmmoType))
  (`BlueprintMapLibrary.Map_Add` (`self.AmmoAmount`) (break `/Game/NovaeTerrae/Core/Characters/Base/Weapons/S_AmmoInfo` _ammo) (`.WeaponAmmoCapacity_14_BC12465A4BB71C38580016A9F06F39A6` (break `/Game/NovaeTerrae/Core/Characters/Base/Weapons/S_AmmoInfo` _ammo)))
  (`KismetArrayLibrary.Array_Set` (`self.AmmoInfo`) _ammoindex (make `/Game/NovaeTerrae/Core/Characters/Base/Weapons/S_AmmoInfo` (break `/Game/NovaeTerrae/Core/Characters/Base/Weapons/S_AmmoInfo` _ammo) (`.WeaponAmmoCapacity_14_BC12465A4BB71C38580016A9F06F39A6` (break `/Game/NovaeTerrae/Core/Characters/Base/Weapons/S_AmmoInfo` _ammo)) true (`.ReloadTime_19_C8C395B94D3B0421BC49B59AC8E4361C` (break `/Game/NovaeTerrae/Core/Characters/Base/Weapons/S_AmmoInfo` _ammo)) (`.AmmoDamage_21_C3C2C3954C29323E2AD4D2B422C91475` (break `/Game/NovaeTerrae/Core/Characters/Base/Weapons/S_AmmoInfo` _ammo)) (`.AmmoRange_23_425AD77141E57E8FA22B0CBD6AE7C776` (break `/Game/NovaeTerrae/Core/Characters/Base/Weapons/S_AmmoInfo` _ammo)) (`.AmmoPause_25_69546E354FB80927769991988191512C` (break `/Game/NovaeTerrae/Core/Characters/Base/Weapons/S_AmmoInfo` _ammo)) (`.ExplosionRadius_31_6E673FEB4889A8675ABC5F920CD2792C` (break `/Game/NovaeTerrae/Core/Characters/Base/Weapons/S_AmmoInfo` _ammo))))
  (`self.SaveUnlockedAmmo`)
  (return))

(fn `PrintInfo`
  (bind _keys (`BlueprintMapLibrary.Map_Keys` (`self.AmmoAmount`)))
  (for _array_element _keys
    (`KismetSystemLibrary.PrintString` (`KismetStringLibrary.Concat_StrStr` (`KismetStringLibrary.Concat_StrStr` (`|GetEnumeratorNameAsString` _array_element) ": ") (`KismetStringLibrary.Conv_IntToString` (`BlueprintMapLibrary.Map_Find` (`self.AmmoAmount`) _array_element)))))
  (`KismetSystemLibrary.PrintString` (`KismetStringLibrary.Concat_StrStr` "CurrentAmmoType: " (`|GetEnumeratorNameAsString` (`self.CurrentAmmoType`)))))

(fn `SaveUnlockedAmmo`
  (bind _returnvalue (`GameplayStatics.DoesSaveGameExist` "Save_Info"))
  (if _returnvalue
    (bind _returnvalue_2 (`GameplayStatics.LoadGameFromSlot` "Save_Info"))
    (bind _asbp_save (cast `/Game/NovaeTerrae/Puzzles/Altar/BP_Save` _returnvalue_2))
    (set `/Game/NovaeTerrae/Puzzles/Altar/BP_Save.Ammo_Stun_Unlocked` (`self.GetIsUnlocked` "NewEnumerator1") _asbp_save)
    (set `/Game/NovaeTerrae/Puzzles/Altar/BP_Save.Ammo_Shield_Unlocked` (`self.GetIsUnlocked` "NewEnumerator2") _asbp_save)
    (set `/Game/NovaeTerrae/Puzzles/Altar/BP_Save.Ammo_AoE_Unlocked` (`self.GetIsUnlocked` "NewEnumerator3") _asbp_save)
    (`GameplayStatics.SaveGameToSlot` _asbp_save "Save_Info")))

(fn `ShootingBase`
  (params (DamagedActor :type "Actor Object Reference"))
  (`GameplayStatics.PlayWorldCameraShake` "/Game/NovaeTerrae/Core/Characters/Base/CameraShakes/BP_BaseShootingCameraShake.BP_BaseShootingCameraShake_C" (`Actor.K2_GetActorLocation` (`self.GetOwner`)) 0.0 500.0)
  (`/Engine/EditorBlueprintResources/StandardMacros.IsValid` (`local.DamagedActor`)
    (:`Is Valid`
      (`GameplayStatics.ApplyDamage` (`local.DamagedActor`) (`self.GetAmmoDamage` (`self.CurrentAmmoType`)) null (`self.GetOwner`)))))

(fn `ShootingExplosive`
  (params (ImpactPoint :type "Vector Structure"))
  (bind _explosion_radius (`self.GetExplosionRadius` (`self.CurrentAmmoType`)))
  (`GameplayStatics.PlayWorldCameraShake` "/Game/NovaeTerrae/Core/Characters/Base/CameraShakes/BP_ExplosiveShootingCameraShake.BP_ExplosiveShootingCameraShake_C" (`Actor.K2_GetActorLocation` (`self.GetOwner`)) 0.0 500.0)
  (`GameplayStatics.ApplyRadialDamage` :`BaseDamage` (`self.GetAmmoDamage` (`self.CurrentAmmoType`)) :`Origin` (`local.ImpactPoint`) :`DamageRadius` _explosion_radius :`DamageCauser` (`self.GetOwner`) :`InstigatedByController` null)
  (`NiagaraFunctionLibrary.SpawnSystemAtLocation` "/Game/NovaeTerrae/Art/VFX/NS_Explosion_eyes.NS_Explosion_eyes" (`local.ImpactPoint`) (struct) (`KismetMathLibrary.Conv_DoubleToVector` (`KismetMathLibrary.FClamp` _explosion_radius 0.5 3.0))))

(fn `ShootingShield`
  (params (DamagedActor :type "Actor Object Reference"))
  (bind _damagedactor (`local.DamagedActor`))
  (bind _returnvalue (`Actor.GetComponentByClass` (`self.GetOwner`) "/Script/NovaeTerrae.NTHealthComponent"))
  (`/Engine/EditorBlueprintResources/StandardMacros.IsValid` DamagedActor
    (:`Is Valid`
      (`GameplayStatics.ApplyDamage` (`local.DamagedActor`) (`self.GetAmmoDamage` (`self.CurrentAmmoType`)) null (`self.GetOwner`))
      (if (`GameplayStatics.ObjectIsA` _damagedactor "/Script/NovaeTerrae.NTBaseEnemyCharacter")
        (if (not (`NTHealthComponent.IsDead` (`Actor.GetComponentByClass` _damagedactor "/Script/NovaeTerrae.NTEnemyHealthComponent")))
          (`/Engine/EditorBlueprintResources/StandardMacros.IsValid` _returnvalue
            (:`Is Valid`
              (`NTHealthComponent.SetShieldHealth` _returnvalue (+ (`NTHealthComponent.GetCurrentShieldHealth` _returnvalue) (`self.ShieldAccumulation`))))))))))

(fn `ShootingStun`
  (params (DamagedActor :type "Actor Object Reference"))
  (`/Engine/EditorBlueprintResources/StandardMacros.IsValid` DamagedActor
    (:`Is Valid`
      (`GameplayStatics.ApplyDamage` (`local.DamagedActor`) (`self.GetAmmoDamage` (`self.CurrentAmmoType`)) null (`self.GetOwner`))
      (if (`GameplayStatics.ObjectIsA` (`local.DamagedActor`) "/Script/NovaeTerrae.NTBaseEnemyCharacter")
        (message `/Game/NovaeTerrae/AI/Interfaces/BPI_StatusInterface.ApplyStun` (`AIBlueprintHelperLibrary.GetAIController` (`local.DamagedActor`)) (`self.StunDuration`))))))

(fn `StartShooting`
  (returns (IsShootingAvailable :type Boolean))
  (if (and (`self.AimMode`) (> (`self.GetLoadedAmmo` (`self.CurrentAmmoType`)) 0) (`self.CanShoot`) (not (`KismetSystemLibrary.K2_IsTimerActiveHandle` (`self.ReloadTimerHandle`))))
    (set `self.CanShoot` false)
    (`/Game/NovaeTerrae/UI/Char_WG/Crosshair_Aim.Anim_Choice` (`self.CrosshairWidget`))
    (return true)
    (else
      (return false))))

(fn `SwitchAmmoType`
  (params (AmmoType :type "/Game/NovaeTerrae/Core/Characters/Base/Weapons/E_AmmoType Enum" :default "NewEnumerator0") (GameTags :type "GameplayTagContainer Structure"))
  (if (`|EnumInequality` AmmoType (`self.CurrentAmmoType`))
    (if (`self.GetIsUnlocked` (`local.AmmoType`))
      (if (not (`BlueprintGameplayTagLibrary.HasTag` (`local.GameTags`) (struct :`TagName` "Status.Thirst") true))
        (`/Game/NovaeTerrae/UI/Char_WG/Crosshair_Aim.Save Perc` (`self.CrosshairWidget`))
        (`self.OnAmmoSwitch` (`self.CurrentAmmoType`) (`local.AmmoType`))
        (set `self.CurrentAmmoType` (`local.AmmoType`))
        (`/Game/NovaeTerrae/UI/Char_WG/Crosshair_Aim.Set Current Ammo Value` (`self.CrosshairWidget`))
        (if (`KismetSystemLibrary.K2_IsTimerActiveHandle` (`self.ReloadTimerHandle`))
          (`self.CancelReload`)
          (`/Game/NovaeTerrae/UI/Char_WG/Crosshair_Aim.Cancel_Filling_Bar` (`self.CrosshairWidget`)))))))