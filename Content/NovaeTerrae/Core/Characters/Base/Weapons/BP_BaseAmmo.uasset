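; BP_BaseAmmo is an interactable ammo pickup that grants one ammo type to the player character.
; On interaction it removes its hint, hands the ammo to the character's weapon manager, and updates HUD ammo tracking and message.
; It also unlocks the journal module matching the type, with an extra GiveBase call for the first type.
; A DoOnce guards the pickup, and the actor destroys itself after a short delay.
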(event `self.ReceiveBeginPlay`
  (`parent.ReceiveBeginPlay`)
  (bind _asbp_ntbase_character (cast `/Game/NovaeTerrae/Core/Characters/Base/BP_NTBaseCharacter` (`GameplayStatics.GetPlayerCharacter` 0)))
  (set `self.Char_Ref` _asbp_ntbase_character))

(event `/Game/NovaeTerrae/Puzzles/BPI_InteractionInterface.StartInteraction`
  (if (`self.InteractionAvailable`)
    (`self.Give_Ammo`)
    (`self.RemoveHintWidget`)
    (set `self.InteractionAvailable` false)
    (`self.Give_Ammo_Amount`)))

(event `Give_Ammo`
  (bind _ammotype (`self.AmmoType`))
  ;[0 0 0] Give Char Ammo
  (`/Engine/EditorBlueprintResources/StandardMacros.DoOnce` false
    (:`Completed`
      (`/Game/NovaeTerrae/Core/Characters/Base/Weapons/BP_WeaponManagerComponent.PickUpAmmo` (`/Game/NovaeTerrae/Core/Characters/Base/BP_NTBaseCharacter.BP_WeaponManagerComponent` (`self.Char_Ref`)) _ammotype)
      (if (`|EnumEquality` _ammotype "NewEnumerator0")
        (`/Game/NovaeTerrae/Core/Characters/Base/BP_NTBaseCharacter.Give_Base` (`self.Char_Ref`)))
      (`/Game/NovaeTerrae/UI/Char_WG/WBP_Hud.Show_Message` (`/Game/NovaeTerrae/Core/Characters/Base/BP_NTBaseCharacter.Char_Hud_WG` (`self.Char_Ref`)) false false false true false)
      (`self.Set Ammo to Journal`)
      (`KismetSystemLibrary.Delay` 0.2)
      (`self.K2_DestroyActor`))))

(fn `Give_Ammo_Amount`
  (bind _ammotype (`self.AmmoType`))
  (bind _bp_weaponmanagercomponent (`/Game/NovaeTerrae/Core/Characters/Base/BP_NTBaseCharacter.BP_WeaponManagerComponent` (`self.Char_Ref`)))
  (`/Game/NovaeTerrae/UI/Char_WG/WBP_Hud.Track_Ammo` (`/Game/NovaeTerrae/Core/Characters/Base/BP_NTBaseCharacter.Char_Hud_WG` (`self.Char_Ref`)) _ammotype (`/Game/NovaeTerrae/Core/Characters/Base/Weapons/BP_WeaponManagerComponent.GetLoadedAmmo` _bp_weaponmanagercomponent _ammotype) (`/Game/NovaeTerrae/Core/Characters/Base/Weapons/BP_WeaponManagerComponent.GetAmmoCapacity` _bp_weaponmanagercomponent _ammotype)))

(fn `Set Ammo to Journal`
  (if (`|EnumEquality` (`self.AmmoType`) "NewEnumerator0")
    (set `/Game/NovaeTerrae/UI/System_WG/Journal_WG.Module_1_Unlocked` true (`/Game/NovaeTerrae/Core/Characters/Base/BP_NTBaseCharacter.Journal_WG` (`self.Char_Ref`)))
    (elif (`|EnumEquality` (`self.AmmoType`) "NewEnumerator1")
      (set `/Game/NovaeTerrae/UI/System_WG/Journal_WG.Module_2_Unlocked` true (`/Game/NovaeTerrae/Core/Characters/Base/BP_NTBaseCharacter.Journal_WG` (`self.Char_Ref`)))
      (elif (`|EnumEquality` (`self.AmmoType`) "NewEnumerator2")
        (set `/Game/NovaeTerrae/UI/System_WG/Journal_WG.Module_3_Unlocked` true (`/Game/NovaeTerrae/Core/Characters/Base/BP_NTBaseCharacter.Journal_WG` (`self.Char_Ref`)))
        (elif (`|EnumEquality` (`self.AmmoType`) "NewEnumerator3")
          (set `/Game/NovaeTerrae/UI/System_WG/Journal_WG.Module_4_Unlocked` true (`/Game/NovaeTerrae/Core/Characters/Base/BP_NTBaseCharacter.Journal_WG` (`self.Char_Ref`))))))))

(fn `UserConstructionScript`)