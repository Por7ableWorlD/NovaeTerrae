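; Base player character for a third-person shooter with puzzle interaction, creating HUD, pause and death widgets and restoring its saved position on BeginPlay.
; Aimed camera line traces fire four ammo types (Base, Stun, Shield, radial AoE), each with saved counts and timed reloads.
; A timer-driven laser sphere-trace ability depends on the last death signal's flag.
; Interaction traces use actor tags to destroy pickups or pulse chest, button and panel booleans.
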(event `OnDeathSignature_Event`
  (params (IsLazer :type Boolean))
  ;[0 0 0] Char Death
  (set `self.IsLastLazer` IsLazer)
  (`KismetSystemLibrary.Delay` 2.0)
  (bind _returnvalue (`|CreateWidget` "/Game/NovaeTerrae/UI/Char_WG/Death.Death_C" (`GameplayStatics.GetPlayerController` 0)))
  (bind _output_get (set `self.DeathWidget` _returnvalue))
  (`UserWidget.AddToViewport` _output_get 0))

(event `self.ReceiveBeginPlay`
  ;[0.2016 1 0.2346] Begin Play
  (`self.Check_Save`)
  (`self.Change_Crosshair`)
  ;[0 0 0] Add Crosshair
  (bind _returnvalue (`|CreateWidget` "/Game/NovaeTerrae/UI/Char_WG/Crosshair_Aim.Crosshair_Aim_C" :!label _label))
  (bind _output_get (set `self.Crosshair_Aim` _returnvalue))
  (`UserWidget.AddToViewport` _output_get 0)
  ;[0 0 0] Pause
  (bind _returnvalue_2 (`|CreateWidget` "/Game/NovaeTerrae/UI/System_WG/Pause_WG.Pause_WG_C"))
  (bind _output_get_2 (set `self.Pause_WG` _returnvalue_2))
  (`UserWidget.AddToViewport` _output_get_2 0)
  (`Widget.SetVisibility` _output_get_2 "Hidden")
  ;[0 0 0] Add Ammo
  (bind _returnvalue_3 (`|CreateWidget` "/Game/NovaeTerrae/UI/Char_WG/Ammo.Ammo_C"))
  (bind _output_get_3 (set `self.Ammo_WG` _returnvalue_3))
  (`UserWidget.AddToViewport` _output_get_3 0)
  ;[0 0 0] Item (Key) Widget
  (bind _returnvalue_4 (`|CreateWidget` "/Game/NovaeTerrae/UI/Puzzle_WG/Item_Now_WG.Item_Now_WG_C"))
  (bind _output_get_4 (set `self.Item_WG` _returnvalue_4))
  (`UserWidget.AddToViewport` _output_get_4 0)
  ;[0 0 0] Interaction Widget
  (bind _returnvalue_5 (`|CreateWidget` "/Game/NovaeTerrae/UI/Puzzle_WG/Interaction_Puzzle.Interaction_Puzzle_C"))
  (bind _output_get_5 (set `self.Interaction_WG` _returnvalue_5))
  (`UserWidget.AddToViewport` _output_get_5 0)
  ;[0 0 0] Char Death
  (add `self.OnResetPlayerDeathSignature` (delegate `OnResetDeathSignature_Event`))
  (add `self.OnPlayerDeathSignature` (delegate `OnDeathSignature_Event`))
  (bind _returnvalue_6 (`GameplayStatics.GetActorOfClass` "/Game/NovaeTerrae/AI/Blueprints/BP_ChallengeZone.BP_ChallengeZone_C"))
  (set `self.ChallengeZone` _returnvalue_6))

(event `Create_Widgets`
  (goto _label))

(event `OnResetDeathSignature_Event`
  ;[0 0 0] Char Death
  (`self.OnPlayerDeath`)
  (`KismetSystemLibrary.Delay` 1.0)
  (`/Engine/EditorBlueprintResources/StandardMacros.IsValid` (`self.DeathWidget`)
    (:`Is Valid`
      (`Widget.RemoveFromParent` (`self.DeathWidget`))
      (set `self.DeathWidget` null))))

(event `Key|R`
  (params (Key :type "Key Structure"))
  ;[0 0 0] R Key -- Reload
  (:`Pressed`
    (if (`self.Reloading_Now`)
      _
      (elif (== (`self.Ammo_Now`) (`self.Max_Ammo`))
        (`KismetSystemLibrary.PrintString` "Ammo is Full!" true true (struct :`A` 1.0))
        (else
          ;[0 0 0] Shooting
          (`self.Reloading_Event` :!label _label_2))))))

(event `Key|E`
  (params (Key :type "Key Structure"))
  ;[0 0 0] E Key
  (:`Pressed`
    (`self.OnInteract`)
    (`self.Interact_wth_Obj`)))

(event `Key|LeftMouseButton`
  (params (Key :type "Key Structure"))
  (bind _returnvalue (`GameplayStatics.GetPlayerCameraManager` 0))
  (bind _returnvalue_2 (`self.K2_GetActorLocation` _returnvalue))
  ;[0 0 0] Shooting
  (:`Pressed`
    (if (`self.Aim_Mode`)
      (if (`self.Have Ammo`)
        (if (not (`self.Pause`))
          (bind (_outhit _returnvalue_3) (`KismetSystemLibrary.LineTraceSingle` :`Start` _returnvalue_2 :`End` (+ _returnvalue_2 (* (`self.GetActorForwardVector` _returnvalue) (`self.Ammo_Range`))) :`TraceChannel` "TraceTypeQuery1" :`DrawDebugType` "ForDuration" :`DrawTime` 2.0))
          (if _returnvalue_3
            _
            (else
              _))
          (`self.Pause_Shots`)
          (if (== 4 (`self.Ammo_Int`))
            (bind (_bblockinghit _binitialoverlap _time _distance _location _impactpoint _normal _impactnormal _physmat _hitactor) (`GameplayStatics.BreakHitResult` _outhit))
            (`self.Aoe_Explosion` _impactpoint)
            (else
              (`GameplayStatics.ApplyDamage` _hitactor (`self.Ammo_Damage`) null self)))
          (bind _result (`/Engine/EditorBlueprintResources/StandardMacros.DecrementInt` (`self.Ammo_Now`))
            (:`  `
              (if (== _result 0)
                (goto _label_2)))))))))

(event `Reloading_Event`
  ;[0 0 0] Reload Event
  (`/Game/NovaeTerrae/UI/Char_WG/Crosshair_Aim.Fill_Reload_Bar` (`self.Crosshair_Aim`))
  (set `self.Ammo_To_Reload` (`self.Ammo_Int`))
  (set `self.Have Ammo` false)
  (set `self.Reloading_Now` true)
  (`KismetSystemLibrary.Delay` (`self.GetReloadTime`))
  (if (`self.Was_Switched`)
    (set `self.Have Ammo` true)
    (set `self.Ammo_Now` (`self.Ammo_Now`) :!label _label_3)
    (else
      (set `self.Have Ammo` true)
      (if (== (`self.Ammo_To_Reload`) (`self.Ammo_Int`))
        (set `self.Ammo_Now` (`self.Max_Ammo`))
        (else
          (goto _label_3)))))
  (set `self.Was_Switched` false)
  (set `self.Reloading_Now` false))

(event `Key|Q`
  (params (Key :type "Key Structure"))
  ;[0 0 0] Lazer
  (:`Pressed`
    (if (`self.AbilityOnCooldown`)
      _
      (elif (`self.IsLastLazer`)
        (set `self.AbilityOnCooldown` true)
        (set `self.LazerCounter` 0)
        (bind _returnvalue (`KismetSystemLibrary.K2_SetTimerDelegate` (delegate `EmitLazer`) 0.1 true))
        (set `self.Timer` _returnvalue))))
  (:`Released`
    (`KismetSystemLibrary.K2_ClearAndInvalidateTimerHandle` (`self.Timer`) :!label _label_4)
    (`KismetSystemLibrary.Delay` 5.0)
    (set `self.AbilityOnCooldown` false)))

(event `Key|Escape` :paused true
  (params (Key :type "Key Structure"))
  (bind _pause_wg (`self.Pause_WG`))
  ;[0 0 0] Open / Close Pause Widget
  (:`Pressed`
    (if (`/Game/NovaeTerrae/UI/System_WG/Pause_WG.Pause_Active` _pause_wg) :!label _label_5
      (`/Game/NovaeTerrae/UI/System_WG/Pause_WG.Close_Pause_Anim` _pause_wg)
      (else
        (`/Game/NovaeTerrae/UI/System_WG/Pause_WG.Open_Pause_Anim` _pause_wg)))))

(event `Key|P` :paused true
  (params (Key :type "Key Structure"))
  ;[0 0 0] Open / Close Pause Widget
  (:`Pressed`
    (goto _label_5)))

(event `EmitLazer`
  (bind _returnvalue (`self.K2_GetActorLocation`))
  (bind _returnvalue_2 (* (`self.GetActorForwardVector`) 150.0))
  ;[0 0 0] Lazer
  (`KismetSystemLibrary.DrawDebugCylinder` _returnvalue _returnvalue_2 100.0 12 (struct :`R` 1.0 :`G` 0.477468 :`B` 0.054318 :`A` 1.0) 0.1 4.0)
  (bind _outhits (`KismetSystemLibrary.SphereTraceMulti` _returnvalue _returnvalue_2 100.0 "TraceTypeQuery1"))
  (for _array_element _outhits
    (cast `/Game/NovaeTerrae/AI/EyeSentinel/BP_EyeSentinel` (`.HitActor` (`GameplayStatics.BreakHitResult` _array_element))
      (:`then`
        _)
      (:`CastFailed`
        (cast `/Game/NovaeTerrae/AI/Blueprints/BP_DeactivationObject` (`.HitActor` (`GameplayStatics.BreakHitResult` _array_element)))))
    (`GameplayStatics.ApplyDamage` (`.HitActor` (`GameplayStatics.BreakHitResult` _array_element)) 5.0 null self "/Script/NovaeTerrae.LazerDamageType")
    (bind _result (`/Engine/EditorBlueprintResources/StandardMacros.IncrementInt` (`self.LazerCounter`))
      (:`  `
        (if (== _result 10)
          (goto _label_4))))))

(event `Ammo_Switch`
  ;[0 0 0] Add Info on Current Ammo Type
  (if (== (`self.Ammo_Int`) 1)
    (set `self.Ammo_Type` "Base")
    (set `self.Ammo_Now` (`self.Ammo_In_Base`))
    (set `self.Max_Ammo` 15)
    (set `self.Reload_Time` 3.0)
    (set `self.Ammo_Damage` 20.0)
    (set `self.Ammo_Range` (6000.0 6000.0 6000.0))
    (set `self.Ammo_Pause` 0.5)
    (elif (== (`self.Ammo_Int`) 2)
      (set `self.Ammo_Type` "Stun")
      (set `self.Ammo_Now` (`self.Ammo_In_Stun`))
      (set `self.Max_Ammo` 10)
      (set `self.Reload_Time` 3.0)
      (set `self.Ammo_Damage` 5.0)
      (set `self.Ammo_Range` (5000.0 5000.0 5000.0))
      (set `self.Ammo_Pause` 0.5)
      (elif (== (`self.Ammo_Int`) 3)
        (set `self.Ammo_Type` "Shield")
        (set `self.Ammo_Now` (`self.Ammo_In_Shield`))
        (set `self.Max_Ammo` 3)
        (set `self.Reload_Time` 4.0)
        (set `self.Ammo_Damage` 15.0)
        (set `self.Ammo_Range` (5000.0 5000.0 5000.0))
        (set `self.Ammo_Pause` 0.5)
        (else
          (set `self.Ammo_Type` "AoE")
          (set `self.Ammo_Now` (`self.Ammo_In_AoE`))
          (set `self.Max_Ammo` 1)
          (set `self.Reload_Time` 5.0)
          (set `self.Ammo_Damage` 40.0)
          (set `self.Ammo_Range` (4000.0 4000.0 4000.0))
          (set `self.Ammo_Pause` 0.0)))))
  (if (`self.Reloading_Now`)
    (set `self.Was_Switched` true)
    (`/Game/NovaeTerrae/UI/Char_WG/Crosshair_Aim.Cancel_Filling_Bar` (`self.Crosshair_Aim`))
    (else
      (set `self.Was_Switched` false))))

(event `Save info on current ammo`
  ;[0 0 0] Save Info on Current Ammo Before Switching
  (if (== (`self.Ammo_Int`) 1)
    (if (== (`self.Ammo_Max`) 1)
      (set `self.Ammo_In_Base` (`self.Ammo_Now`)))
    (elif (== (`self.Ammo_Int`) 2)
      (if (`self.Stun_Unlocked`)
        (set `self.Ammo_In_Stun` (`self.Ammo_Now`)))
      (elif (== (`self.Ammo_Int`) 3)
        (if (`self.Shield_Unlocked`)
          (set `self.Ammo_In_Shield` (`self.Ammo_Now`)))
        (elif (`self.AoE_Unlocked`)
          (set `self.Ammo_In_AoE` (`self.Ammo_Now`)))))))

(event `Key|RightMouseButton`
  (params (Key :type "Key Structure"))
  ;[0 0 0] Aim Mode On / Off
  (:`Pressed`
    (`/Engine/EditorBlueprintResources/StandardMacros.FlipFlop`
      (:`A`
        (set `self.Aim_Mode` true)
        (bind (_direction _take_aim) (`Timeline|Change View` :!via `PlayFromStart` :!label _label_6)
          (:`Update`
            (bind _returnvalue_location (`KismetMathLibrary.BreakTransform` (`KismetMathLibrary.TLerp` (`KismetMathLibrary.MakeTransform` (-150.0 50.0 65.0)) (`KismetMathLibrary.MakeTransform` (-100.0 50.0 60.0)) _take_aim)))
            (set `SpringArmComponent.SocketOffset` _returnvalue_location (`self.SpringArmComponent`)))))
      (:`B`
        (set `self.Aim_Mode` false)
        (goto _label_6 :!via `ReverseFromEnd`)))))

(event `Pause_Shots`
  ;[0 0 0] Pause Between Shots
  (set `self.Pause` true)
  (`/Game/NovaeTerrae/UI/Char_WG/Crosshair_Aim.Anim_Choice` (`self.Crosshair_Aim`))
  (`KismetSystemLibrary.Delay` (`self.Ammo_Pause`))
  (set `self.Pause` false))

(event `Key|MouseScrollUp`
  (params (Key :type "Key Structure"))
  ;[0 0 0] Switch Ammo Type With Mouse Wheel
  (:`Pressed`
    (if (and (!= (`self.Ammo_Max`) 1) (>= (`self.Ammo_Max`) (`self.Ammo_Int`)))
      (`self.Save info on current ammo`)
      (set `self.Have Ammo` true)
      (if (== (`self.Ammo_Max`) (`self.Ammo_Int`))
        (set `self.Ammo_Int` 1)
        (else
          (bind _result (`/Engine/EditorBlueprintResources/StandardMacros.IncrementInt` (`self.Ammo_Int`))
            (:`  `
              (set `self.Ammo_Int` _result)))))
      (`self.Ammo_Switch` :!label _label_7))))

(event `Key|One`
  (params (Key :type "Key Structure"))
  ;[0 0 0] Switch Ammo Type With Keys
  (:`Pressed`
    (if (not (== (`self.Ammo_Max`) 1))
      (`self.Save info on current ammo`)
      (set `self.Have Ammo` true)
      (set `self.Ammo_Int` 1)
      (`self.Ammo_Switch` :!label _label_8))))

(event `Aoe_Explosion`
  (params (`Explosion Point` :type "Vector Structure"))
  (bind _aoe_explosion_radius (`self.AoE_Explosion_Radius`))
  ;[0 0 0] AoE Ammo Explosion
  ;;[0 0 0] Это для наглядности, можно удалить
  (`KismetSystemLibrary.SphereTraceMulti` :`Start` `Explosion Point` :`End` `Explosion Point` :`Radius` _aoe_explosion_radius :`TraceChannel` "TraceTypeQuery1" :`DrawDebugType` "ForDuration" :`TraceHitColor` (struct :`R` 1.0 :`B` 0.047856 :`A` 1.0) :`DrawTime` 1.0)
  (`GameplayStatics.ApplyRadialDamage` :`BaseDamage` (`self.Ammo_Damage`) :`Origin` `Explosion Point` :`DamageRadius` _aoe_explosion_radius :`DamageCauser` self :`InstigatedByController` null :`bDoFullDamage` true))

(event `Key|Two`
  (params (Key :type "Key Structure"))
  ;[0 0 0] Switch Ammo Type With Keys
  (:`Pressed`
    (if (`self.Stun_Unlocked`)
      (`self.Save info on current ammo`)
      (set `self.Have Ammo` true)
      (set `self.Ammo_Int` 2)
      (goto _label_8))))

(event `Key|Three`
  (params (Key :type "Key Structure"))
  ;[0 0 0] Switch Ammo Type With Keys
  (:`Pressed`
    (if (`self.Shield_Unlocked`)
      (`self.Save info on current ammo`)
      (set `self.Have Ammo` true)
      (set `self.Ammo_Int` 3)
      (goto _label_8))))

(event `Key|MouseScrollDown`
  (params (Key :type "Key Structure"))
  ;[0 0 0] Switch Ammo Type With Mouse Wheel
  (:`Pressed`
    (if (and (!= (`self.Ammo_Max`) 1) (>= (`self.Ammo_Max`) (`self.Ammo_Int`)))
      (`self.Save info on current ammo`)
      (set `self.Have Ammo` true)
      (if (== (`self.Ammo_Int`) 1)
        (set `self.Ammo_Int` (`self.Ammo_Max`))
        (goto _label_7)
        (else
          (bind _result (`/Engine/EditorBlueprintResources/StandardMacros.DecrementInt` (`self.Ammo_Int`))
            (:`  `
              (set `self.Ammo_Int` _result)
              (goto _label_7))))))))

(event `Key|Four`
  (params (Key :type "Key Structure"))
  ;[0 0 0] Switch Ammo Type With Keys
  (:`Pressed`
    (if (`self.AoE_Unlocked`)
      (`self.Save info on current ammo`)
      (set `self.Have Ammo` true)
      (set `self.Ammo_Int` 4)
      (goto _label_8))))

(event `Change_Crosshair`
  ;[0 0 0] Check if looking at the enemy
)

(event `Interact_wth_Obj`
  (bind _returnvalue (`GameplayStatics.GetPlayerCameraManager` 0))
  (bind _returnvalue_2 (`self.K2_GetActorLocation` _returnvalue))
  ;[0 0 0] Interact with object
  (bind (_outhit _returnvalue_3) (`KismetSystemLibrary.LineTraceSingle` :`Start` _returnvalue_2 :`End` (+ _returnvalue_2 (* (`self.GetActorForwardVector` _returnvalue) (600.0 600.0 600.0))) :`TraceChannel` "TraceTypeQuery1" :`DrawDebugType` "ForDuration" :`TraceColor` (struct :`R` 1.0 :`B` 0.987977 :`A` 1.0) :`DrawTime` 2.0))
  (if _returnvalue_3
    (bind (_bblockinghit _binitialoverlap _time _distance _location _impactpoint _normal _impactnormal _physmat _hitactor) (`GameplayStatics.BreakHitResult` _outhit))
    ;;[0.151 0 0.1493] Pick Up Key
    (if (`self.ActorHasTag` _hitactor "Key")
      (set `self.Old_Key` (`self.Current_Key`))
      (`self.K2_DestroyActor` _hitactor)
      (else
        ;;[0.151 0 0.1493] Open Chest
        (if (`self.ActorHasTag` _hitactor "Chest")
          (set `self.Open_Chest` true)
          (`KismetSystemLibrary.Delay` 1.0)
          (set `self.Open_Chest` false)
          (else
            ;;[0.151 0 0.1493] Pick Up Ammo
            (if (`self.ActorHasTag` _hitactor "Ammo")
              (`self.K2_DestroyActor` _hitactor)
              (else
                ;;[0.151 0 0.1493] Push Button
                (if (`self.ActorHasTag` _hitactor "Button")
                  (set `self.Push_Button` true)
                  (`KismetSystemLibrary.Delay` 0.1)
                  (set `self.Push_Button` false)
                  (else
                    ;;[0.15 0 0.15] Change Panel Color
                    (if (`self.ActorHasTag` _hitactor "Panel_1")
                      (set `self.Change_Panel_1` true)
                      (`KismetSystemLibrary.Delay` 0.1 :!label _label_9)
                      (set `self.Change_Panel_1` false)
                      (set `self.Change_Panel_2` false)
                      (set `self.Change_Panel_3` false)
                      (elif (`self.ActorHasTag` _hitactor "Panel_2")
                        (set `self.Change_Panel_2` true)
                        (goto _label_9)
                        (elif (`self.ActorHasTag` _hitactor "Panel_3")
                          (set `self.Change_Panel_3` true)
                          (goto _label_9))))))))))))))

(event `Check_Save`
  ;[0 0 0] Load / Create Save Game
  (bind _returnvalue (`GameplayStatics.DoesSaveGameExist` "Save_Info"))
  (if _returnvalue
    (bind _returnvalue_2 (`GameplayStatics.LoadGameFromSlot` "Save_Info"))
    (bind _asbp_save (cast `/Game/NovaeTerrae/Puzzles/Altar/BP_Save` _returnvalue_2))
    (set `self.Save_Ref` _asbp_save)
    (`self.K2_SetActorTransform` (`/Game/NovaeTerrae/Puzzles/Altar/BP_Save.Char_Location` _asbp_save))
    (else
      (bind _returnvalue_3 (`GameplayStatics.CreateSaveGameObject` "/Game/NovaeTerrae/Puzzles/Altar/BP_Save.BP_Save_C"))
      (`GameplayStatics.SaveGameToSlot` _returnvalue_3 "Save_Info")
      (set `self.Save_Ref` _returnvalue_3))))

(fn `GetReloadTime`
  (returns (Reload :type "Float (double-precision)"))
  (return (`KismetMathLibrary.SelectFloat` 0.1 (`self.Reload_Time`) (`self.IsFastReloadEnabled`))))

(fn `UserConstructionScript`)