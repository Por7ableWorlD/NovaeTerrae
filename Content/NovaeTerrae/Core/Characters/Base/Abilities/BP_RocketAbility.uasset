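; Rocket ability for the player character that fires limited homing missiles, one per use, at the nearest enemy.
; Each use while off cooldown spawns a BP_HomingMissile at the user's shooting point and passes it damage and blast radius.
; A linear distance search over all NTBaseEnemyCharacter actors picks the homing target.
; Spending the last missile starts the cooldown, whose completion event refills the missile count.
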(event `self.ReceiveBeginPlay`
  (bind _asbp_ntbase_character (cast `/Game/NovaeTerrae/Core/Characters/Base/BP_NTBaseCharacter` (`GameplayStatics.GetPlayerCharacter` 0)))
  (set `self.AbilityUser` _asbp_ntbase_character)
  (set `self.CurrentNumberOfMissiles` (`self.MaxNumberOfMissiles`))
  (set `self.Cooldown` 15.0)
  (add `self.OnAbilityCooldownFinished` (delegate `ResetMissiles`)))

(event `ResetMissiles`
  (set `self.CurrentNumberOfMissiles` (`self.MaxNumberOfMissiles`)))

(event `/Game/NovaeTerrae/Core/Characters/Base/Abilities/BPI_AbilityInterface.UseAbility`
  (bind _currentnumberofmissiles (`self.CurrentNumberOfMissiles`))
  (if (`|EnumEquality` (`self.AbilityState`) "NewEnumerator0")
    (if (> _currentnumberofmissiles 0)
      (`/Engine/EditorBlueprintResources/StandardMacros.DecrementInt` _currentnumberofmissiles
        (:`  `
          (`KismetSystemLibrary.PrintString` (`KismetStringLibrary.Concat_StrStr` "Missiles Left:" (`KismetStringLibrary.Conv_IntToString` _currentnumberofmissiles)))
          (bind _outactors (`GameplayStatics.GetAllActorsOfClass` "/Script/NovaeTerrae.NTBaseEnemyCharacter"))
          (bind _closestenemy (`self.FindClosestEnemy` _outactors))
          (bind _returnvalue (`|SpawnActorFromClass` "/Game/NovaeTerrae/AI/Blueprints/BP_HomingMissile.BP_HomingMissile_C" (`KismetMathLibrary.MakeTransform` (`SceneComponent.K2_GetComponentLocation` (`/Game/NovaeTerrae/Core/Characters/Base/BP_NTBaseCharacter.Shooting_Point` (`self.AbilityUser`))) (`self.K2_GetActorRotation`)) "Undefined" "MultiplyWithRoot" (`self.AbilityUser`) null))
          (`/Game/NovaeTerrae/AI/Blueprints/BP_HomingMissile.SetupHomingMissile` _returnvalue)
          (set `ProjectileMovementComponent.HomingTargetComponent` (`Actor.RootComponent` _closestenemy) (`/Game/NovaeTerrae/AI/Blueprints/BP_HomingMissile.ProjectileMovement` _returnvalue))
          (`/Game/NovaeTerrae/AI/Blueprints/BP_HomingMissile.SetupParameters` _returnvalue (`self.MissilesDamage`) (`self.DamageRadius`))
          (if (== (`self.CurrentNumberOfMissiles`) 0)
            (`self.StartCooldown`)))))
    (else
      (`KismetSystemLibrary.PrintString` "Ability on cooldown!" true true (struct :`R` 1.0 :`A` 1.0)))))

(event `/Game/NovaeTerrae/Core/Characters/Base/Abilities/BPI_AbilityInterface.StopChannelingAbility`)

(fn `FindClosestEnemy`
  (params (Enemies :type "Array of NTBaseEnemyCharacter Object Reference"))
  (returns (ClosestEnemy :type "NTBaseEnemyCharacter Object Reference"))
  (locals (Result :type "NTBaseEnemyCharacter Object Reference") (ClosestDistance :type "Float (double-precision)"))
  (for (_array_element _array_index) (`local.Enemies`)
    (if (!= _array_index 0)
      (bind _returnvalue (`self.GetDistanceTo` _array_element (`self.AbilityUser`)))
      (if (< _returnvalue (`local.ClosestDistance`))
        (set `local.Result` _array_element :!label _label)
        (set `local.ClosestDistance` _returnvalue))
      (else
        (goto _label))))
  (return (`local.Result`)))

(fn `UserConstructionScript`
  (`parent.UserConstructionScript`))