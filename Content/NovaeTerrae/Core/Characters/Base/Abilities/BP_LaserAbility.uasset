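; Channeled laser ability that fires from the player character toward the point the camera aims at, damaging what it hits.
; UseAbility starts looping EmitLaser and duration timers; Clear, on timeout or early stop, ends the beam and starts cooldown.
; Each tick sphere-traces while ignoring player and companion, updates the Niagara beam endpoint, applies damage, and sends the hit actor a reflect message with trace data.
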(event `self.ReceiveBeginPlay`
  (set `self.Camera` (`GameplayStatics.GetPlayerCameraManager` 0))
  (set `self.AbilityUser` (`GameplayStatics.GetPlayerCharacter` 0))
  (bind _returnvalue (`GameplayStatics.GetActorOfClass` "/Game/NovaeTerrae/AI/Companion/BP_Companion.BP_Companion_C"))
  (set `self.ActorsToIgnore` (`|MakeArray` _returnvalue (`self.AbilityUser`) :!type "Actor Object Reference"))
  (set `self.Cooldown` 5.0))

(event `self.ReceiveTick`
  (params (DeltaSeconds :type "Float (single-precision)")))

(event `/Game/NovaeTerrae/Core/Characters/Base/Abilities/BPI_AbilityInterface.UseAbility`
  (if (`|EnumEquality` (`self.AbilityState`) "NewEnumerator0")
    (set `self.AbilityState` "NewEnumerator1")
    (bind _returnvalue (`KismetSystemLibrary.K2_SetTimerDelegate` (delegate `EmitLaser`) 0.02 true (`self.AttackDelay`)))
    (set `self.LaserTimer` _returnvalue)
    (bind _returnvalue_2 (`NiagaraFunctionLibrary.SpawnSystemAtLocation` "/Game/NovaeTerrae/Art/VFX/NS_laser_eyes.NS_laser_eyes" (`self.K2_GetActorLocation` (`self.AbilityUser`)) (struct) (1.0 1.0 1.0) true false))
    (set `self.Laser` _returnvalue_2)
    (bind _returnvalue_3 (`KismetSystemLibrary.K2_SetTimerDelegate` (delegate `Clear`) (`self.LaserDuration`) false (`self.AttackDelay`)))
    (set `self.ClearTimer` _returnvalue_3)
    (else
      (`KismetSystemLibrary.PrintString` "Ability on cooldown!" true true (struct :`R` 1.0 :`A` 1.0)))))

(event `Clear`
  (`KismetSystemLibrary.K2_ClearAndInvalidateTimerHandle` (`self.LaserTimer`))
  (`ActorComponent.Deactivate` (`self.Laser`))
  (`self.StartCooldown`))

(event `EmitLaser`
  (bind _outhit (`KismetSystemLibrary.SphereTraceSingle` (`self.GetLaserStart`) (`self.GetLaserEnd`) 15.0 "TraceTypeQuery2" false (`self.ActorsToIgnore`)))
  (`FXSystemComponent.SetVectorParameter` (`self.Laser`) "LaserEnd" (`KismetMathLibrary.SelectVector` (`.Location` (`GameplayStatics.BreakHitResult` _outhit)) (`self.GetLaserEnd`) (`GameplayStatics.BreakHitResult` _outhit)))
  (`SceneComponent.K2_SetWorldLocation` (`self.Laser`) (`self.GetLaserStart`) false true)
  (if (not (`ActorComponent.IsActive` (`self.Laser`)))
    (`ActorComponent.Activate` (`self.Laser`) false))
  (`GameplayStatics.ApplyDamage` (`.HitActor` (`GameplayStatics.BreakHitResult` _outhit)) (`self.LaserTickDamage`) null (`self.AbilityUser`) "/Script/NovaeTerrae.LazerDamageType")
  (message `/Game/NovaeTerrae/Puzzles/Mirrors/BPI_ReflectableInterface.Reflect` (`.HitActor` (`GameplayStatics.BreakHitResult` _outhit)) (`.Location` (`GameplayStatics.BreakHitResult` _outhit)) (`.TraceStart` (`GameplayStatics.BreakHitResult` _outhit)) (`.TraceEnd` (`GameplayStatics.BreakHitResult` _outhit)) (`.Normal` (`GameplayStatics.BreakHitResult` _outhit))))

(event `/Game/NovaeTerrae/Core/Characters/Base/Abilities/BPI_AbilityInterface.StopChannelingAbility`
  (if (`|EnumEquality` (`self.AbilityState`) "NewEnumerator1")
    (`self.Laser`
      (:`then`
        (`KismetSystemLibrary.K2_ClearAndInvalidateTimerHandle` (`self.ClearTimer`))
        (`self.Clear`))
      (:`else`))))

(fn `GetLaserEnd`
  (returns (LaserEnd :type "Vector Structure"))
  (bind _camera (`self.Camera`))
  (return (+ (`self.K2_GetActorLocation` _camera) (* (`self.GetActorForwardVector` _camera) (`self.AttackDistance`)))))

(fn `GetLaserStart`
  (returns (LaserStart :type "Vector Structure"))
  (return (`self.K2_GetActorLocation` (`self.AbilityUser`))))

(fn `UserConstructionScript`)