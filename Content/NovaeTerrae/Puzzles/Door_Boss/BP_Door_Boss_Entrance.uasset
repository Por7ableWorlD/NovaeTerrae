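; Boss room entrance door that closes once the companion enters its trigger and stays closed across saved games.
; After a 3-second delay, the Close timeline sets the mesh from a start-to-end point lerp, though Alpha is fixed at zero.
; Each timeline update flags the door closed and, if the Save_Info slot exists, saves it through the player character's save reference.
; BeginPlay reads that slot and snaps the door shut if flagged.
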(event `self.ReceiveBeginPlay`
  ;[0 0 0] Begin Play
  (bind _asbp_ntbase_character (cast `/Game/NovaeTerrae/Core/Characters/Base/BP_NTBaseCharacter` (`GameplayStatics.GetPlayerCharacter` 0)))
  (set `self.Char_Ref` _asbp_ntbase_character)
  (bind _returnvalue (`GameplayStatics.LoadGameFromSlot` "Save_Info"))
  (bind _asbp_save (cast `/Game/NovaeTerrae/Puzzles/Altar/BP_Save` _returnvalue))
  (if (`/Game/NovaeTerrae/Puzzles/Altar/BP_Save.Boss_Entrance_Door_Pos` _asbp_save)
    (set `self.Door_Closed` true)
    (`SceneComponent.K2_SetRelativeTransform` (`self.Door_Mesh`) (`SceneComponent.GetRelativeTransform` (`self.Door_MeshEndPoint`)) false false)))

(event `self.Trigger.OnComponentBeginOverlap`
  (params (OverlappedComponent :type "PrimitiveComponent Object Reference") (OtherActor :type "Actor Object Reference") (OtherComp :type "PrimitiveComponent Object Reference") (OtherBodyIndex :type Integer) (bFromSweep :type Boolean) (SweepResult :type "HitResult Structure (by ref)"))
  (bind _save_ref (`/Game/NovaeTerrae/Core/Characters/Base/BP_NTBaseCharacter.Save_Ref` (`self.Char_Ref`)))
  ;[0 0 0] Close Door
  (cast `/Game/NovaeTerrae/AI/Companion/BP_Companion` OtherActor)
  (`KismetSystemLibrary.Delay` 3.0)
  (`Timeline|Close` :!via `PlayFromStart`
    (:`Update`
      (`SceneComponent.K2_SetRelativeTransform` (`self.Door_Mesh`) (`KismetMathLibrary.TLerp` (`SceneComponent.GetRelativeTransform` (`self.Door_MeshStartPoint`)) (`SceneComponent.GetRelativeTransform` (`self.Door_MeshEndPoint`))) false false)
      (set `self.Door_Closed` true)
      (bind _returnvalue (`GameplayStatics.DoesSaveGameExist` "Save_Info"))
      (if _returnvalue
        (set `/Game/NovaeTerrae/Puzzles/Altar/BP_Save.Boss_Entrance_Door_Pos` (`self.Door_Closed`) _save_ref)
        (`GameplayStatics.SaveGameToSlot` _save_ref "Save_Info")))))

(fn `UserConstructionScript`)