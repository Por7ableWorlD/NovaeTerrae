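; BP_Door_Boss is a boss door whose mesh slides open when its death handler fires.
; OnDeath_Event plays the Open_Boss_Door timeline, lerping DoorMesh's relative transform between start and end point components.
; The nodes that would bind this handler to a BP_DistortedHunter's HealthComponent death event are disconnected, so nothing in this Blueprint triggers the opening.
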(event `OnDeath_Event`
  (params (GetAbility :type Boolean))
  (bind (_direction _door_open) (`Timeline|Open_Boss_Door` :!via `PlayFromStart`)
    (:`Update`
      (`SceneComponent.K2_SetRelativeTransform` (`self.Door_Mesh`) (`KismetMathLibrary.TLerp` (`SceneComponent.GetRelativeTransform` (`self.Door_MeshStartPoint`)) (`SceneComponent.GetRelativeTransform` (`self.Door_MeshEndPoint`)) _door_open) false false))))

(fn `UserConstructionScript`)