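; BP_Elevator is a puzzle elevator that lowers its platform when the companion steps onto it.
; An overlap of BP_Companion with the trigger starts a three-second delay, then moves the platform only if WaitingPlayer is set, clearing that flag first.
; The Moving_Down timeline lerps the mesh's relative transform between start and end point components, with no return movement.
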(event `self.Trigger.OnComponentBeginOverlap`
  (params (OverlappedComponent :type "PrimitiveComponent Object Reference") (OtherActor :type "Actor Object Reference") (OtherComp :type "PrimitiveComponent Object Reference") (OtherBodyIndex :type Integer) (bFromSweep :type Boolean) (SweepResult :type "HitResult Structure (by ref)"))
  ;[0 0 0] Step On The Elevator Platform
  (cast `/Game/NovaeTerrae/AI/Companion/BP_Companion` OtherActor)
  (`KismetSystemLibrary.Delay` 3.0)
  (if (`self.Waiting_Player`)
    (set `self.Waiting_Player` false)
    (`self.Down`)))

(event `Down`
  ;[0 0 0] Platform Goes Down
  (bind (_direction _down) (`Timeline|Moving_Down` :!via `PlayFromStart`)
    (:`Update`
      (`SceneComponent.K2_SetRelativeTransform` (`self.Elevator_Mesh`) (`KismetMathLibrary.TLerp` (`SceneComponent.GetRelativeTransform` (`self.Elevator_StartPoint`)) (`SceneComponent.GetRelativeTransform` (`self.Elevator_EndPoint`)) _down) false false))))

(fn `UserConstructionScript`)