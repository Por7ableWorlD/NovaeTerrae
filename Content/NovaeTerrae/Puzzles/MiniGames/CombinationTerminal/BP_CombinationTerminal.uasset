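; BP_CombinationTerminal is a combination terminal puzzle minigame actor that generates and displays random symbol sequences.
; On BeginPlay, GenerateGame fills a map with one randomly generated symbol sequence of configurable length per E_Direction value, each with a current index starting at zero.
; It then converts four of those sequences to strings and shows each on its own TextRender component.
; No input handling or solution checking is implemented here.
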(event `self.ReceiveBeginPlay`
  (`self.GenerateGame`)
  (set `self.String` "")
  (for _array_element (break `/Game/NovaeTerrae/Puzzles/MiniGames/CombinationTerminal/S_SymbolSequence` (`BlueprintMapLibrary.Map_Find` (`self.SymbolSequences`) "NewEnumerator0"))
    (set `self.String` (`KismetStringLibrary.Concat_StrStr` (`self.String`) (`|GetEnumeratorNameAsString` _array_element))))
  (`TextRenderComponent.K2_SetText` (`self.TextRender`) (`KismetTextLibrary.Conv_StringToText` (`self.String`)))
  (set `self.String` "")
  (for _array_element_2 (break `/Game/NovaeTerrae/Puzzles/MiniGames/CombinationTerminal/S_SymbolSequence` (`BlueprintMapLibrary.Map_Find` (`self.SymbolSequences`) "NewEnumerator1"))
    (set `self.String` (`KismetStringLibrary.Concat_StrStr` (`self.String`) (`|GetEnumeratorNameAsString` _array_element_2))))
  (`TextRenderComponent.K2_SetText` (`self.TextRender1`) (`KismetTextLibrary.Conv_StringToText` (`self.String`)))
  (set `self.String` "")
  (for _array_element_3 (break `/Game/NovaeTerrae/Puzzles/MiniGames/CombinationTerminal/S_SymbolSequence` (`BlueprintMapLibrary.Map_Find` (`self.SymbolSequences`) "NewEnumerator2"))
    (set `self.String` (`KismetStringLibrary.Concat_StrStr` (`self.String`) (`|GetEnumeratorNameAsString` _array_element_3))))
  (`TextRenderComponent.K2_SetText` (`self.TextRender2`) (`KismetTextLibrary.Conv_StringToText` (`self.String`)))
  (set `self.String` "")
  (for _array_element_4 (break `/Game/NovaeTerrae/Puzzles/MiniGames/CombinationTerminal/S_SymbolSequence` (`BlueprintMapLibrary.Map_Find` (`self.SymbolSequences`) "NewEnumerator3"))
    (set `self.String` (`KismetStringLibrary.Concat_StrStr` (`self.String`) (`|GetEnumeratorNameAsString` _array_element_4))))
  (`TextRenderComponent.K2_SetText` (`self.TextRender3`) (`KismetTextLibrary.Conv_StringToText` (`self.String`))))

(fn `GenerateGame`
  (bind _enumvalue (foreach `/Game/NovaeTerrae/Puzzles/MiniGames/CombinationTerminal/E_Direction` false)
    (:`LoopBody`
      (`BlueprintMapLibrary.Map_Add` (`self.SymbolSequences`) _enumvalue (make `/Game/NovaeTerrae/Puzzles/MiniGames/CombinationTerminal/S_SymbolSequence` (`self.GenerateSymbolSequenceOfSize` (`self.NumberOfSymbolsInSequence`)))))))

(fn `GenerateSymbolSequenceOfSize`
  (params (Size :type Integer))
  (returns (SymbolSequence :type "Array of /Game/NovaeTerrae/Puzzles/MiniGames/CombinationTerminal/E_Symbol Enum"))
  (locals (Sequence :type "Array of /Game/NovaeTerrae/Puzzles/MiniGames/CombinationTerminal/E_Symbol Enum"))
  (bind _result (`/Engine/EditorBlueprintResources/StandardMacros.DecrementInt` Size)
    (:`  `
      (for _ (range (+ _result 1))
        (`KismetArrayLibrary.Array_Add` (`local.Sequence`) (cast `/Game/NovaeTerrae/Puzzles/MiniGames/CombinationTerminal/E_Symbol` (`KismetMathLibrary.Conv_IntToByte` (`KismetMathLibrary.RandomIntegerInRange` 0 (- (enumcount `/Game/NovaeTerrae/Puzzles/MiniGames/CombinationTerminal/E_Symbol`) 1))))))
      (return (`local.Sequence`)))))

(fn `UserConstructionScript`)