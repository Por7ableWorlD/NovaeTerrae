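; BP_Level_Up_Object is an inspectable item for the LevelUpGame puzzle minigame that the player picks up and rotates with the mouse.
; Starting interaction moves the mesh to the character's ItemSlot and shows the cursor; stopping restores its position, zeroes rotation and returns game-only input.
; Mouse movement applies incremental combined yaw and pitch rotations while either button flag is set.
; The release handlers are crossed, each clearing the opposite button's flag.
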(event `self.ReceiveBeginPlay`
  (`StaticMeshComponent.SetStaticMesh` (`self.Obj_Mesh`) (`self.Mesh`))
  (bind _asbp_ntbase_character (cast `/Game/NovaeTerrae/Core/Characters/Base/BP_NTBaseCharacter` (`GameplayStatics.GetPlayerCharacter` 0)))
  (set `self.Char_Ref` _asbp_ntbase_character))

(event `/Game/NovaeTerrae/Puzzles/BPI_InteractionInterface.StartInteraction`
  ;[0 0 0] Pick Up Item
  (`parent.StartInteraction`)
  (set `self.DefaultMeshPos` (`SceneComponent.K2_GetComponentLocation` (`self.Obj_Mesh`)))
  (`SceneComponent.K2_SetWorldLocation` (`self.Obj_Mesh`) (`SceneComponent.K2_GetComponentLocation` (`/Game/NovaeTerrae/Core/Characters/Base/BP_NTBaseCharacter.Item_Slot` (`self.Char_Ref`))) false false)
  (set `PlayerController.bShowMouseCursor` true (`GameplayStatics.GetPlayerController` 0)))

(event `/Game/NovaeTerrae/Puzzles/BPI_InteractionInterface.StopInteraction`
  (bind _obj_mesh (`self.Obj_Mesh`))
  ;[0 0 0] Put Item Down
  (`self.LeftGame`)
  (`SceneComponent.K2_SetWorldLocation` _obj_mesh (`self.DefaultMeshPos`) false false)
  (`SceneComponent.K2_SetWorldRotation` :`self` _obj_mesh)
  (set `PlayerController.bShowMouseCursor` false (`GameplayStatics.GetPlayerController` 0))
  (set `self.Left_Mouse_Pressed` false)
  (set `self.Right_Mouse_Pressed` false)
  (`WidgetBlueprintLibrary.SetInputMode_GameOnly` (`GameplayStatics.GetPlayerController` 0)))

(event `/Game/NovaeTerrae/Puzzles/BPI_MiniGameInterface.MouseMove`
  (params (AxisValue :type "Vector2D Structure"))
  (bind (_x _y) (`KismetMathLibrary.BreakVector2D` AxisValue))
  (if (or (`self.Left_Mouse_Pressed`) (`self.Right_Mouse_Pressed`))
    (`SceneComponent.K2_SetRelativeRotation` (`self.Obj_Mesh`) (`KismetMathLibrary.ComposeRotators` (`SceneComponent.RelativeRotation` (`self.Obj_Mesh`)) (`KismetMathLibrary.MakeRotator` 0.0 0.0 (* _x -6.0))) false false)
    (`SceneComponent.K2_SetRelativeRotation` (`self.Obj_Mesh`) (`KismetMathLibrary.ComposeRotators` (`SceneComponent.RelativeRotation` (`self.Obj_Mesh`)) (`KismetMathLibrary.MakeRotator` 0.0 (* _y 6.0))) false false)))

(event `/Game/NovaeTerrae/Puzzles/BPI_MiniGameInterface.MouseLeftClick`
  (set `self.Left_Mouse_Pressed` true))

(event `/Game/NovaeTerrae/Puzzles/BPI_MiniGameInterface.MouseRightClick`
  (set `self.Right_Mouse_Pressed` true))

(event `/Game/NovaeTerrae/Puzzles/BPI_MiniGameInterface.MouseRightRelease`
  (set `self.Left_Mouse_Pressed` false))

(event `/Game/NovaeTerrae/Puzzles/BPI_MiniGameInterface.MouseLeftRelease`
  (set `self.Right_Mouse_Pressed` false))

(fn `UserConstructionScript`)