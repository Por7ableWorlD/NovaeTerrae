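; Interactable chest-puzzle minigame where the player clears random symbol sequences, one per direction, against a time limit.
; Up/Down/Left/Right inputs set the current direction, W/A/S/D submit symbols, and the first input starts the widget's timer.
; Each correct match advances that sequence and targets a random unfinished direction until all are complete.
; A wrong input or timeout regenerates the puzzle, updates WG_Chest_Puzzle and plays an audio event if running.
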(event `self.ReceiveBeginPlay`
  (`parent.ReceiveBeginPlay`))

(event `AddGameWidget`
  (bind _returnvalue (`|CreateWidget` "/Game/NovaeTerrae/UI/Puzzle_WG/WG_Chest_Puzzle.WG_Chest_Puzzle_C" null (`self.TimeLimit`)))
  (bind _output_get (set `self.GameWidget` _returnvalue))
  (`UserWidget.AddToViewport` _output_get 1)
  (add `/Game/NovaeTerrae/UI/Puzzle_WG/WG_Chest_Puzzle.ExitWidget` (`self.GameWidget`) (delegate `self.LeftGame`))
  (add `/Game/NovaeTerrae/UI/Puzzle_WG/WG_Chest_Puzzle.TimeFinished` (`self.GameWidget`) (delegate `TimeFinished`))
  (`/Game/NovaeTerrae/UI/Puzzle_WG/WG_Chest_Puzzle.PrepareArrays` (`self.GameWidget`)))

(event `TimeFinished`
  (`self.RestartGame`))

(event `self.LeftGame`
  (`/Game/NovaeTerrae/UI/Puzzle_WG/WG_Chest_Puzzle.LeaveGame` (`self.GameWidget`))
  (set `self.IsGameRunning` false)
  (`parent.LeftGame`))

(event `/Game/NovaeTerrae/Puzzles/BPI_InteractionInterface.StartInteraction`
  (if (`self.InteractionAvailable`)
    (`self.AddGameWidget`)
    (`self.RestartGame`)
    (`self.SetDirection` "NewEnumerator0")))

(event `self.GameFinished`
  (`/Game/NovaeTerrae/UI/Puzzle_WG/WG_Chest_Puzzle.StopTimer` (`self.GameWidget`))
  (`/Game/NovaeTerrae/UI/Puzzle_WG/WG_Chest_Puzzle.LeaveGame` (`self.GameWidget`))
  (`parent.GameFinished`))

(event `/Game/NovaeTerrae/Puzzles/BPI_InteractionInterface.StopInteraction`
  (`self.LeftGame`))

(event `/Game/NovaeTerrae/Puzzles/BPI_MiniGameInterface.StartRight`
  (`self.StartTimer`)
  (`self.SetDirection` "NewEnumerator3"))

(event `/Game/NovaeTerrae/Puzzles/BPI_MiniGameInterface.StartDown`
  (`self.StartTimer`)
  (`self.SetDirection` "NewEnumerator2"))

(event `/Game/NovaeTerrae/Puzzles/BPI_MiniGameInterface.StartLeft`
  (`self.StartTimer`)
  (`self.SetDirection` "NewEnumerator1"))

(event `/Game/NovaeTerrae/Puzzles/BPI_MiniGameInterface.StartUp`
  (`self.StartTimer`)
  (`self.SetDirection` "NewEnumerator0"))

(event `/Game/NovaeTerrae/Puzzles/BPI_MiniGameInterface.StartD`
  (`self.StartTimer`)
  (`self.CheckAction` "NewEnumerator3"))

(event `/Game/NovaeTerrae/Puzzles/BPI_MiniGameInterface.StartS`
  (`self.StartTimer`)
  (`self.CheckAction` "NewEnumerator2"))

(event `/Game/NovaeTerrae/Puzzles/BPI_MiniGameInterface.StartA`
  (`self.StartTimer`)
  (`self.CheckAction` "NewEnumerator1"))

(event `/Game/NovaeTerrae/Puzzles/BPI_MiniGameInterface.StartW`
  (`self.StartTimer`)
  (`self.CheckAction` "NewEnumerator0"))

(fn `CheckAction`
  (params (UsedSymbol :type "/Game/NovaeTerrae/Puzzles/MiniGames/CombinationGame/E_Symbol Enum" :default "NewEnumerator0"))
  (bind _value (`BlueprintMapLibrary.Map_Find` (`self.SymbolSequences`) (`self.TargetDirection`)))
  (if (and (`|EnumEquality` (`self.TargetDirection`) (`self.CurrentDirection`)) (`|EnumEquality` (`self.TargetSymbol`) (`local.UsedSymbol`)))
    (`/Game/NovaeTerrae/UI/Puzzle_WG/WG_Chest_Puzzle.SetFinishedSymbol` (`self.GameWidget`) (`self.TargetDirection`) (`.CurrentSymbolIndex_11_5F0482F44D200CF031243DB3823DC792` (break `/Game/NovaeTerrae/Puzzles/MiniGames/CombinationGame/S_SymbolSequence` _value)))
    (`BlueprintMapLibrary.Map_Add` (`self.SymbolSequences`) (`self.TargetDirection`) (make `/Game/NovaeTerrae/Puzzles/MiniGames/CombinationGame/S_SymbolSequence` (break `/Game/NovaeTerrae/Puzzles/MiniGames/CombinationGame/S_SymbolSequence` _value) (+ (`.CurrentSymbolIndex_11_5F0482F44D200CF031243DB3823DC792` (break `/Game/NovaeTerrae/Puzzles/MiniGames/CombinationGame/S_SymbolSequence` _value)) 1)))
    (bind (_targetindex _gamefinished) (`self.GetNextSymbol`))
    (if _gamefinished
      (`self.GameFinished`)
      (else
        (`/Game/NovaeTerrae/UI/Puzzle_WG/WG_Chest_Puzzle.UpdateActiveSymbol` (`self.GameWidget`) (`self.TargetDirection`) _targetindex (`self.TargetSymbol`))))
    (else
      (`self.RestartGame`))))

(fn `GenerateGame`
  (bind _enumvalue (foreach `/Game/NovaeTerrae/Puzzles/MiniGames/CombinationGame/E_Direction` false)
    (:`LoopBody`
      (`BlueprintMapLibrary.Map_Add` (`self.SymbolSequences`) _enumvalue (make `/Game/NovaeTerrae/Puzzles/MiniGames/CombinationGame/S_SymbolSequence` (`self.GenerateSymbolSequenceOfSize` (`self.NumberOfSymbolsInSequence`)))))))

(fn `GenerateSymbolSequenceOfSize`
  (params (Size :type Integer))
  (returns (SymbolSequence :type "Array of /Game/NovaeTerrae/Puzzles/MiniGames/CombinationGame/E_Symbol Enum"))
  (locals (Sequence :type "Array of /Game/NovaeTerrae/Puzzles/MiniGames/CombinationGame/E_Symbol Enum"))
  (bind _result (`/Engine/EditorBlueprintResources/StandardMacros.DecrementInt` Size)
    (:`  `
      (for _ (range (+ _result 1))
        (`KismetArrayLibrary.Array_Add` (`local.Sequence`) (cast `/Game/NovaeTerrae/Puzzles/MiniGames/CombinationGame/E_Symbol` (`KismetMathLibrary.Conv_IntToByte` (`KismetMathLibrary.RandomIntegerInRange` 0 (- (enumcount `/Game/NovaeTerrae/Puzzles/MiniGames/CombinationGame/E_Symbol`) 1))))))
      (return (`local.Sequence`)))))

(fn `GetNextSymbol`
  (returns (TargetIndex :type Integer) (GameFinished :type Boolean))
  (bind _value (`BlueprintMapLibrary.Map_Find` (`self.SymbolSequences`) (`self.TargetDirection`)))
  (bind (_direction _found) (`self.GetRandomDirection`))
  (if _found
    (set `self.TargetDirection` _direction)
    (set `self.TargetSymbol` (`|GetArrayItem` (break `/Game/NovaeTerrae/Puzzles/MiniGames/CombinationGame/S_SymbolSequence` _value) (`.CurrentSymbolIndex_11_5F0482F44D200CF031243DB3823DC792` (break `/Game/NovaeTerrae/Puzzles/MiniGames/CombinationGame/S_SymbolSequence` _value))))
    (return (`.CurrentSymbolIndex_11_5F0482F44D200CF031243DB3823DC792` (break `/Game/NovaeTerrae/Puzzles/MiniGames/CombinationGame/S_SymbolSequence` _value)) false)
    (else
      (return 0 true))))

(fn `GetRandomDirection`
  (returns (Direction :type "/Game/NovaeTerrae/Puzzles/MiniGames/CombinationGame/E_Direction Enum") (Found :type Boolean))
  (locals (DirectionPool :type "Array of /Game/NovaeTerrae/Puzzles/MiniGames/CombinationGame/E_Direction Enum"))
  (bind _returnvalue (`KismetArrayLibrary.Array_Length` (`local.DirectionPool`)))
  (bind _enumvalue (foreach `/Game/NovaeTerrae/Puzzles/MiniGames/CombinationGame/E_Direction` false)
    (:`LoopBody`
      (bind _value (`BlueprintMapLibrary.Map_Find` (`self.SymbolSequences`) _enumvalue))
      (if (> (`KismetArrayLibrary.Array_Length` (break `/Game/NovaeTerrae/Puzzles/MiniGames/CombinationGame/S_SymbolSequence` _value)) (`.CurrentSymbolIndex_11_5F0482F44D200CF031243DB3823DC792` (break `/Game/NovaeTerrae/Puzzles/MiniGames/CombinationGame/S_SymbolSequence` _value)))
        (`KismetArrayLibrary.Array_Add` (`local.DirectionPool`) _enumvalue)))
    (:`then`
      (if (> _returnvalue 0)
        (return (`|GetArrayItem` (`local.DirectionPool`) (`KismetMathLibrary.RandomIntegerInRange` 0 (- _returnvalue 1))) true)
        (else
          (return "NewEnumerator0" false))))))

(fn `RestartGame`
  (`BlueprintMapLibrary.Map_Clear` (`self.SymbolSequences`))
  (`self.GenerateGame`)
  (`/Game/NovaeTerrae/UI/Puzzle_WG/WG_Chest_Puzzle.SetSymbols` (`self.GameWidget`) (`self.SymbolSequences`))
  (bind _targetindex (`self.GetNextSymbol`))
  (`/Game/NovaeTerrae/UI/Puzzle_WG/WG_Chest_Puzzle.UpdateActiveSymbol` (`self.GameWidget`) (`self.TargetDirection`) _targetindex (`self.TargetSymbol`))
  (if (`self.IsGameRunning`)
    (set `self.IsGameRunning` false)
    (`/Game/NovaeTerrae/UI/Puzzle_WG/WG_Chest_Puzzle.ClearTimer` (`self.GameWidget`))
    (`FMODBlueprintStatics.PlayEventAtLocation` null (`self.GetTransform`))))

(fn `SetDirection`
  (params (NewDirection :type "/Game/NovaeTerrae/Puzzles/MiniGames/CombinationGame/E_Direction Enum" :default "NewEnumerator0"))
  (set `self.CurrentDirection` NewDirection)
  (bind _gamewidget (`self.GameWidget`)
    (:`then`
      (`/Game/NovaeTerrae/UI/Puzzle_WG/WG_Chest_Puzzle.ChangeDirection` _gamewidget (`self.CurrentDirection`)))
    (:`else`)))

(fn `StartTimer`
  (if (not (`self.IsGameRunning`))
    (`/Game/NovaeTerrae/UI/Puzzle_WG/WG_Chest_Puzzle.StartTimer` (`self.GameWidget`))
    (set `self.IsGameRunning` true)))

(fn `UserConstructionScript`
  (`parent.UserConstructionScript`))