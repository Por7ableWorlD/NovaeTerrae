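; One-time trigger pickup that unlocks a note, fragment or item in the player's journal.
; When a BP_NTBaseCharacter first overlaps Trigger, zero checks on NoteToGive, FragToGive and ItemToGive pick the type, and a matching HUD message appears.
; Per-type functions map that number to one of eight journal widget flags, then the journal saves the pickup.
; Only notes play an activation sound.
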(event `self.ReceiveBeginPlay`
  ;[0 0 0] Event Begin Play
  (bind _asbp_ntbase_character (cast `/Game/NovaeTerrae/Core/Characters/Base/BP_NTBaseCharacter` (`GameplayStatics.GetPlayerCharacter` 0)))
  (set `self.Char_Ref` _asbp_ntbase_character))

(event `self.Trigger.OnComponentBeginOverlap`
  (params (OverlappedComponent :type "PrimitiveComponent Object Reference") (OtherActor :type "Actor Object Reference") (OtherComp :type "PrimitiveComponent Object Reference") (OtherBodyIndex :type Integer) (bFromSweep :type Boolean) (SweepResult :type "HitResult Structure (by ref)"))
  ;[0 0 0] On Overlap
  (cast `/Game/NovaeTerrae/Core/Characters/Base/BP_NTBaseCharacter` OtherActor)
  (if (not (`self.Obj_Given`))
    (if (== (`self.Note_To_Give`) 0)
      (if (== (`self.Item_To_Give`) 0)
        (`/Game/NovaeTerrae/UI/Char_WG/WBP_Hud.Show_Message` (`/Game/NovaeTerrae/Core/Characters/Base/BP_NTBaseCharacter.Char_Hud_WG` (`self.Char_Ref`)) false true false false false)
        (`self.Frag_Number_To_Give`)
        (else
          (`/Game/NovaeTerrae/UI/Char_WG/WBP_Hud.Show_Message` (`/Game/NovaeTerrae/Core/Characters/Base/BP_NTBaseCharacter.Char_Hud_WG` (`self.Char_Ref`)) false false true false false :!label _label)
          (`self.Item_Number_To_Give`)))
      (elif (== (`self.Frag_To_Give`) 0)
        (`/Game/NovaeTerrae/UI/Char_WG/WBP_Hud.Show_Message` (`/Game/NovaeTerrae/Core/Characters/Base/BP_NTBaseCharacter.Char_Hud_WG` (`self.Char_Ref`)) true false false false false)
        (`FMODBlueprintStatics.PlayEvent2D` "/Game/FMOD/Events/Interactive/Int_Object_Activate.Int_Object_Activate")
        (`self.Note_Number_To_Give`)
        (else
          (goto _label))))
    (`/Game/NovaeTerrae/UI/System_WG/Journal_WG.Save Picked Obj Info` (`/Game/NovaeTerrae/Core/Characters/Base/BP_NTBaseCharacter.Journal_WG` (`self.Char_Ref`)))
    (set `self.Obj_Given` true)))

(fn `Frag_Number_To_Give`
  (if (== (`self.Frag_To_Give`) 1)
    (set `/Game/NovaeTerrae/UI/System_WG/Journal_WG.Frag_1_Unlocked` true (`/Game/NovaeTerrae/Core/Characters/Base/BP_NTBaseCharacter.Journal_WG` (`self.Char_Ref`)))
    (elif (== (`self.Frag_To_Give`) 2)
      (set `/Game/NovaeTerrae/UI/System_WG/Journal_WG.Frag_2_Unlocked` true (`/Game/NovaeTerrae/Core/Characters/Base/BP_NTBaseCharacter.Journal_WG` (`self.Char_Ref`)))
      (elif (== (`self.Frag_To_Give`) 3)
        (set `/Game/NovaeTerrae/UI/System_WG/Journal_WG.Frag_3_Unlocked` true (`/Game/NovaeTerrae/Core/Characters/Base/BP_NTBaseCharacter.Journal_WG` (`self.Char_Ref`)))
        (elif (== (`self.Frag_To_Give`) 4)
          (set `/Game/NovaeTerrae/UI/System_WG/Journal_WG.Frag_4_Unlocked` true (`/Game/NovaeTerrae/Core/Characters/Base/BP_NTBaseCharacter.Journal_WG` (`self.Char_Ref`)))
          (elif (== (`self.Frag_To_Give`) 5)
            (set `/Game/NovaeTerrae/UI/System_WG/Journal_WG.Frag_5_Unlocked` true (`/Game/NovaeTerrae/Core/Characters/Base/BP_NTBaseCharacter.Journal_WG` (`self.Char_Ref`)))
            (elif (== (`self.Frag_To_Give`) 6)
              (set `/Game/NovaeTerrae/UI/System_WG/Journal_WG.Frag_6_Unlocked` true (`/Game/NovaeTerrae/Core/Characters/Base/BP_NTBaseCharacter.Journal_WG` (`self.Char_Ref`)))
              (elif (== (`self.Frag_To_Give`) 7)
                (set `/Game/NovaeTerrae/UI/System_WG/Journal_WG.Frag_7_Unlocked` true (`/Game/NovaeTerrae/Core/Characters/Base/BP_NTBaseCharacter.Journal_WG` (`self.Char_Ref`)))
                (elif (== (`self.Frag_To_Give`) 8)
                  (set `/Game/NovaeTerrae/UI/System_WG/Journal_WG.Frag_8_Unlocked` true (`/Game/NovaeTerrae/Core/Characters/Base/BP_NTBaseCharacter.Journal_WG` (`self.Char_Ref`))))))))))))

(fn `Item_Number_To_Give`
  (if (== (`self.Item_To_Give`) 1)
    (set `/Game/NovaeTerrae/UI/System_WG/Journal_WG.Item_1_Unlocked` true (`/Game/NovaeTerrae/Core/Characters/Base/BP_NTBaseCharacter.Journal_WG` (`self.Char_Ref`)))
    (elif (== (`self.Item_To_Give`) 2)
      (set `/Game/NovaeTerrae/UI/System_WG/Journal_WG.Item_2_Unlocked` true (`/Game/NovaeTerrae/Core/Characters/Base/BP_NTBaseCharacter.Journal_WG` (`self.Char_Ref`)))
      (elif (== (`self.Item_To_Give`) 3)
        (set `/Game/NovaeTerrae/UI/System_WG/Journal_WG.Item_3_Unlocked` true (`/Game/NovaeTerrae/Core/Characters/Base/BP_NTBaseCharacter.Journal_WG` (`self.Char_Ref`)))
        (elif (== (`self.Item_To_Give`) 4)
          (set `/Game/NovaeTerrae/UI/System_WG/Journal_WG.Item_4_Unlocked` true (`/Game/NovaeTerrae/Core/Characters/Base/BP_NTBaseCharacter.Journal_WG` (`self.Char_Ref`)))
          (elif (== (`self.Item_To_Give`) 5)
            (set `/Game/NovaeTerrae/UI/System_WG/Journal_WG.Item_5_Unlocked` true (`/Game/NovaeTerrae/Core/Characters/Base/BP_NTBaseCharacter.Journal_WG` (`self.Char_Ref`)))
            (elif (== (`self.Item_To_Give`) 6)
              (set `/Game/NovaeTerrae/UI/System_WG/Journal_WG.Item_6_Unlocked` true (`/Game/NovaeTerrae/Core/Characters/Base/BP_NTBaseCharacter.Journal_WG` (`self.Char_Ref`)))
              (elif (== (`self.Item_To_Give`) 7)
                (set `/Game/NovaeTerrae/UI/System_WG/Journal_WG.Item_7_Unlocked` true (`/Game/NovaeTerrae/Core/Characters/Base/BP_NTBaseCharacter.Journal_WG` (`self.Char_Ref`)))
                (elif (== (`self.Item_To_Give`) 8)
                  (set `/Game/NovaeTerrae/UI/System_WG/Journal_WG.Item_8_Unlocked` true (`/Game/NovaeTerrae/Core/Characters/Base/BP_NTBaseCharacter.Journal_WG` (`self.Char_Ref`))))))))))))

(fn `Note_Number_To_Give`
  (if (== (`self.Note_To_Give`) 1)
    (set `/Game/NovaeTerrae/UI/System_WG/Journal_WG.Note_1_Unlocked` true (`/Game/NovaeTerrae/Core/Characters/Base/BP_NTBaseCharacter.Journal_WG` (`self.Char_Ref`)))
    (elif (== (`self.Note_To_Give`) 2)
      (set `/Game/NovaeTerrae/UI/System_WG/Journal_WG.Note_2_Unlocked` true (`/Game/NovaeTerrae/Core/Characters/Base/BP_NTBaseCharacter.Journal_WG` (`self.Char_Ref`)))
      (elif (== (`self.Note_To_Give`) 3)
        (set `/Game/NovaeTerrae/UI/System_WG/Journal_WG.Note_3_Unlocked` true (`/Game/NovaeTerrae/Core/Characters/Base/BP_NTBaseCharacter.Journal_WG` (`self.Char_Ref`)))
        (elif (== (`self.Note_To_Give`) 4)
          (set `/Game/NovaeTerrae/UI/System_WG/Journal_WG.Note_4_Unlocked` true (`/Game/NovaeTerrae/Core/Characters/Base/BP_NTBaseCharacter.Journal_WG` (`self.Char_Ref`)))
          (elif (== (`self.Note_To_Give`) 5)
            (set `/Game/NovaeTerrae/UI/System_WG/Journal_WG.Note_5_Unlocked` true (`/Game/NovaeTerrae/Core/Characters/Base/BP_NTBaseCharacter.Journal_WG` (`self.Char_Ref`)))
            (elif (== (`self.Note_To_Give`) 6)
              (set `/Game/NovaeTerrae/UI/System_WG/Journal_WG.Note_6_Unlocked` true (`/Game/NovaeTerrae/Core/Characters/Base/BP_NTBaseCharacter.Journal_WG` (`self.Char_Ref`)))
              (elif (== (`self.Note_To_Give`) 7)
                (set `/Game/NovaeTerrae/UI/System_WG/Journal_WG.Note_7_Unlocked` true (`/Game/NovaeTerrae/Core/Characters/Base/BP_NTBaseCharacter.Journal_WG` (`self.Char_Ref`)))
                (elif (== (`self.Note_To_Give`) 8)
                  (set `/Game/NovaeTerrae/UI/System_WG/Journal_WG.Note_8_Unlocked` true (`/Game/NovaeTerrae/Core/Characters/Base/BP_NTBaseCharacter.Journal_WG` (`self.Char_Ref`))))))))))))

(fn `UserConstructionScript`)