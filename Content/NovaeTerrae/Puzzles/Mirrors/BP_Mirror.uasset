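; BP_Mirror is a puzzle mirror that bounces an incoming laser onward.
; Its Reflect event mirrors the incoming trace direction about the hit normal and line-traces along it to find the beam's end.
; It spawns a Niagara laser once, updates its endpoints, and forwards Reflect to the hit actor, allowing chained bounces.
; A retriggerable delay deactivates the beam and resets the spawn gate shortly after calls stop.
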(event `self.ReceiveBeginPlay`)

(event `/Game/NovaeTerrae/Puzzles/Mirrors/BPI_ReflectableInterface.Reflect`
  (params (HitLocation :type "Vector Structure") (TraceStart :type "Vector Structure") (TraceEnd :type "Vector Structure") (Normal :type "Vector Structure"))
  (bind _returnvalue (+ (`self.Hit Location`) (* (`KismetMathLibrary.GetReflectionVector` (`KismetMathLibrary.GetDirectionUnitVector` TraceStart TraceEnd) Normal) 3000.0)))
  (set `self.Hit Location` HitLocation)
  (bind (_outhit _returnvalue_2) (`KismetSystemLibrary.LineTraceSingle` (`self.Hit Location`) _returnvalue "TraceTypeQuery1"))
  (set `self.NewHitLocation` (`KismetMathLibrary.SelectVector` (`.Location` (`GameplayStatics.BreakHitResult` _outhit)) _returnvalue _returnvalue_2))
  (`|ExecutionSequence`
    (:`then_0`
      (`/Engine/EditorBlueprintResources/StandardMacros.DoOnce` false :!label _label
        (:`Completed`
          (bind _returnvalue_3 (`NiagaraFunctionLibrary.SpawnSystemAtLocation` "/Game/NovaeTerrae/Art/VFX/NS_laser_eyes.NS_laser_eyes" (`self.Hit Location`) (struct) (1.0 1.0 1.0) true false))
          (set `self.Laser` _returnvalue_3)
          (`FXSystemComponent.SetVectorParameter` (`self.Laser`) "LaserEnd" (`self.NewHitLocation`))
          (`ActorComponent.Activate` (`self.Laser`) false))))
    (:`then_1`
      (message `/Game/NovaeTerrae/Puzzles/Mirrors/BPI_ReflectableInterface.Reflect` (`.HitActor` (`GameplayStatics.BreakHitResult` _outhit)) (`self.NewHitLocation`) (`.TraceStart` (`GameplayStatics.BreakHitResult` _outhit)) (`.TraceEnd` (`GameplayStatics.BreakHitResult` _outhit)) (`.Normal` (`GameplayStatics.BreakHitResult` _outhit)))
      (`FXSystemComponent.SetVectorParameter` (`self.Laser`) "LaserEnd" (`self.NewHitLocation`))
      (`SceneComponent.K2_SetWorldLocation` (`self.Laser`) (`self.Hit Location`) false true)
      (`KismetSystemLibrary.RetriggerableDelay` 0.1)
      (`ActorComponent.Deactivate` (`self.Laser`))
      (goto _label :!via `Reset`))))

(fn `UserConstructionScript`)