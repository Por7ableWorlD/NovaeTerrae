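; Damageable target object for the core deactivation puzzle that can be knocked out temporarily while a challenge is active.
; It follows the activate and deactivate events of the level's BP_ChallengeZone.
; Damage fires OnDisabled, then after DeactivationTime the object revives and fires OnEnabled, unless Die has marked the core permanently deactivated.
; ChangeState swaps the cube's material to show live, disabled or deactivated state.
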(event `self.ReceiveBeginPlay`
  (bind _returnvalue (`GameplayStatics.GetActorOfClass` "/Game/NovaeTerrae/Puzzles/CoreDeactivation/BP_ChallengeZone.BP_ChallengeZone_C"))
  (bind _output_get (set `self.ChallengeZone` _returnvalue))
  (add `/Game/NovaeTerrae/Puzzles/CoreDeactivation/BP_ChallengeZone.OnActivateChallenge` _output_get (delegate `Activate`))
  (add `/Game/NovaeTerrae/Puzzles/CoreDeactivation/BP_ChallengeZone.OnDeactivateChallenge` _output_get (delegate `Deactivate`))
  (add `self.OnTakeAnyDamage` (delegate `TakeDamage`)))

(event `Activate`
  (set `self.IsChallengeActive` true))

(event `Deactivate`
  (set `self.IsChallengeActive` false))

(event `TakeDamage` :!signature `self.OnTakeAnyDamage`
  (params (DamagedActor :type "Actor Object Reference") (Damage :type "Float (single-precision)") (DamageType :type "DamageType Object Reference") (InstigatedBy :type "Controller Object Reference") (DamageCauser :type "Actor Object Reference"))
  (if (`self.IsChallengeActive`)
    (set `self.IsDead` true)
    (`self.ChangeState`)
    (`self.OnDisabled`)
    (`KismetSystemLibrary.Delay` (`self.DeactivationTime`))
    (if (not (`self.IsCoreDeativated`))
      (set `self.IsDead` false)
      (`self.OnEnabled`))
    (`self.ChangeState`)))

(event `Die`
  (set `self.IsDead` true)
  (set `self.IsCoreDeativated` true)
  (`self.ChangeState`))

(fn `ChangeState`
  (bind _cube (`self.Cube`))
  (if (`self.IsCoreDeativated`)
    (`PrimitiveComponent.SetMaterial` _cube 0 "/Engine/EngineMeshes/BackgroundMaterial.BackgroundMaterial")
    (elif (`self.IsDead`)
      (`PrimitiveComponent.SetMaterial` _cube 0 "/Engine/EngineMaterials/DefaultMaterial.DefaultMaterial")
      (else
        (`PrimitiveComponent.SetMaterial` (`self.Cube`) 0 "/Game/NovaeTerrae/Art/Level/Material/M_destroyobject.M_destroyobject")))))

(fn `UserConstructionScript`)