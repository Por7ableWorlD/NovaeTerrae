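; BP_Core is the interactable core of the core deactivation puzzle, letting the player end the challenge once every deactivator is disabled.
; After a short BeginPlay delay, it binds to each Deactivator in the level's BP_ChallengeZone and counts those still enabled.
; At zero it enables interaction and shows a hint; re-enabling one revokes both.
; Interacting ends the challenge and opens the linked Door_Core.
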(event `self.ReceiveBeginPlay`
  (bind _deactivators (`/Game/NovaeTerrae/Puzzles/CoreDeactivation/BP_ChallengeZone.Deactivators` (`self.ChallengeZone`)))
  (`parent.ReceiveBeginPlay`)
  (set `self.InteractionAvailable` false)
  (bind _returnvalue (`GameplayStatics.GetActorOfClass` "/Game/NovaeTerrae/Puzzles/CoreDeactivation/BP_ChallengeZone.BP_ChallengeZone_C"))
  (set `self.ChallengeZone` _returnvalue)
  (`KismetSystemLibrary.Delay` 0.5)
  (set `self.DeactivatorsCounter` (`KismetArrayLibrary.Array_Length` _deactivators))
  (for _array_element _deactivators
    (add `/Game/NovaeTerrae/Puzzles/CoreDeactivation/BP_DeactivationObject.OnDisabled` _array_element (delegate `DecreaseCounter`))
    (add `/Game/NovaeTerrae/Puzzles/CoreDeactivation/BP_DeactivationObject.OnEnabled` _array_element (delegate `IncreaseCounter`))))

(event `DecreaseCounter`
  (bind _result (`/Engine/EditorBlueprintResources/StandardMacros.DecrementInt` (`self.DeactivatorsCounter`))
    (:`  `
      (if (== _result 0)
        (`self.StartReactivationSequence`)))))

(event `IncreaseCounter`
  (`/Engine/EditorBlueprintResources/StandardMacros.IncrementInt` (`self.DeactivatorsCounter`)
    (:`  `
      (if (`self.InteractionAvailable`)
        (`self.RemoveHintWidget`)
        (set `self.InteractionAvailable` false)))))

(event `StartReactivationSequence`
  (set `self.InteractionAvailable` true)
  (if (`PrimitiveComponent.IsOverlappingActor` (`self.HintTrigger`) (`GameplayStatics.GetPlayerCharacter` 0))
    (`self.AddHintWidget`)))

(event `/Game/NovaeTerrae/Puzzles/BPI_InteractionInterface.StartInteraction`
  (if (`self.InteractionAvailable`)
    (`self.RemoveHintWidget`)
    (set `self.InteractionAvailable` false)
    (`/Game/NovaeTerrae/Puzzles/CoreDeactivation/BP_ChallengeZone.EndChallenge` (`self.ChallengeZone`))
    (bind _asdoor_core (cast `/Game/NovaeTerrae/Puzzles/Door_Core/Door_Core` (`self.Door_Core`)))
    (`/Game/NovaeTerrae/Puzzles/Door_Core/Door_Core.Open_Door` _asdoor_core)))

(fn `UserConstructionScript`)