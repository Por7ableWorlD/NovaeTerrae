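; Base Blueprint for puzzle interactables, providing a proximity hint and hold-to-interact progress UI.
; HintTrigger overlaps with BP_NTBaseCharacter toggle the InteractGuide while interaction is available, showing it only when not held.
; Hold events manage a WBP_HoldInteractWidget and an InteractionTime timer, with UpdateTimer re-calling itself through a short Delay to feed elapsed time to the widget.
; StartInteraction only prints an invalid-interactable message, apparently as a placeholder for child overrides.
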(event `self.ReceiveBeginPlay`
  (bind _interact_guide (`self.Interact_Guide`)
    (:`then`
      (`SceneComponent.SetVisibility` _interact_guide false false))
    (:`else`)))

(event `/Game/NovaeTerrae/Puzzles/BPI_InteractionInterface.StartInteraction`
  (`KismetSystemLibrary.PrintString` "Invalid Interactable!" true true (struct :`R` 1.0 :`A` 1.0)))

(event `self.HintTrigger.OnComponentBeginOverlap`
  (params (OverlappedComponent :type "PrimitiveComponent Object Reference") (OtherActor :type "Actor Object Reference") (OtherComp :type "PrimitiveComponent Object Reference") (OtherBodyIndex :type Integer) (bFromSweep :type Boolean) (SweepResult :type "HitResult Structure (by ref)"))
  (cast `/Game/NovaeTerrae/Core/Characters/Base/BP_NTBaseCharacter` OtherActor)
  (`self.AddHintWidget`))

(event `self.HintTrigger.OnComponentEndOverlap`
  (params (OverlappedComponent :type "PrimitiveComponent Object Reference") (OtherActor :type "Actor Object Reference") (OtherComp :type "PrimitiveComponent Object Reference") (OtherBodyIndex :type Integer))
  (cast `/Game/NovaeTerrae/Core/Characters/Base/BP_NTBaseCharacter` OtherActor)
  (`self.RemoveHintWidget`))

(event `AddHintWidget`
  (if (and (`self.InteractionAvailable`) (not (`self.IsHeld`)))
    (bind _interact_guide (`self.Interact_Guide`)
      (:`then`
        (`SceneComponent.SetVisibility` _interact_guide true false))
      (:`else`))))

(event `RemoveHintWidget`
  (if (`self.InteractionAvailable`)
    (bind _interact_guide (`self.Interact_Guide`)
      (:`then`
        (`SceneComponent.SetVisibility` _interact_guide false false))
      (:`else`))))

(event `AddHoldWidget`
  (`self.RemoveHintWidget`)
  (if (`self.InteractionAvailable`)
    (bind _returnvalue (`|CreateWidget` "/Game/NovaeTerrae/UI/WBP_HoldInteractWidget.WBP_HoldInteractWidget_C"))
    (bind _output_get (set `self.HoldWidget` _returnvalue))
    (`UserWidget.AddToViewport` _output_get 0)
    (set `/Game/NovaeTerrae/UI/WBP_HoldInteractWidget.MaxTimeHeld` (`self.InteractionTime`) (`self.HoldWidget`))))

(event `RemoveHoldWidget`
  (if (`self.InteractionAvailable`)
    (bind _holdwidget (`self.HoldWidget`)
      (:`then`
        (`Widget.RemoveFromParent` _holdwidget))
      (:`else`))))

(event `StopTimer`
  (`KismetSystemLibrary.K2_PauseTimerHandle` (`self.HoldInteractionTimerHandle`)))

(event `SetupTimer`
  (bind _returnvalue (`KismetSystemLibrary.K2_SetTimerDelegate` (delegate `SetupTimer`) (`self.InteractionTime`)))
  (set `self.HoldInteractionTimerHandle` _returnvalue))

(event `UpdateTimer`
  (if (`self.IsHeld`)
    (set `/Game/NovaeTerrae/UI/WBP_HoldInteractWidget.TimeHeld` (`KismetSystemLibrary.K2_GetTimerElapsedTimeHandle` (`self.HoldInteractionTimerHandle`)) (`self.HoldWidget`))
    (`KismetSystemLibrary.Delay` 0.01)
    (`self.UpdateTimer`)
    (else
      (`self.StopTimer`)
      (set `/Game/NovaeTerrae/UI/WBP_HoldInteractWidget.TimeHeld` 0.0 (`self.HoldWidget`)))))

(fn `UserConstructionScript`)