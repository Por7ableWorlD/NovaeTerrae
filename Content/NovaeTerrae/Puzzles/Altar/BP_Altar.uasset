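; BP_Altar is a checkpoint altar that saves the player's location when the player character overlaps its Save_Trigger.
; Saving writes SpawnPoint's X and Y, with Z and rotation zeroed, into the character's SaveRef and the Save_Info slot, only if that slot already exists.
; A Save_WG widget created at BeginPlay shows save feedback, with a delayed flag preventing overlapping replays.
; A full-health restore node is present but unconnected.
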(event `self.ReceiveBeginPlay`
  ;[0 0 0] Begin Play
  (bind _asbp_ntbase_character (cast `/Game/NovaeTerrae/Core/Characters/Base/BP_NTBaseCharacter` (`GameplayStatics.GetPlayerCharacter` 0)))
  (set `self.Char_Ref` _asbp_ntbase_character)
  (bind _returnvalue (`|CreateWidget` "/Game/NovaeTerrae/UI/Char_WG/Save_WG.Save_WG_C" (`GameplayStatics.GetPlayerController` 0)))
  (bind _output_get (set `self.Save_Wg` _returnvalue))
  (`UserWidget.AddToViewport` _output_get 0))

(event `self.Save_Trigger.OnComponentBeginOverlap`
  (params (OverlappedComponent :type "PrimitiveComponent Object Reference") (OtherActor :type "Actor Object Reference") (OtherComp :type "PrimitiveComponent Object Reference") (OtherBodyIndex :type Integer) (bFromSweep :type Boolean) (SweepResult :type "HitResult Structure (by ref)"))
  ;[0 0 0] Trigger Save
  (cast `/Game/NovaeTerrae/Core/Characters/Base/BP_NTBaseCharacter` OtherActor)
  (`self.Save_Game`)
  (if (not (`self.Anim_Playing`))
    (set `self.Anim_Playing` true)
    (`/Game/NovaeTerrae/UI/Char_WG/Save_WG.Save_Game` (`self.Save_Wg`))
    (`KismetSystemLibrary.Delay` 3.25)
    (set `self.Anim_Playing` false)))

(event `Save_Game`
  (bind (_returnvalue_x _returnvalue_y) (`KismetMathLibrary.BreakVector` (`SceneComponent.K2_GetComponentLocation` (`self.Spawn_Point`))))
  (bind _save_ref (`/Game/NovaeTerrae/Core/Characters/Base/BP_NTBaseCharacter.Save_Ref` (`self.Char_Ref`)))
  ;[0 0 0] Save Game
  (bind _returnvalue (`GameplayStatics.DoesSaveGameExist` "Save_Info"))
  (if _returnvalue
    (set `/Game/NovaeTerrae/Puzzles/Altar/BP_Save.Char_Location` (`KismetMathLibrary.MakeTransform` (`KismetMathLibrary.MakeVector` _returnvalue_x _returnvalue_y)) _save_ref)
    (`GameplayStatics.SaveGameToSlot` _save_ref "Save_Info")))

(fn `UserConstructionScript`)