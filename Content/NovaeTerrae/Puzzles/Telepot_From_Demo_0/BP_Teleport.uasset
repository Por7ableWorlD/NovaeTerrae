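; BP_Teleport is a trigger actor that moves the player to the demo level lvl_demo_L1_1.
; On player overlap it shows the Teleport_Error_WG widget, then waits a few seconds.
; It writes hardcoded CharLocation and CompLocation transforms to the Save_Info slot through the cached character's SaveRef, then opens the level.
; LvlToLoad is set and saved again only after the OpenLevel call, alongside restoring game-only input.
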(event `self.ReceiveBeginPlay`
  (bind _asbp_ntbase_character (cast `/Game/NovaeTerrae/Core/Characters/Base/BP_NTBaseCharacter` (`GameplayStatics.GetPlayerCharacter` 0)))
  (set `self.Char_Ref` _asbp_ntbase_character))

(event `self.Trigger.OnComponentBeginOverlap`
  (params (OverlappedComponent :type "PrimitiveComponent Object Reference") (OtherActor :type "Actor Object Reference") (OtherComp :type "PrimitiveComponent Object Reference") (OtherBodyIndex :type Integer) (bFromSweep :type Boolean) (SweepResult :type "HitResult Structure (by ref)"))
  (bind _save_ref (`/Game/NovaeTerrae/Core/Characters/Base/BP_NTBaseCharacter.Save_Ref` (`self.Char_Ref`)))
  (bind _save_ref_2 (`/Game/NovaeTerrae/Core/Characters/Base/BP_NTBaseCharacter.Save_Ref` (`self.Char_Ref`)))
  (cast `/Game/NovaeTerrae/Core/Characters/Base/BP_NTBaseCharacter` OtherActor)
  (bind _returnvalue (`|CreateWidget` "/Game/NovaeTerrae/Puzzles/Telepot_From_Demo_0/Teleport_Error_WG.Teleport_Error_WG_C"))
  (`UserWidget.AddToViewport` _returnvalue 5)
  (`KismetSystemLibrary.Delay` 5.2)
  (set `/Game/NovaeTerrae/Puzzles/Altar/BP_Save.Char_Location` (`KismetMathLibrary.MakeTransform` (-7170.274167 27997.299964 363.7962) (struct :`Yaw` -60.0)) _save_ref)
  (set `/Game/NovaeTerrae/Puzzles/Altar/BP_Save.Comp_Location` (`KismetMathLibrary.MakeTransform` (-7560.735195 28160.858668 394.247359)) _save_ref)
  (`GameplayStatics.SaveGameToSlot` _save_ref "Save_Info")
  (`GameplayStatics.OpenLevel` "lvl_demo_L1_1")
  (`WidgetBlueprintLibrary.SetInputMode_GameOnly` (`GameplayStatics.GetPlayerController` 0))
  (set `/Game/NovaeTerrae/Puzzles/Altar/BP_Save.Lvl_To_Load` "lvl_demo_L1_1" _save_ref_2)
  (`GameplayStatics.SaveGameToSlot` _save_ref_2 "Save_Info"))

(fn `UserConstructionScript`)